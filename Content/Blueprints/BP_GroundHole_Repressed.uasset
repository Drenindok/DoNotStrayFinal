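; BP_GroundHole_Repressed is a placeable ground hole actor that appears tied to the player's repressed form.
; Its construction script traces vertically through the actor's location and lays the Plane just above the hit surface, aligned to its normal.
; BeginPlay caches the player character as PlayerRef.
; The Activated event checks InRepressedForm, but that branch is empty, so activation has no effect yet.
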(event Custom|Activated
  (if (Variables|Default|GetInRepressedForm)
    _))

(event EventBeginPlay
  (bind _asplayer_character (Utilities|Casting|CastToPlayerCharacter (Game|GetPlayerCharacter 0)))
  (Variables|Default|SetPlayerRef _asplayer_character))

(fn ConstructionScript
  (bind _returnvalue (Transformation|GetActorLocation))
  (if (Variables|Default|GetUpdate)
    (Variables|Default|SetUpdate false))
  (bind _outhit (Collision|LineTraceByChannel (+ _returnvalue "0, 0,100.000000") (+ _returnvalue "0,0.000000,-100.000000") "TraceTypeQuery1" false 0 "None"))
  (Transformation|SetWorldLocationAndRotation (Variables|Default|GetPlane) (+ (.Location (Collision|BreakHitResult _outhit)) "0, 0,1.000000") (Math|Rotator|MakeRotfromZ (.ImpactNormal (Collision|BreakHitResult _outhit))) false true))