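; BP_InvisibleWall is a box blocker that stops the player with an "I'm not going back out there..." thought message.
; The construction script enables or disables the box's collision from CollisionOnByDefault.
; When the cached player character hits the box, it creates a timed, fading UI_ThoughtText widget near screen center horizontally.
; The stored widget reference prevents duplicate messages while one is still in the viewport.
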(event OnComponentHit(Box)
  (params (HitComponent :type Primitive%20Component%20Object%20Reference) (OtherActor :type Actor%20Object%20Reference) (OtherComp :type Primitive%20Component%20Object%20Reference) (NormalImpulse :type Vector :default "0, 0, 0") (Hit :type Hit%20Result%20Structure%20%28by%20ref%29))
  (if (== OtherActor (Variables|Default|GetPlayerRef))
    (Utilities|IsValid (Variables|Default|GetNotGoingBackMessageRef)
      (:Is%20Valid
        (if (not (UserInterface|Viewport|IsinViewport (Variables|Default|GetNotGoingBackMessageRef)))
          (bind _returnvalue (UserInterface|CreateWidget "/Game/UI/UI_ThoughtText.UI_ThoughtText_C" 0 "I'm not going back out there... " 5.0 3.0 0.0 0.0 (Math|Vector2D|MakeVector2D (.x (* (Viewport|GetViewportSize) 0.5)) 5.5e+02) "Center" (Utilities|Struct|MakeSlateColor "(R=1.000000,G=1.000000,B=1.000000,A=1.000000)" "UseColor_Specified") (Utilities|Struct|MakeSlateFontInfo "/Game/Fonts/VCR_OSD_MONO/VCR_OSD_MONO_1_001_Font.VCR_OSD_MONO_1_001_Font" 0 (Utilities|Struct|MakeFontOutlineSettings 2 false false 0 "(R=0.000000,G=0.000000,B=0.000000,A=1.000000)") "None" 24 0) :!label _label))
          (Variables|Default|SetNotGoingBackMessageRef _returnvalue)
          (UserInterface|Viewport|AddtoViewport _returnvalue 0)))
      (:Is%20Not%20Valid
        (goto _label)))))

(event EventBeginPlay
  (bind _asplayer_character (Utilities|Casting|CastToPlayerCharacter (Game|GetPlayerCharacter 0)))
  (Variables|Default|SetPlayerRef _asplayer_character))

(fn ConstructionScript
  (Collision|SetCollisionEnabled (Variables|Default|GetBox) (select (Variables|Default|GetCollisionOnByDefault) "QueryAndPhysics" "NoCollision")))