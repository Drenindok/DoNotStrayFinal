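; Ending cutscene actor that runs the game's finales, either on entering the car or through EndGame.
; EnterCar fades out, then branches on Leave: credits, save and main menu, or timed recursive thoughts leading to the memory-format prompt.
; EndGame despawns the monster and fades to white, then shows thoughts or plays a camera-fall sequence.
; During the fall, Tick pins the phone mesh to a level CameraActor, then eases it back to the player.
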(event OnComponentBeginOverlap(Sphere)
  (params (OverlappedComponent :type Primitive%20Component%20Object%20Reference) (OtherActor :type Actor%20Object%20Reference) (OtherComp :type Primitive%20Component%20Object%20Reference) (OtherBodyIndex :type Integer) (bFromSweep :type Boolean) (SweepResult :type Hit%20Result%20Structure%20%28by%20ref%29))
  (if (== OtherActor (Variables|Default|GetPlayerRef))
    _))

(event Custom|EndGame
  (params (StaticEnding? :type Boolean))
  (CameraFades|StartCameraFade (Game|GetPlayerCameraManager 0) 0.0 1.0 3.0 "(R=1.000000,G=1.000000,B=1.000000,A=1.000000)" false true)
  (Variables|/Game/Blueprints/Monster/MonsterCharacter.MonsterCharacter_C|SetDifficulty (Variables|/Game/Blueprints/ThirdPersonBP/Blueprints/PlayerCharacter.PlayerCharacter_C|GetMonsterRef (Variables|Default|GetPlayerRef)) (Utilities|Struct|Makevar_Difficulty "(GLITCHChance_37_E73C82214BAB7F2F947AA7A623ECD544=0.000000,DespawnedTimeMin_52_634BC33F40C3C03546AEDCB070081242=0.000000,DespawnedTimeMax_54_74AECF2841DFFE347F97D78B6E69C2AE=60.000000,MoveGlitchIndependantly_42_C250E44047F519ABF110769D7D293B9C=False,MoveInChanceFarWander_47_AD20563042386C7A9393608281F29D09=0.000000,BackOffChance_33_977D54AA430FF5A844FAE48872CC2B70=0.000000,DurrationMin_14_4A9AB6FA4F2F5378381E74A29F1B0A9A=8.000000,DurrationMax_13_BF5CB1C14CC2246EB2A910B2CCA3AC7D=20.000000,Strength_12_A692411E477FE254A01001BC29D0A3C3=0.800000,Volume_20_4A82EE5C4235D8454519CB952AD1FA7F=0.000000,SingVolume_36_2A91C09D4F1457266C5814BC17071A10=0.000000)" "(Radius_26_71EAF0EE472424D0622003BF92DDBA4E=1250.000000,MoveSpeed_27_5CB97014430CB08BE3B3A98736F63799=0.000000,WaitMinTime_6_0E656BA94424221B2E30B9AD05A6E1BF=5.000000,WaitMaxTime_8_0E37781B45EC9F5B9CF50D896178F248=15.000000,MoveInChance_25_9A97DB2844E56E0B3C9D238BA1DA0A2A=0.250000,LeaveChance_10_33B858DF446A4138FB1811B764D033CE=0.250000)" "(Radius_25_5CB97014430CB08BE3B3A98736F63799=1000.000000,MoveSpeed_35_BBBC26A24CE9EF946372A2ABABB74848=100.000000,IgnorePlayer_28_13DC21314D26AB5721E395AAA5DD0C15=False,WaitMinTime_6_0E656BA94424221B2E30B9AD05A6E1BF=2.500000,WaitMaxTime_8_0E37781B45EC9F5B9CF50D896178F248=5.000000,StopHearBuffer_12_9A97DB2844E56E0B3C9D238BA1DA0A2A=2.000000,SeePlayerDelay_32_F0DFAD42448A58399E318D94A68EE297=2.000000,LeaveAfterMin_37_33B858DF446A4138FB1811B764D033CE=0,LeaveAfterMax_39_B9560D57448B8A1B45B5DAB49ACDDE7B=1)" 0.0 (Utilities|Array|MakeArray "") 6e+01 1.5785116693933588e+19 0.0 4.0 false 0.0 0.0 false false false false))
  (Default|SwitchtoDespawned (Variables|/Game/Blueprints/ThirdPersonBP/Blueprints/PlayerCharacter.PlayerCharacter_C|GetMonsterRef (Variables|Default|GetPlayerRef)) true false -1.0)
  (if StaticEnding?
    (Audio|SetSoundMixClassOverride "/Game/Audio/DefaultSoundMix.DefaultSoundMix" "/Game/Audio/SoundClass_WorldSounds.SoundClass_WorldSounds" 0.0 1.0 3.0 true)
    (bind _returnvalue (Audio|CreateSound2D "/Game/Audio/Ambient/wav_vinylCrackle.wav_vinylCrackle" 1.0 1.0 0.0 0))
    (Audio|Components|Audio|FadeIn _returnvalue 3.0 0.5 0.0 "Linear" :!class /Script/Engine.AudioComponent))
  (Utilities|FlowControl|Delay 3.0)
  (Viewport|RemoveAllWidgets)
  (Variables|/Game/Blueprints/ThirdPersonBP/Blueprints/PlayerCharacter.PlayerCharacter_C|SetLockMovement (Variables|Default|GetPlayerRef) true)
  (Input|DisableInput (Variables|Default|GetPlayerRef) (Game|GetPlayerController 0))
  (if StaticEnding?
    (Utilities|FlowControl|Delay 5.0)
    (CallFunction|DisplayNextThought)
    (else
      (|Dropcameratoground,thenpickbackup))))

(event Custom|DisplayNextThought
  (bind _returnvalue (Game|GetPlayerController 0))
  (bind _currentthought_ (Variables|Default|GetCurrentThought#))
  (bind _thoughts (Variables|Default|GetThoughts))
  (bind _output (Utilities|Array|Get(acopy) _thoughts _currentthought_))
  (if (Utilities|Array|IsValidIndex _thoughts _currentthought_)
    (bind _returnvalue_2 (UserInterface|CreateWidget "/Game/UI/UI_ThoughtText.UI_ThoughtText_C" 0 (.text _output) -1.0 3.0 0.0 0.0 (Math|Vector2D|MakeVector2D 1e+02 (+ 5.5e+02 (* (Variables|Default|GetPositionOffset) 25.0))) "Left" (Utilities|Struct|MakeSlateColor "(R=1.000000,G=1.000000,B=1.000000,A=1.000000)") (Utilities|Struct|MakeSlateFontInfo "/Engine/EngineFonts/Roboto.Roboto")))
    (Utilities|Array|Add (Variables|Default|GetDisplayedTexts) _returnvalue_2)
    (UserInterface|Viewport|AddtoViewport _returnvalue_2 0)
    (Utilities|FlowControl|Delay (.delaytonext _output))
    (if (.resetafter _output)
      (for _array_element (Variables|Default|GetDisplayedTexts)
        (Variables|/Game/UI/UI_ThoughtText.UI_ThoughtText_C|SetFadeIn _array_element false))
      (Utilities|FlowControl|Delay (.delayafterresetting _output))
      (Variables|Default|SetPositionOffset 0))
    (Math|Integer|IncrementInt (Variables|Default|GetCurrentThought#)
      (:%20%20
        (Math|Integer|IncrementInt (Variables|Default|GetPositionOffset)
          (:%20%20
            (CallFunction|DisplayNextThought)))))
    (elif (Variables|Default|GetLeave)
      (Utilities|FlowControl|Delay 3.0)
      (if (not (Variables|Default|GetShowEndCredits))
        (bind _asmain_game_instance (Utilities|Casting|CastToMainGameInstance (Game|GetGameInstance)))
        (Default|FadeOutAllPlayingSounds _asmain_game_instance 5.0)
        (Utilities|FlowControl|Delay 8.0)
        (Variables|/Game/MainGameInstance.MainGameInstance_C|SetShowEndingBPopup _asmain_game_instance true)
        (bind _returnvalue_3 (SaveGame|LoadGamefromSlot "PlayerData"))
        (bind _asplayer_save_data (Utilities|Casting|CastToPlayerSaveData _returnvalue_3))
        (Variables|/Game/PlayerSaveData.PlayerSaveData_C|SetUnlockedFirstRunCompleted _asplayer_save_data true)
        (SaveGame|SaveGametoSlot _asplayer_save_data "PlayerData")
        (Game|OpenLevel(byName) "Level_MainMenu"))
      (else
        (Utilities|FlowControl|Delay 8.0)
        (bind _returnvalue_4 (UserInterface|CreateWidget "/Game/UI/DeletePopups/UI_FormatMemory_2nd.UI_FormatMemory_2nd_C"))
        (UserInterface|Viewport|AddtoViewport _returnvalue_4 0)
        (Variables|/Script/Engine.PlayerController|SetbShowMouseCursor _returnvalue true)
        (Input|SetInputModeGameandUI _returnvalue _returnvalue_4 "DoNotLock" false)))))

(event Custom|EnterCar
  (bind _leave (Variables|Default|GetLeave))
  (Utilities|FlowControl|DoOnce false
    (:Completed
      (Variables|/Game/Blueprints/ThirdPersonBP/Blueprints/PlayerCharacter.PlayerCharacter_C|SetLockMovement (Variables|Default|GetPlayerRef) true)
      (Variables|/Game/UI/PlayerHUD.PlayerHUD_C|SetShouldShowKeyPrompts (Variables|/Game/Blueprints/ThirdPersonBP/Blueprints/PlayerCharacter.PlayerCharacter_C|GetHUDref (Variables|Default|GetPlayerRef)) false)
      (Input|DisableInput (Variables|Default|GetPlayerRef) (Game|GetPlayerController 0))
      (CameraFades|StartCameraFade :self (Game|GetPlayerCameraManager 0) :ToAlpha 1.0 :Duration 1.0 :bHoldWhenFinished true)
      (bind _outactors (Actor|GetAllActorswithTag "ForestAmbience"))
      (bind _asambient_sound (Utilities|Casting|CastToAmbientSound (Utilities|Array|Get(acopy) _outactors))
        (:then
          (Audio|Components|Audio|FadeOut (Variables|/Script/Engine.AmbientSound|GetAudioComponent _asambient_sound) 5.0 0.0 "Linear" :!class /Script/Engine.AudioComponent)
          (bind _asmain_game_instance (Utilities|Casting|CastToMainGameInstance (Game|GetGameInstance)))
          (Default|PlayPersistentAudio _asmain_game_instance (select _leave "/Game/Audio/Cutscenes/wav_Cutscene_EnterCar_Leave.wav_Cutscene_EnterCar_Leave" "/Game/Audio/Cutscenes/wav_Cutscene_JustEnterCar.wav_Cutscene_JustEnterCar") 1.0 1.0 11.0)
          (Utilities|FlowControl|Sequence
            (:then_0
              (if (Variables|Default|GetLeave)
                (Utilities|FlowControl|Delay 17.0) ; Finished first run, doesn't have evidence
                ;[0.401 0 0] Show "I couldn't find anything" thoughts
                (bind _asmain_game_instance_2 (Utilities|Casting|CastToMainGameInstance (Game|GetGameInstance)))
                (Default|ShowThoughts _asmain_game_instance_2 "In the end, I...[D=3][LasD=5] 
>I couldn't find anything... 
>Maybe next year..." (Utilities|Struct|MakeSlateFontInfo "/Game/Fonts/naomis_hand-NewFathersFont/NaomisHand-Regular_Font.NaomisHand-Regular_Font") (Utilities|Struct|MakeSlateColor "(R=1.000000,G=1.000000,B=1.000000,A=1.000000)") true 25.0 0.0 0.0 false false)
                (Utilities|FlowControl|Delay 12.0)
                ;[0 0.6142 1] End credits
                (|ShowCredits
                  (:%20
                    (Utilities|FlowControl|Delay 25.0)
                    (bind _asmain_game_instance_3 (Utilities|Casting|CastToMainGameInstance (Game|GetGameInstance)))
                    (Default|FadeOutAllPlayingSounds _asmain_game_instance_3 5.0)
                    (Utilities|FlowControl|Delay 8.0)
                    (Variables|/Game/MainGameInstance.MainGameInstance_C|SetShowEndingBPopup _asmain_game_instance_3 true)
                    (bind _returnvalue (SaveGame|LoadGamefromSlot "PlayerData"))
                    (bind _asplayer_save_data (Utilities|Casting|CastToPlayerSaveData _returnvalue))
                    (Variables|/Game/PlayerSaveData.PlayerSaveData_C|SetUnlockedFirstRunCompleted _asplayer_save_data true)
                    (SaveGame|SaveGametoSlot _asplayer_save_data "PlayerData")
                    (Game|OpenLevel(byName) "Level_MainMenu")))
                (else
                  (Utilities|FlowControl|Delay 17.0) ; Finished 2nd run, has evidence
                  (Variables|Default|SetThoughts (Variables|Default|GetCryThoughts))
                  (CallFunction|DisplayNextThought))))
            (:then_1
              (if (not _leave)
                (Utilities|FlowControl|Delay 5.0)
                (Default|FadeOutAllPlayingSounds _asmain_game_instance 6.0)
                (Default|PlayPersistentAudio _asmain_game_instance "/Game/Audio/Cutscenes/wav_Heartbeat.wav_Heartbeat" 6.0 1.0 0.0)))))
        (:CastFailed
          (Development|PrintString "ERROR : Sound_ForestAmbience NOT TAGGED AS \"ForestAmbience\"!!!" true true "(R=1.000000,G=0.000000,B=0.000000,A=1.000000)"))))))

(event Custom|JustDisplayLeaveThoughts)

(event EventBeginPlay
  (bind _asplayer_character (Utilities|Casting|CastToPlayerCharacter (Game|GetPlayerCharacter 0)))
  (Variables|Default|SetPlayerRef _asplayer_character)
  (Collision|SetCollisionEnabled (Variables|Default|GetSphere) (select (Variables|Default|GetCollisionOnByDefault) "QueryAndPhysics" "NoCollision")))

(fn ConstructionScript)

(event EventTick
  (params (DeltaSeconds :type Float%20%28single-precision%29))
  (bind _dropcameraref (Variables|Default|GetDropCameraRef))
  (bind _dropcameraref_2 (Variables|Default|GetDropCameraRef))
  (bind _playerref (Variables|Default|GetPlayerRef))
  (bind _scenecomponent (Variables|/Script/Engine.CameraActor|GetSceneComponent _dropcameraref))
  (bind _scenecomponent_2 (Variables|/Script/Engine.CameraActor|GetSceneComponent _dropcameraref_2))
  (bind _returnvalue (Transformation|GetWorldTransform _scenecomponent))
  (bind _returnvalue_2 (Transformation|GetWorldTransform _scenecomponent_2))
  (if (Variables|Default|GetInCameraDropCutscene)
    (if (Variables|Default|GetTransitionOutOfCameraDrop)
      (Variables|Default|SetCameraDropFade (Math|Interpolation|FInterpTo (Variables|Default|GetCameraDropFade) 1.0 (Utilities|Time|GetWorldDeltaSeconds) 1.5))
      (Transformation|SetWorldLocationAndRotation (Variables|/Game/Blueprints/ThirdPersonBP/Blueprints/PlayerCharacter.PlayerCharacter_C|GetPhoneMesh _playerref) (Math|Vector|Lerp(Vector) (.location _returnvalue_2) (Transformation|GetWorldLocation (Variables|/Game/Blueprints/ThirdPersonBP/Blueprints/PlayerCharacter.PlayerCharacter_C|GetCam-PhoneArm _playerref)) (Class|KismetMathLibrary|FInterpEaseinOut 0.0 1.0 (Variables|Default|GetCameraDropFade) 2.0)) (Math|Rotator|Lerp(Rotator) (.rotation _returnvalue_2) (Pawn|GetControlRotation (Game|GetPlayerController 0) :!class /Script/Engine.Controller) (Class|KismetMathLibrary|FInterpEaseinOut 0.0 1.0 (Variables|Default|GetCameraDropFade) 2.0) true) false false)
      (if (== (Variables|Default|GetCameraDropFade) 1.0)
        (Variables|Default|SetInCameraDropCutscene false))
      (else
        (Transformation|SetWorldLocationAndRotation (Variables|/Game/Blueprints/ThirdPersonBP/Blueprints/PlayerCharacter.PlayerCharacter_C|GetPhoneMesh (Variables|Default|GetPlayerRef)) (.location _returnvalue) (.rotation _returnvalue) false false)))))