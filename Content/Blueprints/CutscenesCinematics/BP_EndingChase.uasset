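; Scripted ending chase: StartChase sets the monster chasing the player while on-screen thought text plays.
; DisplayNextThought steps through the Thoughts array, spawning styled text widgets that stack or reset per entry.
; The seventh thought disables the monster and runs a timeline fading screen and world sound, adding static and slowing time.
; Inverse CustomTimeDilation offsets the slowdown for this actor; the timeline's finish triggers BP_Static_Cutscene's static ending.
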(event Custom|StartChase
  (bind _asplayer_character (Utilities|Casting|CastToPlayerCharacter (Game|GetPlayerCharacter 0)))
  (Variables|Default|SetPlayerRef _asplayer_character)
  (Utilities|FlowControl|Sequence
    (:then_0
      (Utilities|FlowControl|Delay 2.0)
      (Variables|/Game/Blueprints/Monster/MonsterCharacter.MonsterCharacter_C|SetDifficulty (Variables|/Game/Blueprints/ThirdPersonBP/Blueprints/PlayerCharacter.PlayerCharacter_C|GetMonsterRef (Variables|Default|GetPlayerRef)) (Utilities|Struct|Makevar_Difficulty "(GLITCHChance_37_E73C82214BAB7F2F947AA7A623ECD544=0.000000,MoveGlitchIndependantly_42_C250E44047F519ABF110769D7D293B9C=False,MoveInChanceDespawned_46_160AF2A8488CD7184D73AB973C2870FB=0.000000,MoveInChanceFarWander_47_AD20563042386C7A9393608281F29D09=0.000000,BackOffChance_33_977D54AA430FF5A844FAE48872CC2B70=0.000000,DurrationMin_14_4A9AB6FA4F2F5378381E74A29F1B0A9A=8.000000,DurrationMax_13_BF5CB1C14CC2246EB2A910B2CCA3AC7D=20.000000,Strength_12_A692411E477FE254A01001BC29D0A3C3=0.800000,Volume_20_4A82EE5C4235D8454519CB952AD1FA7F=0.000000,SingVolume_36_2A91C09D4F1457266C5814BC17071A10=0.000000)" "(Radius_26_71EAF0EE472424D0622003BF92DDBA4E=1250.000000,MoveSpeed_27_5CB97014430CB08BE3B3A98736F63799=0.000000,WaitMinTime_6_0E656BA94424221B2E30B9AD05A6E1BF=5.000000,WaitMaxTime_8_0E37781B45EC9F5B9CF50D896178F248=15.000000,MoveInChance_25_9A97DB2844E56E0B3C9D238BA1DA0A2A=0.250000,LeaveChance_10_33B858DF446A4138FB1811B764D033CE=0.250000)" "(Radius_25_5CB97014430CB08BE3B3A98736F63799=1000.000000,MoveSpeed_35_BBBC26A24CE9EF946372A2ABABB74848=100.000000,IgnorePlayer_28_13DC21314D26AB5721E395AAA5DD0C15=False,WaitMinTime_6_0E656BA94424221B2E30B9AD05A6E1BF=2.500000,WaitMaxTime_8_0E37781B45EC9F5B9CF50D896178F248=5.000000,StopHearBuffer_12_9A97DB2844E56E0B3C9D238BA1DA0A2A=2.000000,SeePlayerDelay_32_F0DFAD42448A58399E318D94A68EE297=2.000000,LeaveChance_10_33B858DF446A4138FB1811B764D033CE=0.250000)" 0.0 (Utilities|Array|MakeArray) 6e+01 4e+03 0.0 4.0 false 0.0 0.0 true true false true))
      (Variables|/Game/Blueprints/ThirdPersonBP/Blueprints/PlayerCharacter.PlayerCharacter_C|SetRewindSoundClipStartTime (Variables|Default|GetPlayerRef) 0.05)
      (Default|SwitchtoChasing (Variables|/Game/Blueprints/ThirdPersonBP/Blueprints/PlayerCharacter.PlayerCharacter_C|GetMonsterRef (Variables|Default|GetPlayerRef)))
      (Transformation|SetActorLocation (Variables|/Game/Blueprints/ThirdPersonBP/Blueprints/PlayerCharacter.PlayerCharacter_C|GetMonsterRef (Variables|Default|GetPlayerRef)) (+ (Transformation|GetActorLocation (Variables|Default|GetPlayerRef)) "0,1500.000000, 0") false true))
    (:then_1
      (CallFunction|DisplayNextThought))
    (:then_2
      (Utilities|FlowControl|Delay 11.41) ; ends when monster lights up red after\nrising up\n\ndefault 9.11s\n\n10.01s if using whole note as a delay
      (Default|SaveNumberOfDeathsFun (Variables|Default|GetPlayerRef) true)
      (Default|UpdateFogEffects (Variables|Default|GetPlayerRef)))))

(event Custom|DisplayNextThought
  (bind _returnvalue (Viewport|GetViewportSize))
  (bind _playerref (Variables|Default|GetPlayerRef))
  (bind _currentthought_ (Variables|Default|GetCurrentThought#))
  (bind _thoughts (Variables|Default|GetThoughts))
  (bind _output (Utilities|Array|Get(acopy) _thoughts _currentthought_))
  (bind _monsterref (Variables|/Game/Blueprints/ThirdPersonBP/Blueprints/PlayerCharacter.PlayerCharacter_C|GetMonsterRef _playerref))
  (if (Utilities|Array|IsValidIndex _thoughts _currentthought_)
    (if (== _currentthought_ 6)
      (Utilities|FlowControl|Sequence ; fade away chase sequence when this thought hits
        (:then_0
          (Components|Movement|StopMovementImmediately (Variables|/Script/Engine.Character|GetCharacterMovement _monsterref))
          (Variables|/Game/Blueprints/Monster/MonsterCharacter.MonsterCharacter_C|SetBehaviourState _monsterref "DoNothing") ; disables killing player and doesn't let him do anything
          ;[1 1 1] Fade away/End chase
          (Variables|/Game/UI/PlayerHUD.PlayerHUD_C|SetShouldShowSignposts+Tutorials (Variables|/Game/Blueprints/ThirdPersonBP/Blueprints/PlayerCharacter.PlayerCharacter_C|GetHUDref (Variables|Default|GetPlayerRef)) false) ; setting this to false hides all tutorial text, \nsign post text, etc
          (Audio|SetSoundMixClassOverride "/Game/Audio/DefaultSoundMix.DefaultSoundMix" "/Game/Audio/SoundClass_WorldSounds.SoundClass_WorldSounds" 0.0 1.0 13.81 true)
          (bind (_direction _timescale _screenfade) (Timeline|TimeSlowTimeline Play)
            (:Update
              (Class|PlayerCameraManager|SetManualCameraFade (Game|GetPlayerCameraManager 0) _screenfade "(R=0.000000,G=0.000000,B=0.000000,A=1.000000)" false)
              (Utilities|Time|SetGlobalTimeDilation _timescale)
              (Variables|Default|SetCustomTimeDilation (/ 1.0 _timescale))
              (Rendering|Material|SetScalarParameterValue "/Game/MeshesMaterialsTextures/GlobalMaterialParams.GlobalMaterialParams" "ScreenStatic" (* _screenfade 0.5) :!class /Script/Engine.KismetMaterialLibrary))
            (:Finished
              ;;[1 1 1] End chase
              (bind _outactors (Actor|GetAllActorsOfClass "/Game/Blueprints/CutscenesCinematics/BP_Static_Cutscene.BP_Static_Cutscene_C"))
              (Default|EndGame (Utilities|Array|Get(acopy) _outactors) true false false false)
              (Class|PlayerCameraManager|SetManualCameraFade (Game|GetPlayerCameraManager 0) 1.0 "(R=0.000000,G=0.000000,B=0.000000,A=1.000000)" false)
              (Utilities|Time|SetGlobalTimeDilation 1.0))
            (:DisplayNextThought
              (if (.resetafter _output) :!label _label
                (for _array_element (Variables|Default|GetDisplayedTexts)
                  (Variables|/Game/UI/UI_ThoughtText.UI_ThoughtText_C|SetFadeIn _array_element false))
                (Utilities|FlowControl|Delay (.delayafterresetting _output))
                (Variables|Default|SetPositionOffset 0)
                (else
                  (Math|Integer|IncrementInt (Variables|Default|GetPositionOffset)
                    (:%20%20
                      _))))
              (Math|Integer|IncrementInt (Variables|Default|GetCurrentThought#)
                (:%20%20
                  (CallFunction|DisplayNextThought))))))
        (:then_1
          (bind _returnvalue_2 (UserInterface|CreateWidget "/Game/UI/UI_ThoughtText.UI_ThoughtText_C" 0 (.text _output) -1.0 (.fadespeed _output) (.charshake _output) (.charglitch _output) (select (Math|Vector|Equal(Vector) (.forcescreenpos _output) "(X=-1.000000,Y=-1.000000)" 0.0001) (Math|Vector2D|MakeVector2D (* (.x (Viewport|GetViewportSize)) 0.5) (+ 5.5e+02 (* (Variables|Default|GetPositionOffset) 25.0))) (+ (Math|Vector2D|MakeVector2D (* (.x _returnvalue) 0.5) (* (.y _returnvalue) 0.5)) (.forcescreenpos _output))) "Center" (.fontcolor _output) (.font _output) :!label _label_2))
          (Utilities|Array|Add (Variables|Default|GetDisplayedTexts) _returnvalue_2)
          (UserInterface|Viewport|AddtoViewport _returnvalue_2 0)
          (Utilities|FlowControl|Delay (.delaytonext _output))
          (goto _label)))
      (else
        (goto _label_2)))))

(fn ConstructionScript)