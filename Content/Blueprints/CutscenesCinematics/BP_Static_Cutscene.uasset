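; Ending cutscene actor that runs the game's finales: static ending, camera-drop escape and footage-deleted time unfreeze.
; EndGame branches on flags, disabling the monster and either freezing the player amid vinyl static or restoring play.
; The camera drop plays a level sequence, drives glitch strength from audio playback through a curve, then eases the phone back into hand.
; RollCredits saves the static-ending unlock, shows credits and opens the delete-footage prompt.
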(event Custom|EndGame
  (params (StaticEnding? :type Boolean) (InstantCameraHit :type Boolean) (show%20"Oh...%20I%20made%20it..." :type Boolean) (EscapedParadox%28FootageDeleted%29 :type Boolean))
  (bind _escapedstaticrespawnpoint (Variables|Default|GetEscapedStaticRespawnPoint))
  (bind _returnvalue (Transformation|GetWorldTransform _escapedstaticrespawnpoint))
  (if EscapedParadox%28FootageDeleted%29
    ;[1 1 1] Unfreeze time
    (|Unfreezetime)
    (elif StaticEnding?
      (CallFunction|CompletelyRemoveandDisableEnemy)
      (Transformation|SetActorLocation (Variables|Default|GetPlayerRef) (.location _returnvalue) false true)
      (Pawn|SetControlRotation (Game|GetPlayerController 0) (.rotation _returnvalue))
      (Audio|SetSoundMixClassOverride "/Game/Audio/DefaultSoundMix.DefaultSoundMix" "/Game/Audio/SoundClass_WorldSounds.SoundClass_WorldSounds" 0.0 1.0 0.0 true)
      (bind _returnvalue_2 (Audio|CreateSound2D "/Game/Audio/Ambient/wav_vinylCrackle.wav_vinylCrackle" 1.0 1.0 0.0 0))
      (bind _output_get (Variables|Default|SetVinylStaticSound _returnvalue_2))
      (Audio|Components|Audio|FadeIn _output_get 0.0 0.5 0.0 "Linear" :!class /Script/Engine.AudioComponent)
      (CallFunction|FreezePlayer :!label _label)
      (Utilities|FlowControl|Sequence
        (:then_0
          (Utilities|FlowControl|Delay 5.0)
          (Variables|Default|SetFadeOutScreenStatic true))
        (:then_1
          (if StaticEnding?
            (Utilities|FlowControl|Delay 15.0) ; default 12
            (bind _asmain_game_instance (Utilities|Casting|CastToMainGameInstance (Game|GetGameInstance)))
            (Default|ShowThoughts _asmain_game_instance (Variables|Default|GetThoughts) (Utilities|Struct|MakeSlateFontInfo "/Game/Fonts/naomis_hand-NewFathersFont/NaomisHand-Regular_Font.NaomisHand-Regular_Font" 0 "(OutlineSize=0,bSeparateFillAlpha=False,bApplyOutlineToDropShadows=False,OutlineMaterial=None,OutlineColor=(R=0.000000,G=0.000000,B=0.000000,A=1.000000))" "None" 20) (Utilities|Struct|MakeSlateColor "(R=0.247059,G=0.247059,B=0.247059,A=1.000000)") true 25.0 0.0 0.0 true false)
            (else
              (CallFunction|UnlockCheckpoint (Utilities|String|MakeLiteralString "EndingChoice") :!label _label_2)
              (|Dropcameratoground,thenpickbackup show%20"Oh...%20I%20made%20it...")))))
      (elif InstantCameraHit
        (CallFunction|CompletelyRemoveandDisableEnemy)
        (CallFunction|FreezePlayer)
        (Viewport|RemoveAllWidgets)
        (goto _label_2)
        (else
          (CameraFades|StartCameraFade (Game|GetPlayerCameraManager 0) 0.0 1.0 3.0 "(R=1.000000,G=1.000000,B=1.000000,A=1.000000)" false true)
          (CallFunction|CompletelyRemoveandDisableEnemy)
          (Utilities|FlowControl|Delay 3.0)
          (goto _label))))))

(event Custom|UnFreezeTime
  ;[1 1 1] Unfreeze time when you delete footage
  (Utilities|Time|SetGlobalTimeDilation 1.0)
  (Audio|Components|Audio|Stop (Variables|Default|GetVinylStaticSound))
  (Input|DisableInput (Game|GetPlayerController 0))
  (Audio|SetSoundMixClassOverride "/Game/Audio/DefaultSoundMix.DefaultSoundMix" "/Game/Audio/SoundClass_WorldSounds.SoundClass_WorldSounds" 1.0 1.0 0.0 true)
  (bind _outactors (Actor|GetAllActorswithTag "ForestAmbience"))
  (bind _asambient_sound (Utilities|Casting|CastToAmbientSound (Utilities|Array|Get(acopy) _outactors)))
  (Audio|Components|Audio|Play (Variables|/Script/Engine.AmbientSound|GetAudioComponent _asambient_sound) 0.0))

(event Custom|RollCredits
  (bind _returnvalue (Game|GetPlayerController 0))
  (bind _slatecolor (Utilities|Struct|MakeSlateColor "(R=0.000000,G=0.000000,B=0.000000,A=1.000000)"))
  (bind _fontoutlinesettings (Utilities|Struct|MakeFontOutlineSettings 2 false false 0 "(R=0.500000,G=0.500000,B=0.500000,A=1.000000)"))
  (bind _slatefontinfo (Utilities|Struct|MakeSlateFontInfo "/Game/Fonts/VCR_OSD_MONO/VCR_OSD_MONO_1_001_Font.VCR_OSD_MONO_1_001_Font" 0 _fontoutlinesettings "None" 16))
  ;[0 0.9636 1] Roll credits and unlock secret static ending
  (CallFunction|UnlockStaticEnding)
  (Utilities|FlowControl|DoOnce false
    (:Completed
      ;[0 0.6142 1] End credits
      (|ShowCredits
        (:%20
          (Utilities|FlowControl|Delay 3e+01)
          ;[0.1875 0.1875 0.1875] Monster talks to you, tells you to delete footage. Enable player's input to let them click
          (bind _asmain_game_instance (Utilities|Casting|CastToMainGameInstance (Game|GetGameInstance)))
          (Default|ShowThoughts _asmain_game_instance "Like it or not...[D=2][LasD=5] 
>There's only one way out of this." _slatefontinfo _slatecolor true 25.0 0.0 0.0 true false)
          (Utilities|FlowControl|Delay 8.0)
          (bind _returnvalue_2 (UserInterface|CreateWidget "/Game/UI/DeletePopups/UI_FormatMemory_1st.UI_FormatMemory_1st_C" 0 true))
          (UserInterface|Viewport|AddtoViewport _returnvalue_2 0)
          (Input|SetInputModeGameandUI _returnvalue _returnvalue_2 "DoNotLock" true)
          (Variables|/Script/Engine.PlayerController|SetbShowMouseCursor _returnvalue true)
          (Input|EnableInput (Game|GetPlayerController 0))
          (Default|ShowThoughts _asmain_game_instance " " _slatefontinfo _slatecolor true 25.0 0.0 0.0 true false) ; there was a glitch where monster's thoughts would play endlessly when you delete\nfootage in loop
        )))))

(event Custom|TickScreenStatic
  (if (Variables|Default|GetFadeOutScreenStatic)
    (bind _returnvalue (Rendering|Material|GetScalarParameterValue "/Game/ModelsMaterialsTextures/GlobalMaterialParams.GlobalMaterialParams" "ScreenStatic" :!class /Script/Engine.KismetMaterialLibrary))
    (Rendering|Material|SetScalarParameterValue "/Game/ModelsMaterialsTextures/GlobalMaterialParams.GlobalMaterialParams" "ScreenStatic" (Math|Interpolation|FInterpTo _returnvalue 0.0 (Utilities|Time|GetWorldDeltaSeconds) 0.5) :!class /Script/Engine.KismetMaterialLibrary)))

(event EventTick
  (params (DeltaSeconds :type Float%20%28single-precision%29))
  (CallFunction|TickPickUpCamera)
  (CallFunction|TickScreenStatic))

(event EventBeginPlay
  (bind _asplayer_character (Utilities|Casting|CastToPlayerCharacter (Game|GetPlayerCharacter 0)))
  (Variables|Default|SetPlayerRef _asplayer_character))

(event Input|MouseEvents|LeftMouseButton
  (params (Key :type Key%20Structure :default "None"))
  ;[1 1 1] Spawn delete prompt whenever you left click
  (:Pressed
    (if (Variables|Default|GetAnyKeyMakesDeleteMessageAppear)
      (bind _returnvalue (UserInterface|CreateWidget "/Game/UI/DeletePopups/UI_FormatMemory_1st.UI_FormatMemory_1st_C"))
      (UserInterface|Viewport|AddtoViewport _returnvalue 0)
      (Variables|/Script/Engine.PlayerController|SetbShowMouseCursor (Game|GetPlayerController 0) true))))

(fn ConstructionScript)

(fn UnlockCheckpoint
  (params (CheckpointName :type String))
  (bind _returnvalue (SaveGame|LoadGamefromSlot "PlayerData"))
  (bind _asplayer_save_data (Utilities|Casting|CastToPlayerSaveData _returnvalue))
  (Utilities|Array|AddUnique (Variables|/Game/PlayerSaveData.PlayerSaveData_C|GetCheckpoints _asplayer_save_data) CheckpointName)
  (SaveGame|SaveGametoSlot _asplayer_save_data "PlayerData"))

(fn CompletelyRemoveandDisableEnemy
  (bind _playerref (Variables|Default|GetPlayerRef))
  (bind _monsterref (Variables|/Game/Blueprints/ThirdPersonBP/Blueprints/PlayerCharacter.PlayerCharacter_C|GetMonsterRef _playerref))
  (Variables|/Game/Blueprints/Monster/MonsterCharacter.MonsterCharacter_C|SetDifficulty (Variables|/Game/Blueprints/ThirdPersonBP/Blueprints/PlayerCharacter.PlayerCharacter_C|GetMonsterRef (Variables|Default|GetPlayerRef)) (Utilities|Struct|Makevar_Difficulty 2e+03 1.5785116693933588e+19 0.0 "(GLITCHChance_37_E73C82214BAB7F2F947AA7A623ECD544=0.000000,DespawnedTimeMin_52_634BC33F40C3C03546AEDCB070081242=0.000000,DespawnedTimeMax_54_74AECF2841DFFE347F97D78B6E69C2AE=60.000000,MoveGlitchIndependantly_42_C250E44047F519ABF110769D7D293B9C=False,DurrationMin_14_4A9AB6FA4F2F5378381E74A29F1B0A9A=8.000000,DurrationMax_13_BF5CB1C14CC2246EB2A910B2CCA3AC7D=20.000000,Strength_12_A692411E477FE254A01001BC29D0A3C3=0.800000,Volume_20_4A82EE5C4235D8454519CB952AD1FA7F=0.000000)" "(Radius_25_5CB97014430CB08BE3B3A98736F63799=1000.000000,MoveSpeed_35_BBBC26A24CE9EF946372A2ABABB74848=100.000000,IgnorePlayer_28_13DC21314D26AB5721E395AAA5DD0C15=False,WaitMinTime_6_0E656BA94424221B2E30B9AD05A6E1BF=2.500000,WaitMaxTime_8_0E37781B45EC9F5B9CF50D896178F248=5.000000,StopHearBuffer_12_9A97DB2844E56E0B3C9D238BA1DA0A2A=2.000000,SeePlayerDelay_32_F0DFAD42448A58399E318D94A68EE297=2.000000,LeaveAfterMin_37_33B858DF446A4138FB1811B764D033CE=0,LeaveAfterMax_39_B9560D57448B8A1B45B5DAB49ACDDE7B=1)" 0.0 (Utilities|Array|MakeArray "") 4.0 false false false))
  (Default|SwitchtoDespawned _monsterref true false)
  (Variables|/Game/Blueprints/Monster/MonsterCharacter.MonsterCharacter_C|SetCOMPLETELYDESPAWNANDDISABLEDON'TDOANYTHINGNOMATTERWHAT _monsterref true))

(fn FreezePlayer
  (Variables|/Game/Blueprints/ThirdPersonBP/Blueprints/PlayerCharacter.PlayerCharacter_C|SetLockMovement (Variables|Default|GetPlayerRef) true)
  (Input|DisableInput (Variables|Default|GetPlayerRef) (Game|GetPlayerController 0))
  (Variables|/Game/Blueprints/ThirdPersonBP/Blueprints/PlayerCharacter.PlayerCharacter_C|SetInEndingChase (Variables|Default|GetPlayerRef) false))

(fn UnlockStaticEnding
  (bind _returnvalue (SaveGame|LoadGamefromSlot "PlayerData"))
  (bind _asplayer_save_data (Utilities|Casting|CastToPlayerSaveData _returnvalue))
  (bind _output_get (LocalVariables|SetSaveData _asplayer_save_data))
  (Variables|/Game/PlayerSaveData.PlayerSaveData_C|SetUnlockedStaticEnding _output_get true)
  (SaveGame|SaveGametoSlot _output_get "PlayerData"))

(event Custom|TickPickUpCamera
  (bind _dropcameraref (Variables|Default|GetDropCameraRef))
  (bind _dropcameraref_2 (Variables|Default|GetDropCameraRef))
  (bind _playerref (Variables|Default|GetPlayerRef))
  (bind _scenecomponent (Variables|/Script/Engine.CameraActor|GetSceneComponent _dropcameraref))
  (bind _scenecomponent_2 (Variables|/Script/Engine.CameraActor|GetSceneComponent _dropcameraref_2))
  (bind _returnvalue (Transformation|GetWorldTransform _scenecomponent_2))
  (bind _returnvalue_2 (Transformation|GetWorldTransform _scenecomponent))
  (if (Variables|Default|GetInCameraDropCutscene)
    (if (Variables|Default|GetTransitionOutOfCameraDrop)
      (Variables|Default|SetCameraDropFade (Math|Interpolation|FInterpTo (Variables|Default|GetCameraDropFade) 1.0 (Utilities|Time|GetWorldDeltaSeconds) 1.5))
      (Transformation|SetWorldLocationAndRotation (Variables|/Game/Blueprints/ThirdPersonBP/Blueprints/PlayerCharacter.PlayerCharacter_C|GetPhoneMesh _playerref) (Math|Vector|Lerp(Vector) (.location _returnvalue) (Transformation|GetWorldLocation (Variables|/Game/Blueprints/ThirdPersonBP/Blueprints/PlayerCharacter.PlayerCharacter_C|GetCam-PhoneArm _playerref)) (Class|KismetMathLibrary|FInterpEaseinOut 0.0 1.0 (Variables|Default|GetCameraDropFade) 2.0)) (Math|Rotator|Lerp(Rotator) (.rotation _returnvalue) (Pawn|GetControlRotation (Game|GetPlayerController 0) :!class /Script/Engine.Controller) (Class|KismetMathLibrary|FInterpEaseinOut 0.0 1.0 (Variables|Default|GetCameraDropFade) 2.0) true) false false)
      (if (== (Variables|Default|GetCameraDropFade) 1.0)
        (Variables|Default|SetInCameraDropCutscene false))
      (else
        (Transformation|SetWorldLocationAndRotation (Variables|/Game/Blueprints/ThirdPersonBP/Blueprints/PlayerCharacter.PlayerCharacter_C|GetPhoneMesh (Variables|Default|GetPlayerRef)) (.location _returnvalue_2) (.rotation _returnvalue_2) false false)))))

(event Custom|SetCameraGlitchStrength
  (params (PlayingSoundWave :type Sound%20Wave%20Object%20Reference) (PlaybackPercent :type Float%20%28single-precision%29))
  (bind _playerref (Variables|Default|GetPlayerRef))
  (Rendering|Material|SetScalarParameterValue "/Game/ModelsMaterialsTextures/GlobalMaterialParams.GlobalMaterialParams" "GlitchStrength" (Math|Curves|GetFloatValue (Variables|Default|GetCurve_CameraDropGlitch) (* (Variables|/Script/Engine.SoundBase|GetDuration PlayingSoundWave) PlaybackPercent)) :!class /Script/Engine.KismetMaterialLibrary)
  (Variables|/Game/Blueprints/ThirdPersonBP/Blueprints/PlayerCharacter.PlayerCharacter_C|SetCurrentGlitchScale _playerref 0.0)
  (Rendering|Material|SetScalarParameterValue (Variables|/Game/Blueprints/ThirdPersonBP/Blueprints/PlayerCharacter.PlayerCharacter_C|GetVideoGlitchMat _playerref) "GlitchStrength" 0.0 :!class /Script/Engine.MaterialInstanceDynamic)
  (Rendering|Material|SetScalarParameterValue "/Game/ModelsMaterialsTextures/GlobalMaterialParams.GlobalMaterialParams" "ScreenStatic" 0.0 :!class /Script/Engine.KismetMaterialLibrary))