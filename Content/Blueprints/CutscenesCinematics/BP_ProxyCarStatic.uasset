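; Cutscene proxy car that, once activated, distorts the game by player distance and triggers the static ending at close range.
; Each tick a vector curve of distance drives screen static, glitch, black fade, flashlight brightness, audio volume, time dilation and world-sound pitch.
; Very close, it fades audio, blacks out and calls EndGame on BP_Static_Cutscene.
; UnFreezeTime stops the effect, mutes audio, sets flashlight values and enables invisible-wall collision.
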(event Custom|UnFreezeTime
  (bind _playerref (Variables|Default|GetPlayerRef))
  (Variables|Default|SetUnfrozen true)
  (Audio|Components|Audio|SetVolumeMultiplier (Variables|Default|GetAudio) 0.0 :!class /Script/Engine.AudioComponent)
  (Audio|Components|Audio|SetVolumeMultiplier (Variables|Default|GetEndlessDistortion) 0.0 :!class /Script/Engine.AudioComponent)
  (Variables|/Game/Blueprints/ThirdPersonBP/Blueprints/PlayerCharacter.PlayerCharacter_C|SetTargetFlickerBrightness _playerref 1.0)
  (Variables|/Game/Blueprints/ThirdPersonBP/Blueprints/PlayerCharacter.PlayerCharacter_C|SetLightMaxBrightness _playerref 2e+03)
  (bind _outactors (Actor|GetAllActorsOfClass "/Game/Blueprints/BP_InvisibleWall.BP_InvisibleWall_C"))
  (for _array_element _outactors
    (Collision|SetCollisionEnabled (Variables|/Game/Blueprints/BP_InvisibleWall.BP_InvisibleWall_C|GetBox _array_element) "QueryAndPhysics"))
  (Variables|/Game/Blueprints/ThirdPersonBP/Blueprints/PlayerCharacter.PlayerCharacter_C|SetHoldingShift (Variables|Default|GetPlayerRef) false))

(event EventBeginPlay
  (bind _asplayer_character (Utilities|Casting|CastToPlayerCharacter (Game|GetPlayerCharacter 0)))
  (Variables|Default|SetPlayerRef _asplayer_character))

(event EventTick
  (params (DeltaSeconds :type Float%20%28single-precision%29))
  (bind _returnvalue (Transformation|GetActorLocation))
  (bind _curve (Variables|Default|GetCurve))
  (bind _playerref (Variables|Default|GetPlayerRef))
  (bind _returnvalue_2 (Transformation|GetActorLocation _playerref))
  (bind _returnvalue_3 (- _returnvalue _returnvalue_2))
  (bind _returnvalue_4 (Math|Vector|VectorLength _returnvalue_3))
  (bind _returnvalue_5 (Math|Curves|GetVectorValue _curve _returnvalue_4))
  (if (Variables|Default|GetActivated)
    (if (not (Variables|Default|GetUnfrozen))
      (Development|PrintString (Utilities|String|ToString(Float) _returnvalue_4))
      (if (< _returnvalue_4 5e+04)
        (if (< _returnvalue_4 1.5e+03)
          (Utilities|FlowControl|DoOnce false
            (:Completed
              (Audio|Components|Audio|FadeOut (Variables|Default|GetAudio) 1.0 0.0 "Linear" :!class /Script/Engine.AudioComponent)
              (Audio|Components|Audio|FadeIn (Variables|Default|GetDistFadeOut) 0.0 1.0 0.0 "Linear" :!class /Script/Engine.AudioComponent)
              (bind _outactors (Actor|GetAllActorsOfClass "/Game/Blueprints/CutscenesCinematics/BP_Static_Cutscene.BP_Static_Cutscene_C"))
              (Default|EndGame (Utilities|Array|Get(acopy) _outactors) true false false false)
              (Rendering|Material|SetScalarParameterValue "/Game/ModelsMaterialsTextures/GlobalMaterialParams.GlobalMaterialParams" "ScreenStatic" 0.1 :!class /Script/Engine.KismetMaterialLibrary)
              (Class|PlayerCameraManager|SetManualCameraFade (Game|GetPlayerCameraManager 0) 1.0 "(R=0.000000,G=0.000000,B=0.000000,A=1.000000)" false)
              (Utilities|Time|SetGlobalTimeDilation 1.0)))
          (else
            (|SetScreenStatic/FlashlightMult (.x _returnvalue_5) (.y _returnvalue_5)
              (:execute
                (Utilities|Time|SetGlobalTimeDilation (.z _returnvalue_5))
                (Audio|SetSoundMixClassOverride "/Game/Audio/DefaultSoundMix.DefaultSoundMix" "/Game/Audio/SoundClass_WorldSounds.SoundClass_WorldSounds" 1.0 (.z _returnvalue_5) 0.0 true)))))))))

(fn ConstructionScript)