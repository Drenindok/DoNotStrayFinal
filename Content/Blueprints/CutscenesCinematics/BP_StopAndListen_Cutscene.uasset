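; Scripted first-death cutscene actor: a sunny flashback with thoughts snaps to night and the monster approaches the player.
; Once close, it locks movement and forces the player's gaze, then timed delays stage death, glitch video and the next level load.
; Audio playback percent drives glitch, rewind and post-process curves.
; With a completed first run saved, shaking the mouse can break free, stunning the monster and destroying this actor.
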(event Custom|PlayCutscene
  (bind _playerref (Variables|Default|GetPlayerRef))
  (bind _playerref_2 (Variables|Default|GetPlayerRef))
  (bind _cameralandpoint (Variables|Default|GetCameraLandPoint))
  (bind _playerref_3 (Variables|Default|GetPlayerRef))
  (bind _respawnpoint (Variables|Default|GetRespawnPoint))
  (bind _monsterref (Variables|Default|GetMonsterRef))
  (bind _playerref_4 (Variables|Default|GetPlayerRef))
  (bind _playerref_5 (Variables|Default|GetPlayerRef))
  (bind _monsterref_2 (Variables|Default|GetMonsterRef))
  (bind _returnvalue (Transformation|GetWorldTransform _cameralandpoint))
  (bind _returnvalue_2 (Transformation|GetWorldTransform _respawnpoint))
  (bind _phonemesh (Variables|/Game/Blueprints/ThirdPersonBP/Blueprints/PlayerCharacter.PlayerCharacter_C|GetPhoneMesh _playerref_2))
  (bind _returnvalue_3 (Transformation|GetWorldLocation _phonemesh))
  ;[1 1 1] Begin cutscene
  (Utilities|FlowControl|DoOnce false
    (:Completed
      (Default|SwitchtoDespawned (Variables|Default|GetMonsterRef) true false)
      (Variables|Default|SetInCutscene false)
      (Widget|SetRenderOpacity (Variables|/Game/Blueprints/ThirdPersonBP/Blueprints/PlayerCharacter.PlayerCharacter_C|GetHUDref (Variables|Default|GetPlayerRef)) 0.0)
      (Utilities|FlowControl|Delay 4.0)
      ;[1 0.614 0] Daytime flashback to when son was alive
      (Default|ForceLightOff (Variables|Default|GetPlayerRef))
      (bind _asmain_game_instance (Utilities|Casting|CastToMainGameInstance (Game|GetGameInstance)))
      (Default|ShowThoughts _asmain_game_instance "\"Don't go far from me, okay?\"[D=3] 
>She took his hand, and led him into the grass. 
>I close my eyes, and count to ten. 
>\"Ready or not, here I come!\"" (Utilities|Struct|MakeSlateFontInfo "/Game/Fonts/naomis_hand-NewFathersFont/NaomisHand-Regular_Font.NaomisHand-Regular_Font" 0 (Utilities|Struct|MakeFontOutlineSettings 2 false false 0 "(R=0.000000,G=0.000000,B=0.000000,A=1.000000)") "Regular") (Utilities|Struct|MakeSlateColor "(R=1.000000,G=1.000000,B=1.000000,A=1.000000)" "UseColor_Specified") false 25.0 0.0 0.0 true false)
      (bind _outactors (Actor|GetAllActorsOfClass "/Game/Blueprints/BP_LightingManager.BP_LightingManager_C"))
      (Utilities|IsValid (Utilities|Array|Get(acopy) _outactors)
        (:Is%20Valid
          (Default|SwitchtoSunny (Utilities|Array|Get(acopy) _outactors))
          (Utilities|FlowControl|Delay 17.0)
          ;[1 1 1] Snap back to reality with glitch effect, spawn monster
          (bind _returnvalue_4 (Audio|CreateSound2D "/Game/Audio/Glitches_CameraSounds/wav_lightFeedback.wav_lightFeedback" 1.0 1.0 0.0 0))
          (Audio|Components|Audio|Play _returnvalue_4 0.0)
          (Default|PlayGlitchEffect _playerref 2.0 0.0 0.16)
          (Variables|/Game/Blueprints/ThirdPersonBP/Blueprints/PlayerCharacter.PlayerCharacter_C|SetCurrentGlitchScale _playerref 2.0)
          (Utilities|FlowControl|Delay 0.16)
          (Variables|/Game/Blueprints/ThirdPersonBP/Blueprints/PlayerCharacter.PlayerCharacter_C|SetCurrentGlitchScale (Variables|Default|GetPlayerRef) 0.1)
          (Viewport|RemoveAllWidgets)
          (bind _outactors_2 (Actor|GetAllActorsOfClass "/Game/Blueprints/BP_LightingManager.BP_LightingManager_C"))
          (Utilities|IsValid (Utilities|Array|Get(acopy) _outactors_2)
            (:Is%20Valid
              (Default|SwitchtoNight (Utilities|Array|Get(acopy) _outactors_2))
              (Utilities|FlowControl|Delay 0.0) ; default 2
              (Audio|Components|Audio|FadeOut _returnvalue_4 2.0 0.0 "Linear" :!class /Script/Engine.AudioComponent)
              (Utilities|FlowControl|Sequence
                (:then_0
                  ;[0 1 1] Initial surprise after seeing monster
                  (Utilities|FlowControl|Delay 2.0)
                  (bind _asmain_game_instance_2 (Utilities|Casting|CastToMainGameInstance (Game|GetGameInstance)))
                  (Default|ShowThoughts _asmain_game_instance_2 "[D=2][LasD=3]Wha... 
>What is that?" (Utilities|Struct|MakeSlateFontInfo "/Game/Fonts/naomis_hand-NewFathersFont/NaomisHand-Regular_Font.NaomisHand-Regular_Font" 0 (Utilities|Struct|MakeFontOutlineSettings 2 false false 0 "(R=0.000000,G=0.000000,B=0.000000,A=1.000000)") "Regular") (Utilities|Struct|MakeSlateColor "(R=1.000000,G=1.000000,B=1.000000,A=1.000000)" "UseColor_Specified") false 25.0 0.0 0.0 true false))
                (:then_1
                  (Rendering|SetVisibility (Variables|/Game/Blueprints/Monster/MonsterCharacter.MonsterCharacter_C|GetEye (Variables|Default|GetMonsterRef)) true true)
                  (Transformation|SetActorLocationAndRotation (Variables|Default|GetMonsterRef) (.location _returnvalue_2) (.rotation _returnvalue_2) false true)
                  (Default|SetVisualEffects (Variables|Default|GetMonsterRef) true 0.0 0.0 0.0 1.0 0.0 75.0 -1.0 false "(R=1.000000,G=1.000000,B=1.000000,A=1.000000)")
                  (Variables|/Script/Engine.CharacterMovementComponent|SetMaxWalkSpeed (Variables|/Script/Engine.Character|GetCharacterMovement (Variables|Default|GetMonsterRef)) 1e+02)
                  (AI|AIMoveTo _monsterref_2 _monsterref_2 (Transformation|GetActorLocation _playerref_4) _playerref_4 1.5e+03 false
                    (:OnSuccess
                      (Utilities|Time|ClearTimerbyFunctionName 0 "Step")
                      (Utilities|FlowControl|DoOnce false
                        (:Completed
                          (Default|ForceStopGlitchEffect _playerref_3)
                          (Variables|/Game/Blueprints/ThirdPersonBP/Blueprints/PlayerCharacter.PlayerCharacter_C|SetForceLookAtMonster _playerref_3 true)
                          (Default|ForceLightOff _playerref_3)
                          (Variables|Default|SetRiseUp true)
                          (Variables|/Game/Blueprints/ThirdPersonBP/Blueprints/PlayerCharacter.PlayerCharacter_C|SetLockMovement (Variables|Default|GetPlayerRef) true)
                          (AI|Navigation|StopMovement (Pawn|GetController (Variables|Default|GetMonsterRef)))
                          (Variables|/Game/Blueprints/Monster/MonsterCharacter.MonsterCharacter_C|SetBehaviourState _monsterref "KillCutscene")
                          (Audio|Components|Audio|SetVolumeMultiplier (Variables|/Game/Blueprints/Monster/MonsterCharacter.MonsterCharacter_C|Getaudio_breathing _monsterref) 0.0 :!class /Script/Engine.AudioComponent)
                          (Utilities|FlowControl|Sequence
                            (:then_0
                              ;[1 0 0] Shake mouse to look away from light
                              ;;[1 1 1] Activate option to break free from light if you have beat the game already (disabled for demo!)
                              (bind _returnvalue_5 (SaveGame|LoadGamefromSlot "PlayerData"))
                              (bind _asplayer_save_data (Utilities|Casting|CastToSave_PlayerData _returnvalue_5))
                              (if (Variables|/Game/Save_PlayerData.Save_PlayerData_C|GetUnlockedFirstRunCompleted _asplayer_save_data)
                                (bind _returnvalue_6 (UserInterface|CreateWidget "/Game/UI/UI_ThoughtText.UI_ThoughtText_C" 0 "(Shake mouse to look away)" 15.0 6.0 5.0 0.0 "(X=960.000000,Y=800.000000)" "Center" (Utilities|Struct|MakeSlateColor "(R=1.000000,G=0.000000,B=0.000000,A=1.000000)") (Utilities|Struct|MakeSlateFontInfo "/Engine/EngineFonts/Roboto.Roboto" 0 (Utilities|Struct|MakeFontOutlineSettings 2 false false 0 "(R=0.000000,G=0.000000,B=0.000000,A=1.000000)") "Regular")))
                                (bind _output_get (Variables|Default|SetShakeToLookAwayPrompt _returnvalue_6))
                                (UserInterface|Viewport|AddtoViewport _output_get 0)
                                (Variables|Default|SetInputMouseShake true)
                                (Input|EnableInput (Game|GetPlayerController 0))
                                (Utilities|FlowControl|Delay 15.0)
                                (Variables|Default|SetInputMouseShake false) ; stops you from excaping if you stare for too long\n(Fixes being able to "escape" after death)
                              ))
                            (:then_1
                              (bind _returnvalue_7 (Audio|CreateSound2D "/Game/Audio/Cutscenes/wav_Cutscene_FirstDeath_NoKillSound.wav_Cutscene_FirstDeath_NoKillSound" 0.001 1.0 0.0 0))
                              (bind _output_get_2 (Variables|Default|SetCutsceneSound _returnvalue_7))
                              (EventDispatchers|BindEventtoOnAudioPlaybackPercent _output_get_2 (delegate Custom|SetCameraGlitchStrength))
                              (Audio|Components|Audio|Play _output_get_2 0.0)
                              (bind _asmain_game_instance_3 (Utilities|Casting|CastToMainGameInstance (Game|GetGameInstance)))
                              (Default|PlayPersistentAudio _asmain_game_instance_3 "/Game/Audio/Cutscenes/wav_Cutscene_FirstDeath_NoKillSound.wav_Cutscene_FirstDeath_NoKillSound" 0.0 1.0 0.0)
                              (bind _returnvalue_8 (CameraShakes|StartCameraShake (Game|GetPlayerCameraManager 0) "/Game/CameraShakes_Anims/shake_panic.shake_panic_C" 1.0 "CameraLocal" "0, 0, 0"))
                              (Variables|Default|SetCutsceneCameraShake _returnvalue_8)
                              (Utilities|FlowControl|Sequence
                                (:then_0
                                  (Utilities|FlowControl|Delay 18.23) ; 18:64 is where player explodes in sound effect
                                  (CameraFades|StartCameraFade (Game|GetPlayerCameraManager 0) 0.0 0.5 0.409999 "(R=1.000000,G=1.000000,B=1.000000,A=1.000000)" false false))
                                (:then_1
                                  (Utilities|FlowControl|Delay 18.639999) ; 18:64 is where player explodes in sound effect
                                  (bind _asmain_game_instance_4 (Utilities|Casting|CastToMainGameInstance (Game|GetGameInstance)))
                                  (Default|ClearThoughts _asmain_game_instance_4 false)
                                  (Variables|/Game/Blueprints/ThirdPersonBP/Blueprints/PlayerCharacter.PlayerCharacter_C|SetLightMaxBrightness (Variables|Default|GetPlayerRef) 1e+05)
                                  ;[1 1 1] Old "Kill and skip to on ground" thing
                                  (CallFunction|SpawnBloodPuddle)
                                  (Default|KillPlayer (Variables|Default|GetPlayerRef) true true)
                                  (Rendering|Material|SetScalarParameterValue (Variables|/Game/Blueprints/ThirdPersonBP/Blueprints/PlayerCharacter.PlayerCharacter_C|GetScreenBloodMat (Variables|Default|GetPlayerRef)) "BloodAmount" 0.0 :!class /Script/Engine.MaterialInstanceDynamic)
                                  (Variables|/Script/Engine.CameraComponent|SetPostProcessSettings (Variables|/Game/Blueprints/ThirdPersonBP/Blueprints/PlayerCharacter.PlayerCharacter_C|GetCamera (Variables|Default|GetPlayerRef)) (Utilities|Struct|MakePostProcessSettings 1e+02 1e-05 4.0 (Utilities|Struct|MakeWeightedBlendables (Utilities|Array|MakeArray (Utilities|Struct|MakeWeightedBlendable 1.0 (Variables|/Game/Blueprints/ThirdPersonBP/Blueprints/PlayerCharacter.PlayerCharacter_C|GetGlitchMat _playerref_5)) (Utilities|Struct|MakeWeightedBlendable 1.0 (Variables|/Game/Blueprints/ThirdPersonBP/Blueprints/PlayerCharacter.PlayerCharacter_C|GetScreenBloodMat _playerref_5)) (Utilities|Struct|MakeWeightedBlendable 1.0 (Variables|/Game/Blueprints/ThirdPersonBP/Blueprints/PlayerCharacter.PlayerCharacter_C|GetInvertColorsMat _playerref_5))))))
                                  (Variables|/Game/Blueprints/ThirdPersonBP/Blueprints/PlayerCharacter.PlayerCharacter_C|SetForceLookAtMonster (Variables|Default|GetPlayerRef) false)
                                  ;[1 1 1] Old "skip to dead on ground"
                                  (Default|SwitchtoDespawned (Variables|Default|GetMonsterRef) true false)
                                  (Default|ForceLighton (Variables|Default|GetPlayerRef))
                                  (Physics|SetSimulatePhysics _phonemesh false)
                                  (bind (_outhit _returnvalue_9) (Collision|LineTraceByChannel _returnvalue_3 (- _returnvalue_3 "0, 0,10000.000000") "TraceTypeQuery3" false 0 "None"))
                                  (if _returnvalue_9
                                    (Transformation|SetWorldLocationAndRotation _phonemesh (+ (.ImpactPoint (Collision|BreakHitResult _outhit)) "0, 0,10.000000") (Math|Rotator|MakeRotator 9e+01 0.0 (.yaw (Transformation|GetWorldRotation _phonemesh))) false true) ; teleport to on the ground after dropping, but always facing up
                                    (else
                                      (Transformation|SetWorldLocationAndRotation _phonemesh (.location _returnvalue) (.rotation _returnvalue) false false) ; teleport to path as a backup
                                    )))
                                (:then_2
                                  (Utilities|FlowControl|Delay 19.17) ; 18:85 is where screen freezes after death
                                  (Class|PlayerCameraManager|SetManualCameraFade :self (Game|GetPlayerCameraManager 0) :InFadeAmount 1.0)
                                  (bind _returnvalue_10 (UserInterface|CreateWidget "/Game/UI/UI_FirstDeathGlitchVideo.UI_FirstDeathGlitchVideo_C"))
                                  (UserInterface|Viewport|AddtoViewport _returnvalue_10 0))
                                (:then_3
                                  ;[1 1 1] LoadNextLevelWithTransition
                                  (Utilities|FlowControl|Delay 20.25)
                                  (Class|PlayerCameraManager|SetManualCameraFade :self (Game|GetPlayerCameraManager 0) :InFadeAmount 1.0)
                                  (Viewport|RemoveAllWidgets)
                                  (Utilities|FlowControl|Delay 0.0)
                                  (Game|OpenLevel(byName) "Level_2ndGlitchyRun"))
                                (:then_4
                                  ;[0 1 1] Thoughts when you see monster for first time
                                  (Utilities|FlowControl|Delay 3.0)
                                  (bind _asmain_game_instance_5 (Utilities|Casting|CastToMainGameInstance (Game|GetGameInstance)))
                                  (Default|ShowThoughts _asmain_game_instance_5 "[D=2][LasD=2]It's you... 
>I found you. 
>I'm not crazy. 
>I knew I wasn't crazy. 
~Will you take me to him? 
>Will you grant me his fate? 
>Please?" (Utilities|Struct|MakeSlateFontInfo "/Game/Fonts/naomis_hand-NewFathersFont/NaomisHand-Regular_Font.NaomisHand-Regular_Font" 0 (Utilities|Struct|MakeFontOutlineSettings 2 false false 0 "(R=0.000000,G=0.000000,B=0.000000,A=1.000000)") "Regular") (Utilities|Struct|MakeSlateColor "(R=1.000000,G=1.000000,B=1.000000,A=1.000000)" "UseColor_Specified") false 25.0 0.0 5.0 false false))))))))))))))))))

(event Custom|SetCameraGlitchStrength
  (params (PlayingSoundWave :type Sound%20Wave%20Object%20Reference) (PlaybackPercent :type Float%20%28single-precision%29))
  (bind _duration (Variables|/Script/Engine.SoundBase|GetDuration PlayingSoundWave))
  (bind _playerref (Variables|Default|GetPlayerRef))
  (bind _returnvalue (* _duration PlaybackPercent))
  (bind _camera (Variables|/Game/Blueprints/ThirdPersonBP/Blueprints/PlayerCharacter.PlayerCharacter_C|GetCamera _playerref))
  ;[1 1 1] Update camera effects based on time in cutscene
  (Rendering|Material|SetScalarParameterValue "/Game/ModelsMaterialsTextures/GlobalMaterialParams.GlobalMaterialParams" "GlitchStrength" (Math|Curves|GetFloatValue (Variables|Default|GetCameraGlitchCurve) _returnvalue) :!class /Script/Engine.KismetMaterialLibrary)
  (Rendering|Material|SetScalarParameterValue "/Game/ModelsMaterialsTextures/GlobalMaterialParams.GlobalMaterialParams" "RewindDistortionIntensity" (Math|Curves|GetFloatValue (Variables|Default|GetCurveRewindDist) _returnvalue) :!class /Script/Engine.KismetMaterialLibrary)
  (Variables|/Script/Engine.CameraComponent|SetPostProcessSettings _camera (Utilities|Struct|MakePostProcessSettings (Math|Curves|GetFloatValue (Variables|Default|GetCurveMonsterLightBrightness) _returnvalue) (Utilities|Struct|BreakPostProcessSettings (Variables|/Script/Engine.CameraComponent|GetPostProcessSettings _camera))))
  (Rendering|Material|SetScalarParameterValue (Variables|/Game/Blueprints/ThirdPersonBP/Blueprints/PlayerCharacter.PlayerCharacter_C|GetVideoGlitchMat _playerref) "VideoOpacity" 1.0 :!class /Script/Engine.MaterialInstanceDynamic))

(event Custom|SpawnLightMonster
  (bind _respawnpoint (Variables|Default|GetRespawnPoint))
  (bind _returnvalue (Transformation|GetWorldTransform _respawnpoint))
  ;[1 1 1] Spawn monster (I think this is outdated and not in use)
  (Utilities|FlowControl|Delay 5.0)
  (Default|PlayGlitchEffect (Variables|Default|GetPlayerRef) 1.0 1.0 16.0)
  (Rendering|SetVisibility (Variables|/Game/Blueprints/Monster/MonsterCharacter.MonsterCharacter_C|GetEye (Variables|Default|GetMonsterRef)) true true)
  (Transformation|SetActorLocationAndRotation (Variables|Default|GetMonsterRef) (.location _returnvalue) (.rotation _returnvalue) false true)
  (Default|SwitchtoInvestigate (Variables|Default|GetMonsterRef) false)
  (AI|AIMoveTo (Variables|Default|GetMonsterRef) (Transformation|GetActorLocation (Variables|Default|GetPlayerRef)) 0 25.0 false) ; use this INSTEAD OF PATROL TO because investigate \npoint can UPDATE if monster continuously hears the player
)

(event EventBeginPlay
  ;[1 1 1] Set references to player and monster
  (bind _asplayer_character (Utilities|Casting|CastToPlayerCharacter (Game|GetPlayerCharacter 0)))
  (Variables|Default|SetPlayerRef _asplayer_character)
  (bind _outactors (Actor|GetAllActorsOfClass "/Game/Blueprints/Monster/MonsterCharacter.MonsterCharacter_C"))
  (Variables|Default|SetMonsterRef (Utilities|Array|Get(acopy) _outactors)))

(event EventTick
  (params (DeltaSeconds :type Float%20%28single-precision%29))
  (bind _playerref (Variables|Default|GetPlayerRef))
  ;[1 0 0] Shake mouse to look away from light
  ;;[1 1 1] Calculate mouse shake amount
  (if (Variables|Default|GetInputMouseShake)
    (bind _output_get (Variables|Default|SetMouseShakeAmount (+ (Variables|Default|GetMouseShakeAmount) (* (Math|Float|Clamp(Float) (+ (Math|Float|Absolute(Float) (Class|Actor|GetInputAxisKeyValue)) (Math|Float|Absolute(Float) (Class|Actor|GetInputAxisKeyValue)))) (Utilities|Time|GetWorldDeltaSeconds) 0.333))))
    (if (> _output_get 1.0)
      ;;[1 1 1] After you have shaken mouse enough, break free from light
      (|BreakFreeFromLight
        (:execute
          (Widget|RemovefromParent (Variables|Default|GetShakeToLookAwayPrompt))
          (Actor|DestroyActor) ; stops cutscene from continuting
          (Default|PlayGlitchEffect _playerref 1.0 0.0 11.349985)
          (Variables|/Game/Blueprints/ThirdPersonBP/Blueprints/PlayerCharacter.PlayerCharacter_C|SetPanicStrength _playerref 0.0)
          (CameraShakes|StopCameraShake (Game|GetPlayerCameraManager 0) (Variables|Default|GetCutsceneCameraShake) true)
          (Default|ShowBreakFreefromLightMessage (Variables|Default|GetPlayerRef)))))))

(fn ConstructionScript)

(fn SpawnBloodPuddle
  (bind _returnvalue (Math|Random|RandomFloatinRange -1e+02 -5e+01))
  (for _array_element (Variables|Default|GetBloodDecalLocations)
    (bind _returnvalue_2 (Rendering|Material|CreateDynamicMaterialInstance "/Game/ModelsMaterialsTextures/Materials/Blood/Mat_Decal_Blood.Mat_Decal_Blood" "None" "None" :!class /Script/Engine.KismetMaterialLibrary))
    (Rendering|Material|SetScalarParameterValue _returnvalue_2 "Frame" (Math|Conversions|ToFloat(Integer) (Math|Random|RandomInteger 5)) :!class /Script/Engine.MaterialInstanceDynamic)
    (Rendering|Decal|SpawnDecalatLocation _returnvalue_2 (Math|Vector|MakeVector _returnvalue _returnvalue _returnvalue) _array_element (Math|Conversions|RotationFromXVector "0, 0,1.000000") 1e+02)))