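; Stop-and-listen cutscene actor for the second run: a hospital flashback with thought text that snaps to night as the monster approaches and holds the player's gaze.
; PlayCutscene runs the timed fades, audio and AI move in parallel, then enables mouse-shake escape.
; Tick turns accumulated, decaying mouse motion into glitch, camera shake and sound intensity.
; At full shake, BreakFreeFromLight restores control and stuns the monster, and Tick later removes the trail blocker.
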(event Custom|PlayCutscene
  (bind _playerref (Variables|Default|GetPlayerRef))
  (bind _respawnpoint (Variables|Default|GetRespawnPoint))
  (bind _monsterref (Variables|Default|GetMonsterRef))
  (bind _playerref_2 (Variables|Default|GetPlayerRef))
  (bind _monsterref_2 (Variables|Default|GetMonsterRef))
  (bind _returnvalue (Transformation|GetWorldTransform _respawnpoint))
  ;[1 1 1] Begin cutscene
  (Utilities|FlowControl|DoOnce false
    (:Completed
      (Default|SwitchtoDespawned (Variables|Default|GetMonsterRef) true false)
      (Variables|Default|SetInCutscene false)
      (Widget|SetRenderOpacity (Variables|/Game/Blueprints/ThirdPersonBP/Blueprints/PlayerCharacter.PlayerCharacter_C|GetHUDref (Variables|Default|GetPlayerRef)) 0.0)
      (Audio|Components|Audio|FadeOut (Variables|/Script/Engine.AmbientSound|GetAudioComponent (Utilities|ResolveSoftReference (Variables|Default|GetRepressedAmbience))) 6.0 0.0 "Linear" :!class /Script/Engine.AudioComponent)
      (bind _returnvalue_2 (Audio|SpawnSound2D "/Game/Audio/Ambient/wav_HospitalRoom.wav_HospitalRoom" 1.0 1.0 0.0 0))
      (Audio|Components|Audio|FadeIn _returnvalue_2 6.0 1.0 0.0 "Linear" :!class /Script/Engine.AudioComponent)
      (Variables|Default|SetHospitalRoomSound _returnvalue_2)
      (Utilities|FlowControl|Sequence
        (:then_0
          ;[1 0.614 0] Daytime flashback to when son was alive
          (bind _fade (Timeline|FadeScreenOutTimeline Play)
            (:Update
              (Rendering|Material|SetVectorParameterValue "/Game/ModelsMaterialsTextures/GlobalMaterialParams.GlobalMaterialParams" "RepressedOutlineColor" (Utilities|Struct|MakeLinearColor 0.5 0.5 0.5 _fade) :!class /Script/Engine.KismetMaterialLibrary))
            (:Finished
              (Utilities|FlowControl|Delay 7.0)
              (bind _asmain_game_instance (Utilities|Casting|CastToMainGameInstance (Game|GetGameInstance)))
              (Default|ShowThoughts _asmain_game_instance "\"Austin...\"[D=3] 
>\"It's going to be okay...\" 
>\"We can still be happy together...\" 
>\"Right?\"" (Utilities|Struct|MakeSlateFontInfo "/Game/Fonts/naomis_hand-NewFathersFont/NaomisHand-Regular_Font.NaomisHand-Regular_Font" 0 (Utilities|Struct|MakeFontOutlineSettings 2 false false 0 "(R=0.000000,G=0.000000,B=0.000000,A=1.000000)") "Regular") (Utilities|Struct|MakeSlateColor "(R=1.000000,G=1.000000,B=1.000000,A=1.000000)" "UseColor_Specified") false 25.0 0.0 0.0 true false)
              (Utilities|FlowControl|Delay 14.0)
              ;[1 1 1] Snap back to reality with glitch effect, spawn monster
              (Variables|/Game/Blueprints/ThirdPersonBP/Blueprints/PlayerCharacter.PlayerCharacter_C|SetCurrentGlitchScale (Variables|Default|GetPlayerRef) 0.1)
              (Utilities|Time|SetGlobalTimeDilation 0.5)
              (Utilities|FlowControl|Delay 0.16)
              (bind _returnvalue_3 (Actor|GetActorOfClass "/Game/Blueprints/BP_LightingManager.BP_LightingManager_C"))
              (Utilities|IsValid _returnvalue_3
                (:Is%20Valid
                  (Default|SwitchtoNight _returnvalue_3)
                  (Audio|SetSoundMixClassOverride "/Game/Audio/DefaultSoundMix.DefaultSoundMix" "/Game/Audio/SoundClass_WorldSounds.SoundClass_WorldSounds" 0.0 1.0 0.0 true)
                  (Audio|SetSoundMixClassOverride "/Game/Audio/DefaultSoundMix.DefaultSoundMix" "/Game/Audio/SoundClass_NightOnlySound.SoundClass_NightOnlySound" 0.0 1.0 0.0 true)
                  ;[1 0 0] Shake mouse to look away from light
                  ;;[1 1 1] Activate option to break free from light if you have beat the game already (disabled for demo!)
                  (Variables|Default|SetInputMouseShake true)
                  (Audio|Components|Audio|Play (Variables|Default|GetFuzzinessSound) 0.0)
                  (bind _returnvalue_4 (CameraShakes|StartCameraShake (Game|GetPlayerCameraManager 0) "/Game/CameraShakes_Anims/shake_LookAwayShake.shake_LookAwayShake_C" 1.0 "World" "0, 0, 0"))
                  (Variables|Default|SetLookAwayShake _returnvalue_4))))))
        (:then_1
          (Utilities|FlowControl|Delay 6.0)
          (bind _returnvalue_5 (Audio|SpawnSound2D "/Game/Audio/Cutscenes/wav_HeartMonitor.wav_HeartMonitor" 1.0 1.0 0.0 0))
          (Audio|Components|Audio|FadeIn _returnvalue_5 3.0 1.0 0.0 "Linear" :!class /Script/Engine.AudioComponent)
          (Variables|Default|SetHeartMonitorSound _returnvalue_5)
          (Rendering|SetVisibility (Variables|/Game/Blueprints/Monster/MonsterCharacter.MonsterCharacter_C|GetEye (Variables|Default|GetMonsterRef)) true true)
          (Transformation|SetActorLocationAndRotation (Variables|Default|GetMonsterRef) (.location _returnvalue) (.rotation _returnvalue) false true)
          (Default|SetVisualEffects (Variables|Default|GetMonsterRef) true 0.0 0.0 0.0 1.0 0.0 75.0 -1.0 false "(R=1.000000,G=1.000000,B=1.000000,A=1.000000)")
          (Variables|/Script/Engine.CharacterMovementComponent|SetMaxWalkSpeed (Variables|/Script/Engine.Character|GetCharacterMovement (Variables|Default|GetMonsterRef)) 1e+02)
          (AI|AIMoveTo _monsterref_2 _monsterref_2 (Transformation|GetActorLocation _playerref_2) _playerref_2 1.5e+03 false
            (:OnSuccess
              (Utilities|Time|ClearTimerbyFunctionName 0 "Step")
              (Utilities|FlowControl|DoOnce false
                (:Completed
                  (Default|ForceStopGlitchEffect _playerref)
                  (Variables|/Game/Blueprints/ThirdPersonBP/Blueprints/PlayerCharacter.PlayerCharacter_C|SetForceLookAtMonster _playerref true)
                  (Default|ForceLightOff _playerref)
                  (Variables|Default|SetRiseUp true)
                  (Variables|/Game/Blueprints/ThirdPersonBP/Blueprints/PlayerCharacter.PlayerCharacter_C|SetLockMovement (Variables|Default|GetPlayerRef) true)
                  (AI|Navigation|StopMovement (Pawn|GetController (Variables|Default|GetMonsterRef)))
                  (Variables|/Game/Blueprints/Monster/MonsterCharacter.MonsterCharacter_C|SetBehaviourState _monsterref "KillCutscene")
                  (Audio|Components|Audio|SetVolumeMultiplier (Variables|/Game/Blueprints/Monster/MonsterCharacter.MonsterCharacter_C|Getaudio_breathing _monsterref) 0.0 :!class /Script/Engine.AudioComponent)
                  (Rendering|Material|SetScalarParameterValue "/Game/ModelsMaterialsTextures/GlobalMaterialParams.GlobalMaterialParams" "GlitchStrength" 1.0 :!class /Script/Engine.KismetMaterialLibrary))))))))))

(event Custom|SetCameraGlitchStrength
  (params (PlayingSoundWave :type Sound%20Wave%20Object%20Reference) (PlaybackPercent :type Float%20%28single-precision%29))
  (bind _duration (Variables|/Script/Engine.SoundBase|GetDuration PlayingSoundWave))
  (bind _playerref (Variables|Default|GetPlayerRef))
  (bind _returnvalue (* _duration PlaybackPercent))
  (bind _camera (Variables|/Game/Blueprints/ThirdPersonBP/Blueprints/PlayerCharacter.PlayerCharacter_C|GetCamera _playerref))
  ;[1 1 1] Update camera effects based on time in cutscene
  (Rendering|Material|SetScalarParameterValue "/Game/ModelsMaterialsTextures/GlobalMaterialParams.GlobalMaterialParams" "GlitchStrength" (Math|Curves|GetFloatValue (Variables|Default|GetCameraGlitchCurve) _returnvalue) :!class /Script/Engine.KismetMaterialLibrary)
  (Rendering|Material|SetScalarParameterValue "/Game/ModelsMaterialsTextures/GlobalMaterialParams.GlobalMaterialParams" "RewindDistortionIntensity" (Math|Curves|GetFloatValue (Variables|Default|GetCurveRewindDist) _returnvalue) :!class /Script/Engine.KismetMaterialLibrary)
  (Variables|/Script/Engine.CameraComponent|SetPostProcessSettings _camera (Utilities|Struct|MakePostProcessSettings (Math|Curves|GetFloatValue (Variables|Default|GetCurveMonsterLightBrightness) _returnvalue) (Utilities|Struct|BreakPostProcessSettings (Variables|/Script/Engine.CameraComponent|GetPostProcessSettings _camera))))
  (Rendering|Material|SetScalarParameterValue (Variables|/Game/Blueprints/ThirdPersonBP/Blueprints/PlayerCharacter.PlayerCharacter_C|GetVideoGlitchMat _playerref) "VideoOpacity" 1.0 :!class /Script/Engine.MaterialInstanceDynamic))

(event Custom|SpawnLightMonster
  (bind _respawnpoint (Variables|Default|GetRespawnPoint))
  (bind _returnvalue (Transformation|GetWorldTransform _respawnpoint))
  ;[1 1 1] Spawn monster (I think this is outdated and not in use)
  (Utilities|FlowControl|Delay 5.0)
  (Default|PlayGlitchEffect (Variables|Default|GetPlayerRef) 1.0 1.0 16.0)
  (Rendering|SetVisibility (Variables|/Game/Blueprints/Monster/MonsterCharacter.MonsterCharacter_C|GetEye (Variables|Default|GetMonsterRef)) true true)
  (Transformation|SetActorLocationAndRotation (Variables|Default|GetMonsterRef) (.location _returnvalue) (.rotation _returnvalue) false true)
  (Default|SwitchtoInvestigate (Variables|Default|GetMonsterRef) false)
  (AI|AIMoveTo (Variables|Default|GetMonsterRef) (Transformation|GetActorLocation (Variables|Default|GetPlayerRef)) 0 25.0 false) ; use this INSTEAD OF PATROL TO because investigate \npoint can UPDATE if monster continuously hears the player
)

(event EventBeginPlay
  ;[1 1 1] Set references to player and monster
  (bind _asplayer_character (Utilities|Casting|CastToPlayerCharacter (Game|GetPlayerCharacter 0)))
  (Variables|Default|SetPlayerRef _asplayer_character)
  (bind _outactors (Actor|GetAllActorsOfClass "/Game/Blueprints/Monster/MonsterCharacter.MonsterCharacter_C"))
  (Variables|Default|SetMonsterRef (Utilities|Array|Get(acopy) _outactors)))

(event EventTick
  (params (DeltaSeconds :type Float%20%28single-precision%29))
  (bind _returnvalue (Game|GetPlayerController 0))
  (bind _returnvalue_2 (Utilities|Time|GetWorldDeltaSeconds))
  (bind _playerref (Variables|Default|GetPlayerRef))
  (bind _fuzzinesssound (Variables|Default|GetFuzzinessSound))
  (bind (_deltax _deltay) (Class|PlayerController|GetInputMouseDelta _returnvalue))
  (if (Variables|Default|GetInputMouseShake)
    (bind _output_get (Variables|Default|SetMouseShakeAmount (Math|Float|Clamp(Float) (+ (Variables|Default|GetMouseShakeAmount) (* (Math|Float|Clamp(Float) (+ (Math|Float|Absolute(Float) _deltax) (Math|Float|Absolute(Float) _deltay))) _returnvalue_2 0.4995) (* _returnvalue_2 -0.333)))))
    (Variables|/Script/Engine.CameraShakeBase|SetShakeScale (Variables|Default|GetLookAwayShake) _output_get)
    ;[1 0 0] Shake mouse to look away from light
    (Variables|/Game/Blueprints/ThirdPersonBP/Blueprints/PlayerCharacter.PlayerCharacter_C|SetCurrentGlitchScale (Variables|Default|GetPlayerRef) (Math|Float|Lerp 0.1 2.0 _output_get))
    ;;[1 1 1] Calculate mouse shake amount
    (Audio|Components|Audio|SetPitchMultiplier _fuzzinesssound (Math|Float|Clamp(Float) _output_get 0.001))
    (Audio|Components|Audio|SetVolumeMultiplier _fuzzinesssound (Math|Float|Clamp(Float) _output_get 0.001) :!class /Script/Engine.AudioComponent)
    (Audio|SetSoundMixClassOverride "/Game/Audio/DefaultSoundMix.DefaultSoundMix" "/Game/Audio/SoundClass_WorldSounds.SoundClass_WorldSounds" _output_get _output_get 0.0 true)
    (Audio|SetSoundMixClassOverride "/Game/Audio/DefaultSoundMix.DefaultSoundMix" "/Game/Audio/SoundClass_NightOnlySound.SoundClass_NightOnlySound" _output_get _output_get 0.0 true)
    (if (== _output_get 1.0)
      ;;[1 1 1] After you have shaken mouse enough, break free from light
      (|BreakFreeFromLight
        (:execute
          (Default|PlayGlitchEffect _playerref 1.0 0.0 11.349985)
          (Variables|/Game/Blueprints/ThirdPersonBP/Blueprints/PlayerCharacter.PlayerCharacter_C|SetPanicStrength _playerref 0.0)
          (CameraShakes|StopCameraShake (Game|GetPlayerCameraManager 0) (Variables|Default|GetCutsceneCameraShake) true)
          (Audio|Components|Audio|Stop (Variables|Default|GetHeartMonitorSound))
          (bind _returnvalue_3 (Audio|SpawnSound2D "/Game/Audio/Cutscenes/wav_HeartMonitor_Flatline.wav_HeartMonitor_Flatline" 1.0 1.0 0.0 0))
          (Variables|Default|SetFlatlineSound _returnvalue_3)
          (Utilities|Time|SetGlobalTimeDilation 1.0)
          (Variables|Default|SetInputMouseShake false)
          (Variables|/Script/Engine.CameraShakeBase|SetShakeScale (Variables|Default|GetLookAwayShake) 0.0)
          (Utilities|FlowControl|Delay 11.349985)
          (Audio|Components|Audio|Stop (Variables|Default|GetFuzzinessSound))
          (Variables|/Game/Blueprints/ThirdPersonBP/Blueprints/PlayerCharacter.PlayerCharacter_C|SetCurrentGlitchScale (Variables|Default|GetPlayerRef) 0.0)
          (Utilities|FlowControl|Delay 1.43)
          (Audio|Components|Audio|Stop (Variables|Default|GetFlatlineSound))
          (Actor|DestroyActor (Utilities|ResolveSoftReference (Variables|Default|GetWall%20Blocking%202nd%20half%20of%20trail))))))))

(fn ConstructionScript)

(fn SpawnBloodPuddle
  (bind _returnvalue (Math|Random|RandomFloatinRange -1e+02 -5e+01))
  (for _array_element (Variables|Default|GetBloodDecalLocations)
    (bind _returnvalue_2 (Rendering|Material|CreateDynamicMaterialInstance "/Game/ModelsMaterialsTextures/Materials/Blood/Mat_Decal_Blood.Mat_Decal_Blood" "None" "None" :!class /Script/Engine.KismetMaterialLibrary))
    (Rendering|Material|SetScalarParameterValue _returnvalue_2 "Frame" (Math|Conversions|ToFloat(Integer) (Math|Random|RandomInteger 5)) :!class /Script/Engine.MaterialInstanceDynamic)
    (Rendering|Decal|SpawnDecalatLocation _returnvalue_2 (Math|Vector|MakeVector _returnvalue _returnvalue _returnvalue) _array_element (Math|Conversions|RotationFromXVector "0, 0,1.000000") 1e+02)))