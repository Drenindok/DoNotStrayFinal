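; Procedural bridge generator that builds a bridge of instanced meshes along BridgeSpline in the construction script.
; SpawnBridgePieces alternates long and short pieces, picking variants and 180-degree flips from the Seed stream, which the Update toggle re-randomizes.
; Accumulated yaw change between pieces, scaled by Uwghewiugh, shifts spacing along the spline to compensate for turns.
; SpawnPosts adds random post pairs either side at each step and after the last piece.
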(fn ConstructionScript
  (if (Variables|Default|GetUpdate)
    (Variables|Default|SetUpdate false)
    (Class|KismetMathLibrary|SeedRandomStream (Variables|Default|GetSeed)))
  (Utilities|FlowControl|Sequence
    (:then_0
      (CallFunction|SpawnBridgePieces))))

(fn SpawnBridgePieces
  (bind _bridgespline (Variables|Default|GetBridgeSpline))
  (bind _seed (Variables|Default|GetSeed))
  (bind _returnvalue (Math|Random|RandomIntegerinRangefromStream 0 2 _seed))
  (Utilities|Array|Clear (Variables|Default|GetPrevious%20Piece%20Angle%20Array))
  (Variables|Default|SetPrevious%20Piece%20Angle "0,180.000000, 0")
  (Variables|Default|SetTurning%20Distance%20Compensation 0.0)
  (Components|InstancedStaticMesh|ClearInstances (Variables|Default|GetShortPiece1))
  (bind _index (Utilities|FlowControl|ForLoopwithBreak 0 (Math|Float|Truncate (- (/ (Spline|GetSplineLength (Variables|Default|GetBridgeSpline)) (Variables|Default|GetDistanceBetweenPieces)) 1.0)) :!label _label)
    (:LoopBody
      (Variables|Default|SetTurning%20Distance%20Compensation (+ (Variables|Default|GetTurning%20Distance%20Compensation) (Math|Float|Absolute(Float) (.Yaw (Math|Rotator|BreakRotator (Math|Rotator|CombineRotators (Math|Rotator|CombineRotators (Math|Rotator|FindLookatRotation (Spline|GetLocationatDistanceAlongSpline _bridgespline (+ (* _index (Variables|Default|GetDistanceBetweenPieces)) (* (Variables|Default|GetTurning%20Distance%20Compensation) (Variables|Default|Getuwghewiugh))) "Local") (Spline|GetLocationatDistanceAlongSpline _bridgespline (+ (+ (* _index (Variables|Default|GetDistanceBetweenPieces)) (* (Variables|Default|GetTurning%20Distance%20Compensation) (Variables|Default|Getuwghewiugh))) (Variables|Default|GetDistanceBetweenPieces)) "Local")) "0,90.000000, 0") (* (Variables|Default|GetPrevious%20Piece%20Angle) -1.0)))))))
      (if (< (Spline|GetSplineLength (Variables|Default|GetBridgeSpline)) (+ (* _index (Variables|Default|GetDistanceBetweenPieces)) (* (Variables|Default|GetTurning%20Distance%20Compensation) (Variables|Default|Getuwghewiugh))))
        (goto _label Break)
        (else
          (Utilities|FlowControl|FlipFlop
            (:A
              (switch int _returnvalue
                (:0
                  (Components|InstancedStaticMesh|AddInstance (Variables|Default|GetLongPiece1) (Math|Transform|MakeTransform (* (+ (Spline|GetLocationatDistanceAlongSpline _bridgespline (+ (* _index (Variables|Default|GetDistanceBetweenPieces)) (* (Variables|Default|GetTurning%20Distance%20Compensation) (Variables|Default|Getuwghewiugh))) "Local") (Spline|GetLocationatDistanceAlongSpline _bridgespline (+ (+ (* _index (Variables|Default|GetDistanceBetweenPieces)) (* (Variables|Default|GetTurning%20Distance%20Compensation) (Variables|Default|Getuwghewiugh))) (Variables|Default|GetDistanceBetweenPieces)) "Local")) 0.5) (Math|Rotator|CombineRotators (Math|Rotator|CombineRotators (Math|Rotator|FindLookatRotation (Spline|GetLocationatDistanceAlongSpline _bridgespline (+ (* _index (Variables|Default|GetDistanceBetweenPieces)) (* (Variables|Default|GetTurning%20Distance%20Compensation) (Variables|Default|Getuwghewiugh))) "Local") (Spline|GetLocationatDistanceAlongSpline _bridgespline (+ (+ (* _index (Variables|Default|GetDistanceBetweenPieces)) (* (Variables|Default|GetTurning%20Distance%20Compensation) (Variables|Default|Getuwghewiugh))) (Variables|Default|GetDistanceBetweenPieces)) "Local")) "0,90.000000, 0") (Math|Rotator|SelectRotator "0, 0, 0" "0,180.000000, 0" (Math|Random|RandomBoolfromStream (Variables|Default|GetSeed)))) "0.666600,0.666600,0.666600")))
                (:1
                  (Components|InstancedStaticMesh|AddInstance (Variables|Default|GetLongPiece2) (Math|Transform|MakeTransform (* (+ (Spline|GetLocationatDistanceAlongSpline _bridgespline (+ (* _index (Variables|Default|GetDistanceBetweenPieces)) (* (Variables|Default|GetTurning%20Distance%20Compensation) (Variables|Default|Getuwghewiugh))) "Local") (Spline|GetLocationatDistanceAlongSpline _bridgespline (+ (+ (* _index (Variables|Default|GetDistanceBetweenPieces)) (* (Variables|Default|GetTurning%20Distance%20Compensation) (Variables|Default|Getuwghewiugh))) (Variables|Default|GetDistanceBetweenPieces)) "Local")) 0.5) (Math|Rotator|CombineRotators (Math|Rotator|CombineRotators (Math|Rotator|FindLookatRotation (Spline|GetLocationatDistanceAlongSpline _bridgespline (+ (* _index (Variables|Default|GetDistanceBetweenPieces)) (* (Variables|Default|GetTurning%20Distance%20Compensation) (Variables|Default|Getuwghewiugh))) "Local") (Spline|GetLocationatDistanceAlongSpline _bridgespline (+ (+ (* _index (Variables|Default|GetDistanceBetweenPieces)) (* (Variables|Default|GetTurning%20Distance%20Compensation) (Variables|Default|Getuwghewiugh))) (Variables|Default|GetDistanceBetweenPieces)) "Local")) "0,90.000000, 0") (Math|Rotator|SelectRotator "0, 0, 0" "0,180.000000, 0" (Math|Random|RandomBoolfromStream (Variables|Default|GetSeed)))) "0.666600,0.666600,0.666600")))
                (:2
                  (Components|InstancedStaticMesh|AddInstance (Variables|Default|GetLongPiece3) (Math|Transform|MakeTransform (* (+ (Spline|GetLocationatDistanceAlongSpline _bridgespline (+ (* _index (Variables|Default|GetDistanceBetweenPieces)) (* (Variables|Default|GetTurning%20Distance%20Compensation) (Variables|Default|Getuwghewiugh))) "Local") (Spline|GetLocationatDistanceAlongSpline _bridgespline (+ (+ (* _index (Variables|Default|GetDistanceBetweenPieces)) (* (Variables|Default|GetTurning%20Distance%20Compensation) (Variables|Default|Getuwghewiugh))) (Variables|Default|GetDistanceBetweenPieces)) "Local")) 0.5) (Math|Rotator|CombineRotators (Math|Rotator|CombineRotators (Math|Rotator|FindLookatRotation (Spline|GetLocationatDistanceAlongSpline _bridgespline (+ (* _index (Variables|Default|GetDistanceBetweenPieces)) (* (Variables|Default|GetTurning%20Distance%20Compensation) (Variables|Default|Getuwghewiugh))) "Local") (Spline|GetLocationatDistanceAlongSpline _bridgespline (+ (+ (* _index (Variables|Default|GetDistanceBetweenPieces)) (* (Variables|Default|GetTurning%20Distance%20Compensation) (Variables|Default|Getuwghewiugh))) (Variables|Default|GetDistanceBetweenPieces)) "Local")) "0,90.000000, 0") (Math|Rotator|SelectRotator "0, 0, 0" "0,180.000000, 0" (Math|Random|RandomBoolfromStream (Variables|Default|GetSeed)))) "0.666600,0.666600,0.666600")))))
            (:B
              (switch int _returnvalue
                (:0
                  (Components|InstancedStaticMesh|AddInstance (Variables|Default|GetShortPiece1) (Math|Transform|MakeTransform (* (+ (Spline|GetLocationatDistanceAlongSpline _bridgespline (+ (* _index (Variables|Default|GetDistanceBetweenPieces)) (* (Variables|Default|GetTurning%20Distance%20Compensation) (Variables|Default|Getuwghewiugh))) "Local") (Spline|GetLocationatDistanceAlongSpline _bridgespline (+ (+ (* _index (Variables|Default|GetDistanceBetweenPieces)) (* (Variables|Default|GetTurning%20Distance%20Compensation) (Variables|Default|Getuwghewiugh))) (Variables|Default|GetDistanceBetweenPieces)) "Local")) 0.5) (Math|Rotator|CombineRotators (Math|Rotator|CombineRotators (Math|Rotator|FindLookatRotation (Spline|GetLocationatDistanceAlongSpline _bridgespline (+ (* _index (Variables|Default|GetDistanceBetweenPieces)) (* (Variables|Default|GetTurning%20Distance%20Compensation) (Variables|Default|Getuwghewiugh))) "Local") (Spline|GetLocationatDistanceAlongSpline _bridgespline (+ (+ (* _index (Variables|Default|GetDistanceBetweenPieces)) (* (Variables|Default|GetTurning%20Distance%20Compensation) (Variables|Default|Getuwghewiugh))) (Variables|Default|GetDistanceBetweenPieces)) "Local")) "0,90.000000, 0") (Math|Rotator|SelectRotator "0, 0, 0" "0,180.000000, 0" (Math|Random|RandomBoolfromStream (Variables|Default|GetSeed)))) "0.666600,0.666600,0.666600")))
                (:1
                  (Components|InstancedStaticMesh|AddInstance (Variables|Default|GetShortPiece2) (Math|Transform|MakeTransform (* (+ (Spline|GetLocationatDistanceAlongSpline _bridgespline (+ (* _index (Variables|Default|GetDistanceBetweenPieces)) (* (Variables|Default|GetTurning%20Distance%20Compensation) (Variables|Default|Getuwghewiugh))) "Local") (Spline|GetLocationatDistanceAlongSpline _bridgespline (+ (+ (* _index (Variables|Default|GetDistanceBetweenPieces)) (* (Variables|Default|GetTurning%20Distance%20Compensation) (Variables|Default|Getuwghewiugh))) (Variables|Default|GetDistanceBetweenPieces)) "Local")) 0.5) (Math|Rotator|CombineRotators (Math|Rotator|CombineRotators (Math|Rotator|FindLookatRotation (Spline|GetLocationatDistanceAlongSpline _bridgespline (+ (* _index (Variables|Default|GetDistanceBetweenPieces)) (* (Variables|Default|GetTurning%20Distance%20Compensation) (Variables|Default|Getuwghewiugh))) "Local") (Spline|GetLocationatDistanceAlongSpline _bridgespline (+ (+ (* _index (Variables|Default|GetDistanceBetweenPieces)) (* (Variables|Default|GetTurning%20Distance%20Compensation) (Variables|Default|Getuwghewiugh))) (Variables|Default|GetDistanceBetweenPieces)) "Local")) "0,90.000000, 0") (Math|Rotator|SelectRotator "0, 0, 0" "0,180.000000, 0" (Math|Random|RandomBoolfromStream (Variables|Default|GetSeed)))) "0.666600,0.666600,0.666600")))
                (:2
                  (Components|InstancedStaticMesh|AddInstance (Variables|Default|GetShortPiece3) (Math|Transform|MakeTransform (* (+ (Spline|GetLocationatDistanceAlongSpline _bridgespline (+ (* _index (Variables|Default|GetDistanceBetweenPieces)) (* (Variables|Default|GetTurning%20Distance%20Compensation) (Variables|Default|Getuwghewiugh))) "Local") (Spline|GetLocationatDistanceAlongSpline _bridgespline (+ (+ (* _index (Variables|Default|GetDistanceBetweenPieces)) (* (Variables|Default|GetTurning%20Distance%20Compensation) (Variables|Default|Getuwghewiugh))) (Variables|Default|GetDistanceBetweenPieces)) "Local")) 0.5) (Math|Rotator|CombineRotators (Math|Rotator|CombineRotators (Math|Rotator|FindLookatRotation (Spline|GetLocationatDistanceAlongSpline _bridgespline (+ (* _index (Variables|Default|GetDistanceBetweenPieces)) (* (Variables|Default|GetTurning%20Distance%20Compensation) (Variables|Default|Getuwghewiugh))) "Local") (Spline|GetLocationatDistanceAlongSpline _bridgespline (+ (+ (* _index (Variables|Default|GetDistanceBetweenPieces)) (* (Variables|Default|GetTurning%20Distance%20Compensation) (Variables|Default|Getuwghewiugh))) (Variables|Default|GetDistanceBetweenPieces)) "Local")) "0,90.000000, 0") (Math|Rotator|SelectRotator "0, 0, 0" "0,180.000000, 0" (Math|Random|RandomBoolfromStream (Variables|Default|GetSeed)))) "0.666600,0.666600,0.666600"))))))
          (if (> _index 1)
            (Utilities|Array|Add (Variables|Default|GetPrevious%20Piece%20Angle%20Array) (Math|Rotator|CombineRotators (Math|Rotator|CombineRotators (Math|Rotator|FindLookatRotation (Spline|GetLocationatDistanceAlongSpline _bridgespline (+ (* _index (Variables|Default|GetDistanceBetweenPieces)) (* (Variables|Default|GetTurning%20Distance%20Compensation) (Variables|Default|Getuwghewiugh))) "Local") (Spline|GetLocationatDistanceAlongSpline _bridgespline (+ (+ (* _index (Variables|Default|GetDistanceBetweenPieces)) (* (Variables|Default|GetTurning%20Distance%20Compensation) (Variables|Default|Getuwghewiugh))) (Variables|Default|GetDistanceBetweenPieces)) "Local")) "0,90.000000, 0") (* (Variables|Default|GetPrevious%20Piece%20Angle) -1.0))))
          (Variables|Default|SetPrevious%20Piece%20Angle (Math|Rotator|CombineRotators (Math|Rotator|FindLookatRotation (Spline|GetLocationatDistanceAlongSpline _bridgespline (+ (* _index (Variables|Default|GetDistanceBetweenPieces)) (* (Variables|Default|GetTurning%20Distance%20Compensation) (Variables|Default|Getuwghewiugh))) "Local") (Spline|GetLocationatDistanceAlongSpline _bridgespline (+ (+ (* _index (Variables|Default|GetDistanceBetweenPieces)) (* (Variables|Default|GetTurning%20Distance%20Compensation) (Variables|Default|Getuwghewiugh))) (Variables|Default|GetDistanceBetweenPieces)) "Local")) "0,90.000000, 0"))
          (CallFunction|SpawnPosts (+ (* _index (Variables|Default|GetDistanceBetweenPieces)) (* (Variables|Default|GetTurning%20Distance%20Compensation) (Variables|Default|Getuwghewiugh)))))))
    (:Completed
      ;[1 1 1] Spawn last bridge posts after rest of bridge has generated
      (CallFunction|SpawnPosts (+ (* _index (Variables|Default|GetDistanceBetweenPieces)) (* (Variables|Default|GetTurning%20Distance%20Compensation) (Variables|Default|Getuwghewiugh)))))))

(fn SpawnPosts
  (params (PointAlongSpline :type Float%20%28single-precision%29))
  (bind _bridgespline (Variables|Default|GetBridgeSpline))
  (bind _returnvalue (Spline|GetRotationatDistanceAlongSpline _bridgespline PointAlongSpline "World"))
  (for _index (range 0 1)
    (switch int (Math|Random|RandomIntegerinRangefromStream 0 2 (Variables|Default|GetSeed))
      (:0
        (Class|InstancedStaticMeshComponent|AddInstanceWorldSpace (Variables|Default|GetPost1) (Math|Transform|MakeTransform (+ (Spline|GetLocationatDistanceAlongSpline _bridgespline PointAlongSpline "World") (* (Math|Vector|GetRightVector _returnvalue) (Utilities|Select :Index _index :Option%200 58.0 :Option%201 -58.0)) (* (Math|Vector|GetUpVector _returnvalue) -1.5e+02)) (Math|Rotator|CombineRotators _returnvalue (Math|Rotator|MakeRotator 0.0 0.0 0.0)) "0.666600,0.666600,0.666600")))
      (:1
        (Class|InstancedStaticMeshComponent|AddInstanceWorldSpace (Variables|Default|GetPost2) (Math|Transform|MakeTransform (+ (Spline|GetLocationatDistanceAlongSpline _bridgespline PointAlongSpline "World") (* (Math|Vector|GetRightVector _returnvalue) (Utilities|Select :Index _index :Option%200 58.0 :Option%201 -58.0)) (* (Math|Vector|GetUpVector _returnvalue) -1.5e+02)) (Math|Rotator|CombineRotators _returnvalue (Math|Rotator|MakeRotator 0.0 0.0 0.0)) "0.666600,0.666600,0.666600")))
      (:2
        (Class|InstancedStaticMeshComponent|AddInstanceWorldSpace (Variables|Default|GetPost3) (Math|Transform|MakeTransform (+ (Spline|GetLocationatDistanceAlongSpline _bridgespline PointAlongSpline "World") (* (Math|Vector|GetRightVector _returnvalue) (Utilities|Select :Index _index :Option%200 58.0 :Option%201 -58.0)) (* (Math|Vector|GetUpVector _returnvalue) -1.5e+02)) (Math|Rotator|CombineRotators _returnvalue (Math|Rotator|MakeRotator 0.0 0.0 0.0)) "0.666600,0.666600,0.666600"))))))