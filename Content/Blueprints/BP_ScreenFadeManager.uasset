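; Manager that fades the screen out and back in, taking the player HUD and the repressed outline color's alpha along with the camera fade.
; FadeScreenOut and FadeScreenIn drive the camera manager fade and share one timeline, scaled to the requested duration and played forward or in reverse.
; Timeline updates write opacity to the global material parameter collection and HUD.
; A zero duration skips the timeline and sets the end state instantly.
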(event Custom|FadeScreenOut
  (params (Duration :type Float%20%28single-precision%29))
  (bind _playerref (Variables|Default|GetPlayerRef))
  (bind _playerref_2 (Variables|Default|GetPlayerRef))
  (if (== Duration 0.0)
    (Class|PlayerCameraManager|SetManualCameraFade :self (Game|GetPlayerCameraManager 0) :InFadeAmount 1.0)
    (bind _returnvalue (Rendering|Material|GetVectorParameterValue "/Game/ModelsMaterialsTextures/GlobalMaterialParams.GlobalMaterialParams" "RepressedOutlineColor" :!class /Script/Engine.KismetMaterialLibrary))
    (Rendering|Material|SetVectorParameterValue "/Game/ModelsMaterialsTextures/GlobalMaterialParams.GlobalMaterialParams" "RepressedOutlineColor" (Utilities|Struct|MakeLinearColor (.r _returnvalue) (.g _returnvalue) (.b _returnvalue) 0.0) :!class /Script/Engine.KismetMaterialLibrary)
    (Utilities|IsValid _playerref_2
      (:Is%20Valid
        (Widget|SetRenderOpacity (Variables|/Game/Blueprints/ThirdPersonBP/Blueprints/PlayerCharacter.PlayerCharacter_C|GetHUDref _playerref_2) 0.0)))
    (else
      (CameraFades|StartCameraFade :self (Game|GetPlayerCameraManager 0) :ToAlpha 1.0 :Duration Duration :bHoldWhenFinished true)
      (Components|Timeline|SetPlayRate (Variables|Default|GetScreenFadeTimeline) (/ 1.0 Duration))
      (bind _screenopacity (Timeline|ScreenFadeTimeline PlayFromStart)
        (:Update
          (bind _returnvalue_2 (Rendering|Material|GetVectorParameterValue "/Game/ModelsMaterialsTextures/GlobalMaterialParams.GlobalMaterialParams" "RepressedOutlineColor" :!class /Script/Engine.KismetMaterialLibrary))
          (Rendering|Material|SetVectorParameterValue "/Game/ModelsMaterialsTextures/GlobalMaterialParams.GlobalMaterialParams" "RepressedOutlineColor" (Utilities|Struct|MakeLinearColor (.r _returnvalue_2) (.g _returnvalue_2) (.b _returnvalue_2) _screenopacity) :!class /Script/Engine.KismetMaterialLibrary)
          (Utilities|IsValid _playerref
            (:Is%20Valid
              (Widget|SetRenderOpacity (Variables|/Game/Blueprints/ThirdPersonBP/Blueprints/PlayerCharacter.PlayerCharacter_C|GetHUDref _playerref) _screenopacity))))))))

(event Custom|FadeScreenIn
  (params (Duration :type Float%20%28single-precision%29))
  (bind _playerref (Variables|Default|GetPlayerRef))
  (bind _playerref_2 (Variables|Default|GetPlayerRef))
  (if (== Duration 0.0)
    (Class|PlayerCameraManager|SetManualCameraFade :self (Game|GetPlayerCameraManager 0))
    (bind _returnvalue (Rendering|Material|GetVectorParameterValue "/Game/ModelsMaterialsTextures/GlobalMaterialParams.GlobalMaterialParams" "RepressedOutlineColor" :!class /Script/Engine.KismetMaterialLibrary))
    (Rendering|Material|SetVectorParameterValue "/Game/ModelsMaterialsTextures/GlobalMaterialParams.GlobalMaterialParams" "RepressedOutlineColor" (Utilities|Struct|MakeLinearColor (.r _returnvalue) (.g _returnvalue) (.b _returnvalue) 1.0) :!class /Script/Engine.KismetMaterialLibrary)
    (Utilities|IsValid _playerref_2
      (:Is%20Valid
        (Widget|SetRenderOpacity (Variables|/Game/Blueprints/ThirdPersonBP/Blueprints/PlayerCharacter.PlayerCharacter_C|GetHUDref _playerref_2) 1.0)))
    (else
      (CameraFades|StartCameraFade :self (Game|GetPlayerCameraManager 0) :FromAlpha 1.0 :Duration Duration :bHoldWhenFinished true)
      (Components|Timeline|SetPlayRate (Variables|Default|GetScreenFadeTimeline) (/ 1.0 Duration))
      (bind _screenopacity (Timeline|ScreenFadeTimeline ReverseFromEnd)
        (:Update
          (bind _returnvalue_2 (Rendering|Material|GetVectorParameterValue "/Game/ModelsMaterialsTextures/GlobalMaterialParams.GlobalMaterialParams" "RepressedOutlineColor" :!class /Script/Engine.KismetMaterialLibrary))
          (Rendering|Material|SetVectorParameterValue "/Game/ModelsMaterialsTextures/GlobalMaterialParams.GlobalMaterialParams" "RepressedOutlineColor" (Utilities|Struct|MakeLinearColor (.r _returnvalue_2) (.g _returnvalue_2) (.b _returnvalue_2) _screenopacity) :!class /Script/Engine.KismetMaterialLibrary)
          (Utilities|IsValid _playerref
            (:Is%20Valid
              (Widget|SetRenderOpacity (Variables|/Game/Blueprints/ThirdPersonBP/Blueprints/PlayerCharacter.PlayerCharacter_C|GetHUDref _playerref) _screenopacity))))))))

(event EventBeginPlay
  (bind _asplayer_character (Utilities|Casting|CastToPlayerCharacter (Game|GetPlayerCharacter 0)))
  (Variables|Default|SetPlayerRef _asplayer_character))

(fn ConstructionScript)