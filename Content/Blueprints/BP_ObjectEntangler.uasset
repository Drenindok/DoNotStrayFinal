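; BP_ObjectEntangler is a placement helper that copies transforms between itself and a referenced actor from its construction script.
; A valid MoveMeTo teleports the entangler onto that actor; otherwise, a valid MoveThisToMe teleports that actor onto the entangler.
; Each move writes the referenced object's name to the TextRender and clears the reference, so it acts as a one-shot trigger.
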(fn ConstructionScript
  ;[1 1 1] Move Object To This Entangler
  (Utilities|IsValid (Utilities|ResolveSoftReference (Variables|Default|GetMove%20Me%20To%20:))
    (:Is%20Valid
      (Transformation|SetActorTransform (Transformation|GetActorTransform (Utilities|ResolveSoftReference (Variables|Default|GetMove%20Me%20To%20:))) false true)
      (Rendering|Components|TextRender|SetText (Variables|Default|GetTextRender) (Utilities|Text|ToText(String) (Utilities|GetObjectName (Utilities|ResolveSoftReference (Variables|Default|GetMove%20Me%20To%20:)))))
      (Variables|Default|SetMove%20Me%20To%20: 0))
    (:Is%20Not%20Valid
      ;[1 1 1] Move this entangler to object
      (Utilities|IsValid (Utilities|ResolveSoftReference (Variables|Default|GetMove%20This%20To%20Me))
        (:Is%20Valid
          (Transformation|SetActorTransform (Utilities|ResolveSoftReference (Variables|Default|GetMove%20This%20To%20Me)) (Transformation|GetActorTransform) false true)
          (Rendering|Components|TextRender|SetText (Variables|Default|GetTextRender) (Utilities|Text|ToText(String) (Utilities|GetObjectName (Utilities|ResolveSoftReference (Variables|Default|GetMove%20This%20To%20Me)))))
          (Variables|Default|SetMove%20This%20To%20Me 0))))))