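; Construction-script generator that scatters broken support posts along BridgeSpline to form a collapsed bridge.
; It steps along the spline, stretching spacing by accumulated yaw change, and tests both sides of each step.
; Where a sphere trace, ignoring NotABridge-tagged actors, hits nothing, a weighted seeded roll adds one of three instanced post meshes with jittered rotation.
; The mesh choice is unseeded, so post types change on each rebuild.
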(event EventBeginPlay)

(event Collision|EventActorBeginOverlap
  (params (OtherActor :type Actor%20Object%20Reference)))

(event EventTick
  (params (DeltaSeconds :type Float%20%28single-precision%29)))

(fn ConstructionScript
  (bind _bridgespline (Variables|Default|GetBridgeSpline))
  (bind _seed (Variables|Default|GetSeed))
  (if (Variables|Default|GetUpdate)
    (Variables|Default|SetUpdate false)
    (Class|KismetMathLibrary|SeedRandomStream (Variables|Default|GetSeed)))
  (Utilities|Array|Clear (Variables|Default|GetPrevious%20Piece%20Angle%20Array))
  (Variables|Default|SetTurning%20Distance%20Compensation 0.0)
  (Components|InstancedStaticMesh|ClearInstances (Variables|Default|GetPost1))
  (bind _index (Utilities|FlowControl|ForLoopwithBreak 0 (Math|Float|Truncate (- (/ (Spline|GetSplineLength (Variables|Default|GetBridgeSpline)) (Variables|Default|GetDistanceBetweenPieces)) 1.0)) :!label _label)
    (:LoopBody
      (Variables|Default|SetTurning%20Distance%20Compensation (+ (Variables|Default|GetTurning%20Distance%20Compensation) (Math|Float|Absolute(Float) (.Yaw (Math|Rotator|BreakRotator (Math|Rotator|CombineRotators (Math|Rotator|FindLookatRotation (Spline|GetLocationatDistanceAlongSpline _bridgespline (+ (* _index (Variables|Default|GetDistanceBetweenPieces)) (* (Variables|Default|GetTurning%20Distance%20Compensation) (Variables|Default|Getuwghewiugh))) "World") (Spline|GetLocationatDistanceAlongSpline _bridgespline (+ (+ (* _index (Variables|Default|GetDistanceBetweenPieces)) (* (Variables|Default|GetTurning%20Distance%20Compensation) (Variables|Default|Getuwghewiugh))) (Variables|Default|GetDistanceBetweenPieces)) "World")) (* (Variables|Default|GetPrevious%20Piece%20Angle) -1.0)))))))
      (if (< (Spline|GetSplineLength (Variables|Default|GetBridgeSpline)) (+ (* _index (Variables|Default|GetDistanceBetweenPieces)) (* (Variables|Default|GetTurning%20Distance%20Compensation) (Variables|Default|Getuwghewiugh))))
        (goto _label Break)
        (else
          (bind _outactors (Actor|GetAllActorswithTag "NotABridge"))
          (for _index_2 (range 0 1)
            (bind _returnvalue (Collision|SphereTraceByChannel (+ (+ (* (+ (Spline|GetLocationatDistanceAlongSpline _bridgespline (+ (* _index (Variables|Default|GetDistanceBetweenPieces)) (* (Variables|Default|GetTurning%20Distance%20Compensation) (Variables|Default|Getuwghewiugh))) "World") (Spline|GetLocationatDistanceAlongSpline _bridgespline (+ (+ (* _index (Variables|Default|GetDistanceBetweenPieces)) (* (Variables|Default|GetTurning%20Distance%20Compensation) (Variables|Default|Getuwghewiugh))) (Variables|Default|GetDistanceBetweenPieces)) "World")) 0.5) (* (Math|Vector|GetRightVector (Math|Rotator|FindLookatRotation (Spline|GetLocationatDistanceAlongSpline _bridgespline (+ (* _index (Variables|Default|GetDistanceBetweenPieces)) (* (Variables|Default|GetTurning%20Distance%20Compensation) (Variables|Default|Getuwghewiugh))) "World") (Spline|GetLocationatDistanceAlongSpline _bridgespline (+ (+ (* _index (Variables|Default|GetDistanceBetweenPieces)) (* (Variables|Default|GetTurning%20Distance%20Compensation) (Variables|Default|Getuwghewiugh))) (Variables|Default|GetDistanceBetweenPieces)) "World"))) (Utilities|Select :Index _index_2 :Option%200 85.0 :Option%201 -85.0)) "0,0,-150.000000") "0, 0, 0") (+ (+ (* (+ (Spline|GetLocationatDistanceAlongSpline _bridgespline (+ (* _index (Variables|Default|GetDistanceBetweenPieces)) (* (Variables|Default|GetTurning%20Distance%20Compensation) (Variables|Default|Getuwghewiugh))) "World") (Spline|GetLocationatDistanceAlongSpline _bridgespline (+ (+ (* _index (Variables|Default|GetDistanceBetweenPieces)) (* (Variables|Default|GetTurning%20Distance%20Compensation) (Variables|Default|Getuwghewiugh))) (Variables|Default|GetDistanceBetweenPieces)) "World")) 0.5) (* (Math|Vector|GetRightVector (Math|Rotator|FindLookatRotation (Spline|GetLocationatDistanceAlongSpline _bridgespline (+ (* _index (Variables|Default|GetDistanceBetweenPieces)) (* (Variables|Default|GetTurning%20Distance%20Compensation) (Variables|Default|Getuwghewiugh))) "World") (Spline|GetLocationatDistanceAlongSpline _bridgespline (+ (+ (* _index (Variables|Default|GetDistanceBetweenPieces)) (* (Variables|Default|GetTurning%20Distance%20Compensation) (Variables|Default|Getuwghewiugh))) (Variables|Default|GetDistanceBetweenPieces)) "World"))) (Utilities|Select :Index _index_2 :Option%200 85.0 :Option%201 -85.0)) "0,0,-150.000000") "0, 0,250.000000") 5.0 "TraceTypeQuery6" false _outactors "ForDuration"))
            (if (not _returnvalue)
              (if (Class|KismetMathLibrary|RandomBoolwithWeightfromStream (Variables|Default|GetPostSpawnChance) (Variables|Default|GetSeed))
                (switch int (Math|Random|RandomIntegerinRange 0 2)
                  (:0
                    (Class|InstancedStaticMeshComponent|AddInstanceWorldSpace (Variables|Default|GetPost1) (Math|Transform|MakeTransform (+ (* (+ (Spline|GetLocationatDistanceAlongSpline _bridgespline (+ (* _index (Variables|Default|GetDistanceBetweenPieces)) (* (Variables|Default|GetTurning%20Distance%20Compensation) (Variables|Default|Getuwghewiugh))) "World") (Spline|GetLocationatDistanceAlongSpline _bridgespline (+ (+ (* _index (Variables|Default|GetDistanceBetweenPieces)) (* (Variables|Default|GetTurning%20Distance%20Compensation) (Variables|Default|Getuwghewiugh))) (Variables|Default|GetDistanceBetweenPieces)) "World")) 0.5) (* (Math|Vector|GetRightVector (Math|Rotator|FindLookatRotation (Spline|GetLocationatDistanceAlongSpline _bridgespline (+ (* _index (Variables|Default|GetDistanceBetweenPieces)) (* (Variables|Default|GetTurning%20Distance%20Compensation) (Variables|Default|Getuwghewiugh))) "World") (Spline|GetLocationatDistanceAlongSpline _bridgespline (+ (+ (* _index (Variables|Default|GetDistanceBetweenPieces)) (* (Variables|Default|GetTurning%20Distance%20Compensation) (Variables|Default|Getuwghewiugh))) (Variables|Default|GetDistanceBetweenPieces)) "World"))) (Utilities|Select :Index _index_2 :Option%200 85.0 :Option%201 -85.0)) "0,0,-150.000000") (Math|Rotator|CombineRotators (Math|Rotator|FindLookatRotation (Spline|GetLocationatDistanceAlongSpline _bridgespline (+ (* _index (Variables|Default|GetDistanceBetweenPieces)) (* (Variables|Default|GetTurning%20Distance%20Compensation) (Variables|Default|Getuwghewiugh))) "World") (Spline|GetLocationatDistanceAlongSpline _bridgespline (+ (+ (* _index (Variables|Default|GetDistanceBetweenPieces)) (* (Variables|Default|GetTurning%20Distance%20Compensation) (Variables|Default|Getuwghewiugh))) (Variables|Default|GetDistanceBetweenPieces)) "World")) (Math|Rotator|MakeRotator (Math|Random|RandomFloatinRangefromStream -5.0 5.0 _seed) (Math|Random|RandomFloatinRangefromStream -5.0 5.0 _seed) (Utilities|Select :Index (Math|Random|RandomIntegerinRangefromStream 0 3 _seed) :Option%200 0.0 :Option%201 9e+01 :Option%202 1.8e+02 :Option%203 2.7e+02))) "0.666600,0.666600,0.666600")))
                  (:1
                    (Class|InstancedStaticMeshComponent|AddInstanceWorldSpace (Variables|Default|GetPost2) (Math|Transform|MakeTransform (+ (* (+ (Spline|GetLocationatDistanceAlongSpline _bridgespline (+ (* _index (Variables|Default|GetDistanceBetweenPieces)) (* (Variables|Default|GetTurning%20Distance%20Compensation) (Variables|Default|Getuwghewiugh))) "World") (Spline|GetLocationatDistanceAlongSpline _bridgespline (+ (+ (* _index (Variables|Default|GetDistanceBetweenPieces)) (* (Variables|Default|GetTurning%20Distance%20Compensation) (Variables|Default|Getuwghewiugh))) (Variables|Default|GetDistanceBetweenPieces)) "World")) 0.5) (* (Math|Vector|GetRightVector (Math|Rotator|FindLookatRotation (Spline|GetLocationatDistanceAlongSpline _bridgespline (+ (* _index (Variables|Default|GetDistanceBetweenPieces)) (* (Variables|Default|GetTurning%20Distance%20Compensation) (Variables|Default|Getuwghewiugh))) "World") (Spline|GetLocationatDistanceAlongSpline _bridgespline (+ (+ (* _index (Variables|Default|GetDistanceBetweenPieces)) (* (Variables|Default|GetTurning%20Distance%20Compensation) (Variables|Default|Getuwghewiugh))) (Variables|Default|GetDistanceBetweenPieces)) "World"))) (Utilities|Select :Index _index_2 :Option%200 85.0 :Option%201 -85.0)) "0,0,-150.000000") (Math|Rotator|CombineRotators (Math|Rotator|FindLookatRotation (Spline|GetLocationatDistanceAlongSpline _bridgespline (+ (* _index (Variables|Default|GetDistanceBetweenPieces)) (* (Variables|Default|GetTurning%20Distance%20Compensation) (Variables|Default|Getuwghewiugh))) "World") (Spline|GetLocationatDistanceAlongSpline _bridgespline (+ (+ (* _index (Variables|Default|GetDistanceBetweenPieces)) (* (Variables|Default|GetTurning%20Distance%20Compensation) (Variables|Default|Getuwghewiugh))) (Variables|Default|GetDistanceBetweenPieces)) "World")) (Math|Rotator|MakeRotator (Math|Random|RandomFloatinRangefromStream -5.0 5.0 _seed) (Math|Random|RandomFloatinRangefromStream -5.0 5.0 _seed) (Utilities|Select :Index (Math|Random|RandomIntegerinRangefromStream 0 3 _seed) :Option%200 0.0 :Option%201 9e+01 :Option%202 1.8e+02 :Option%203 2.7e+02))) "0.666600,0.666600,0.666600")))
                  (:2
                    (Class|InstancedStaticMeshComponent|AddInstanceWorldSpace (Variables|Default|GetPost3) (Math|Transform|MakeTransform (+ (* (+ (Spline|GetLocationatDistanceAlongSpline _bridgespline (+ (* _index (Variables|Default|GetDistanceBetweenPieces)) (* (Variables|Default|GetTurning%20Distance%20Compensation) (Variables|Default|Getuwghewiugh))) "World") (Spline|GetLocationatDistanceAlongSpline _bridgespline (+ (+ (* _index (Variables|Default|GetDistanceBetweenPieces)) (* (Variables|Default|GetTurning%20Distance%20Compensation) (Variables|Default|Getuwghewiugh))) (Variables|Default|GetDistanceBetweenPieces)) "World")) 0.5) (* (Math|Vector|GetRightVector (Math|Rotator|FindLookatRotation (Spline|GetLocationatDistanceAlongSpline _bridgespline (+ (* _index (Variables|Default|GetDistanceBetweenPieces)) (* (Variables|Default|GetTurning%20Distance%20Compensation) (Variables|Default|Getuwghewiugh))) "World") (Spline|GetLocationatDistanceAlongSpline _bridgespline (+ (+ (* _index (Variables|Default|GetDistanceBetweenPieces)) (* (Variables|Default|GetTurning%20Distance%20Compensation) (Variables|Default|Getuwghewiugh))) (Variables|Default|GetDistanceBetweenPieces)) "World"))) (Utilities|Select :Index _index_2 :Option%200 85.0 :Option%201 -85.0)) "0,0,-150.000000") (Math|Rotator|CombineRotators (Math|Rotator|FindLookatRotation (Spline|GetLocationatDistanceAlongSpline _bridgespline (+ (* _index (Variables|Default|GetDistanceBetweenPieces)) (* (Variables|Default|GetTurning%20Distance%20Compensation) (Variables|Default|Getuwghewiugh))) "World") (Spline|GetLocationatDistanceAlongSpline _bridgespline (+ (+ (* _index (Variables|Default|GetDistanceBetweenPieces)) (* (Variables|Default|GetTurning%20Distance%20Compensation) (Variables|Default|Getuwghewiugh))) (Variables|Default|GetDistanceBetweenPieces)) "World")) (Math|Rotator|MakeRotator (Math|Random|RandomFloatinRangefromStream -5.0 5.0 _seed) (Math|Random|RandomFloatinRangefromStream -5.0 5.0 _seed) (Utilities|Select :Index (Math|Random|RandomIntegerinRangefromStream 0 3 _seed) :Option%200 0.0 :Option%201 9e+01 :Option%202 1.8e+02 :Option%203 2.7e+02))) "0.666600,0.666600,0.666600"))))
                (if (> _index 1)
                  (Utilities|Array|Add (Variables|Default|GetPrevious%20Piece%20Angle%20Array) (Math|Rotator|CombineRotators (Math|Rotator|FindLookatRotation (Spline|GetLocationatDistanceAlongSpline _bridgespline (+ (* _index (Variables|Default|GetDistanceBetweenPieces)) (* (Variables|Default|GetTurning%20Distance%20Compensation) (Variables|Default|Getuwghewiugh))) "World") (Spline|GetLocationatDistanceAlongSpline _bridgespline (+ (+ (* _index (Variables|Default|GetDistanceBetweenPieces)) (* (Variables|Default|GetTurning%20Distance%20Compensation) (Variables|Default|Getuwghewiugh))) (Variables|Default|GetDistanceBetweenPieces)) "World")) (* (Variables|Default|GetPrevious%20Piece%20Angle) -1.0))))
                (Variables|Default|SetPrevious%20Piece%20Angle (Math|Rotator|FindLookatRotation (Spline|GetLocationatDistanceAlongSpline _bridgespline (+ (* _index (Variables|Default|GetDistanceBetweenPieces)) (* (Variables|Default|GetTurning%20Distance%20Compensation) (Variables|Default|Getuwghewiugh))) "World") (Spline|GetLocationatDistanceAlongSpline _bridgespline (+ (+ (* _index (Variables|Default|GetDistanceBetweenPieces)) (* (Variables|Default|GetTurning%20Distance%20Compensation) (Variables|Default|Getuwghewiugh))) (Variables|Default|GetDistanceBetweenPieces)) "World")))))))))))