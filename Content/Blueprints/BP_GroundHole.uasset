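; Ground hole the player listens into: on activation it takes input, blends the view to itself and fades the screen out under a sound mix.
; It fades in swamp and forest ambience by level name and player height, then a configurable right-ear sound after a random delay.
; After a wait, any key restores view, input and audio.
; A timeline pins the phone light to the camera during both blends.
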(event Custom|Activated
  (bind _returnvalue (Game|GetPlayerController 0))
  (bind _returnvalue_2 (Game|GetPlayerCameraManager 0))
  (bind _playerref (Variables|Default|GetPlayerRef))
  (bind _phonelight (Variables|/Game/Blueprints/ThirdPersonBP/Blueprints/PlayerCharacter.PlayerCharacter_C|GetPhoneLight _playerref))
  (Utilities|FlowControl|Sequence
    (:then_0
      (Input|DisableInput (Variables|Default|GetPlayerRef) _returnvalue)
      (Input|EnableInput _returnvalue)
      (Audio|PlaySound2D "/Game/Audio/wav_HoleReach.wav_HoleReach" 1.0 1.0 0.2 0 0)
      (Game|Player|SetViewTargetwithBlend (Game|GetPlayerController 0) self 1.0 "VTBlend_EaseInOut" 2.0 false)
      (Utilities|FlowControl|Sequence
        (:then_0
          (|FadeInLeft/RightSounds))
        (:then_1
          (Utilities|FlowControl|Delay 0.75)
          (bind _returnvalue_3 (Actor|GetActorOfClass "/Game/Blueprints/BP_ScreenFadeManager.BP_ScreenFadeManager_C"))
          (Default|FadeScreenOut _returnvalue_3 0.5)
          (Audio|PushSoundMixModifier "/Game/Audio/EarToHoleMix.EarToHoleMix")
          (Utilities|FlowControl|Delay 4.0)
          (Variables|Default|SetReadyToStandUp true))))
    (:then_1
      ;[1 1 1] Makes sure player's flashlight stays attached to camera properly
      (Timeline|Timeline_0 PlayFromStart
        (:Update
          (Transformation|SetWorldLocationAndRotation _phonelight (Camera|GetCameraLocation _returnvalue_2) (Camera|GetCameraRotation _returnvalue_2) false false))
        (:Finished
          (Transformation|SetRelativeLocationAndRotation _phonelight "0,-1.500000, 0" "0, 0, 0" false false))))))

(event EventBeginPlay
  (bind _asplayer_character (Utilities|Casting|CastToPlayerCharacter (Game|GetPlayerCharacter 0)))
  (Variables|Default|SetPlayerRef _asplayer_character))

(event Input|KeyboardEvents|AnyKey
  (params (Key :type Key%20Structure :default "None"))
  (bind _returnvalue (Game|GetPlayerController 0))
  (bind _returnvalue_2 (Game|GetPlayerCameraManager 0))
  (bind _playerref (Variables|Default|GetPlayerRef))
  (bind _phonelight (Variables|/Game/Blueprints/ThirdPersonBP/Blueprints/PlayerCharacter.PlayerCharacter_C|GetPhoneLight _playerref))
  ;[1 1 1] Stand up after you press any key
  (:Pressed
    (if (Variables|Default|GetReadyToStandUp)
      (Utilities|FlowControl|Sequence
        (:then_0
          (Variables|Default|SetReadyToStandUp false)
          (Input|DisableInput _returnvalue)
          (Input|EnableInput (Variables|Default|GetPlayerRef) _returnvalue)
          (Game|Player|SetViewTargetwithBlend (Game|GetPlayerController 0) (Variables|Default|GetPlayerRef) 1.0 "VTBlend_EaseInOut" 2.0 false)
          (bind _returnvalue_3 (Actor|GetActorOfClass "/Game/Blueprints/BP_ScreenFadeManager.BP_ScreenFadeManager_C"))
          (Default|FadeScreenin _returnvalue_3 0.5)
          (Class|GameplayStatics|ClearSoundMixModifiers)
          (Audio|Components|Audio|FadeOut (Variables|Default|GetSwampSound) 0.5 0.0 "Linear" :!class /Script/Engine.AudioComponent))
        (:then_1
          ;[1 1 1] Makes sure player's flashlight stays attached to camera properly
          (Timeline|Timeline_0 PlayFromStart
            (:Update
              (Transformation|SetWorldLocationAndRotation _phonelight (Camera|GetCameraLocation _returnvalue_2) (Camera|GetCameraRotation _returnvalue_2) false false))
            (:Finished
              (Transformation|SetRelativeLocationAndRotation _phonelight "0,-1.500000, 0" "0, 0, 0" false false))))))))

(fn ConstructionScript)