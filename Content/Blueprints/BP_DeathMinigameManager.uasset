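; Manager actor that runs the "repressed" minigames played after player death, selected by death count.
; StartMinigame switches lighting and outline materials, then teleports the player to a tagged start point.
; Events cover an inventory-gated room exit and a panic attack that CalmDown eases stepwise, crossfading audio and interpolating glitch through a Delay loop.
; EndDeathMinigame returns the player to their trail post at night and updates the monster's spawn timer.
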(event Custom|Start%20Minigame
  (params (Number%20of%20deaths :type Integer))
  (bind _playerref (Variables|Default|GetPlayerRef))
  (bind _playerref_2 (Variables|Default|GetPlayerRef))
  (bind _playerref_3 (Variables|Default|GetPlayerRef))
  (bind _playerref_4 (Variables|Default|GetPlayerRef))
  (bind _playerref_5 (Variables|Default|GetPlayerRef))
  (Variables|/Game/Blueprints/ThirdPersonBP/Blueprints/PlayerCharacter.PlayerCharacter_C|SetInDeathMinigame _playerref true)
  (Variables|/Game/Blueprints/ThirdPersonBP/Blueprints/PlayerCharacter.PlayerCharacter_C|SetSprinting _playerref false)
  (Variables|/Game/Blueprints/ThirdPersonBP/Blueprints/PlayerCharacter.PlayerCharacter_C|SetCurrentHarshGlitchStrength _playerref 0.0)
  (Variables|/Game/Blueprints/ThirdPersonBP/Blueprints/PlayerCharacter.PlayerCharacter_C|SetCurrentGlitchScale _playerref 0.0)
  (Variables|/Game/Blueprints/ThirdPersonBP/Blueprints/PlayerCharacter.PlayerCharacter_C|SetTargetHarshGlitchStrength _playerref 0.0)
  (bind _returnvalue (Actor|GetActorOfClass "/Game/Blueprints/BP_LightingManager.BP_LightingManager_C"))
  (Default|SwitchtoRepressed _returnvalue false)
  (Default|ForceLightOff (Variables|Default|GetPlayerRef))
  (Default|ClearThoughts (Variables|Default|GetGameInstanceRef) true)
  (Rendering|Material|SetScalarParameterValue "/Game/ModelsMaterialsTextures/GlobalMaterialParams.GlobalMaterialParams" "GlitchStrength" 0.0 :!class /Script/Engine.KismetMaterialLibrary)
  (switch int Number%20of%20deaths
    (:0
      ;[1 1 1] Minigame 0 (run2 room) start
      (Rendering|Material|SetVectorParameterValue "/Game/ModelsMaterialsTextures/GlobalMaterialParams.GlobalMaterialParams" "RepressedOutlineColor" (Utilities|Struct|MakeLinearColor 0.5 0.5 0.5 1.0) :!class /Script/Engine.KismetMaterialLibrary)
      (bind _outactors (Actor|GetAllActorsOfClasswithTag "/Script/Engine.TargetPoint" "Minigame Start 0"))
      (Transformation|Teleport (Variables|Default|GetPlayerRef) (.location (Transformation|GetActorTransform (Utilities|Array|Get(acopy) _outactors))) "0, 0, 0")
      (Pawn|SetControlRotation (Game|GetPlayerController 0) (.rotation (Transformation|GetActorTransform (Utilities|Array|Get(acopy) _outactors))))
      (Variables|/Script/Engine.SpringArmComponent|SetbEnableCameraRotationLag (Variables|/Game/Blueprints/ThirdPersonBP/Blueprints/PlayerCharacter.PlayerCharacter_C|GetCam-PhoneArm _playerref_3) false)
      (Default|ReEnableCameraLagAfterCheckpointLoad _playerref_3)
      (Variables|/Script/Engine.PostProcessVolume|SetSettings (Utilities|ResolveSoftReference (Variables|Default|GetRepressedPostProcess)) (Utilities|Struct|MakePostProcessSettings (Utilities|Struct|MakeWeightedBlendables (Utilities|Array|MakeArray (Utilities|Struct|MakeWeightedBlendable 0.0 "/Game/ModelsMaterialsTextures/Materials/TORITU_Materials/Mat_PP_RGBify.Mat_PP_RGBify") (Utilities|Struct|MakeWeightedBlendable 1.0 "/Game/ModelsMaterialsTextures/Materials/TORITU_Materials/Mat_PP_Outline_Colored.Mat_PP_Outline_Colored")))))
      (Audio|Components|Audio|Play (Variables|Default|GetWav_Heartbeat) 0.0))
    (:1
      ;[1 1 1] Minigame 1 start
      (Rendering|Material|SetVectorParameterValue "/Game/ModelsMaterialsTextures/GlobalMaterialParams.GlobalMaterialParams" "RepressedOutlineColor" (Utilities|Struct|MakeLinearColor 0.5 0.5 0.5 1.0) :!class /Script/Engine.KismetMaterialLibrary :!label _label)
      (bind _outactors_2 (Actor|GetAllActorsOfClasswithTag "/Script/Engine.TargetPoint" "Minigame Start 1"))
      (Transformation|Teleport (Variables|Default|GetPlayerRef) (.location (Transformation|GetActorTransform (Utilities|Array|Get(acopy) _outactors_2))) "0, 0, 0")
      (Pawn|SetControlRotation (Game|GetPlayerController 0) (.rotation (Transformation|GetActorTransform (Utilities|Array|Get(acopy) _outactors_2))))
      (Variables|/Script/Engine.SpringArmComponent|SetbEnableCameraRotationLag (Variables|/Game/Blueprints/ThirdPersonBP/Blueprints/PlayerCharacter.PlayerCharacter_C|GetCam-PhoneArm _playerref_5) false)
      (Default|ReEnableCameraLagAfterCheckpointLoad _playerref_5)
      (Audio|Components|Audio|Play (Variables|Default|GetWav_Heartbeat) 0.0))
    (:2
      ;[1 1 1] Minigame 2 start
      (Rendering|Material|SetVectorParameterValue "/Game/ModelsMaterialsTextures/GlobalMaterialParams.GlobalMaterialParams" "RepressedOutlineColor" (Utilities|Struct|MakeLinearColor 0.5 0.5 0.5 1.0) :!class /Script/Engine.KismetMaterialLibrary)
      (bind _outactors_3 (Actor|GetAllActorsOfClasswithTag "/Script/Engine.TargetPoint" "Minigame Start 2"))
      (Transformation|Teleport (Variables|Default|GetPlayerRef) (.location (Transformation|GetActorTransform (Utilities|Array|Get(acopy) _outactors_3))) "0, 0, 0")
      (Pawn|SetControlRotation (Game|GetPlayerController 0) (.rotation (Transformation|GetActorTransform (Utilities|Array|Get(acopy) _outactors_3))))
      (Variables|/Script/Engine.SpringArmComponent|SetbEnableCameraRotationLag (Variables|/Game/Blueprints/ThirdPersonBP/Blueprints/PlayerCharacter.PlayerCharacter_C|GetCam-PhoneArm _playerref_2) false)
      (Default|ReEnableCameraLagAfterCheckpointLoad _playerref_2)
      (Audio|Components|Audio|Play (Variables|Default|GetWav_PhonePanicAttack_Intro) 0.0)
      (Utilities|FlowControl|Delay 19.300703)
      (Audio|Components|Audio|Play (Variables|Default|Getwav_PhonePanicAttack_Main) 0.0)
      (Rendering|Material|SetScalarParameterValue "/Game/ModelsMaterialsTextures/GlobalMaterialParams.GlobalMaterialParams" "GlitchStrength" 1.0 :!class /Script/Engine.KismetMaterialLibrary)
      (Rendering|Material|SetVectorParameterValue "/Game/ModelsMaterialsTextures/GlobalMaterialParams.GlobalMaterialParams" "RepressedOutlineColor" (Utilities|Struct|MakeLinearColor 0.5 0.0 0.0 1.0) :!class /Script/Engine.KismetMaterialLibrary)
      (Default|ClearThoughts (Variables|Default|GetGameInstanceRef) true)
      (Transformation|SetActorLocation _playerref_4 (+ (Transformation|GetActorLocation _playerref_4) "1000.000000, 0, 0") false true)
      (Default|ClearThoughts (Variables|Default|GetGameInstanceRef) true))
    (:3
      (goto _label))))

(event Custom|FadeOutScreen
  (Input|DisableInput (Variables|Default|GetPlayerRef) (Game|GetPlayerController 0))
  (Default|ClearThoughts (Variables|Default|GetGameInstanceRef) false)
  (bind _returnvalue (Actor|GetActorOfClass "/Game/Blueprints/BP_ScreenFadeManager.BP_ScreenFadeManager_C"))
  (Default|FadeScreenOut _returnvalue 1.0))

(event Custom|End%20Death%20Minigame
  (bind _playerref (Variables|Default|GetPlayerRef))
  (bind _playerref_2 (Variables|Default|GetPlayerRef))
  (Variables|/Game/Blueprints/ThirdPersonBP/Blueprints/PlayerCharacter.PlayerCharacter_C|SetSprinting (Variables|Default|GetPlayerRef) false)
  (Rendering|Material|SetVectorParameterValue "/Game/ModelsMaterialsTextures/GlobalMaterialParams.GlobalMaterialParams" "RepressedOutlineColor" (Utilities|Struct|MakeLinearColor 0.0 0.0 0.0 1.0) :!class /Script/Engine.KismetMaterialLibrary)
  (Default|ClearThoughts (Variables|Default|GetGameInstanceRef) true)
  (Audio|Components|Audio|Stop (Variables|Default|GetWav_Heartbeat))
  (bind _outactors (Actor|GetAllActorsOfClasswithTag "/Game/Blueprints/BP_TrailPost.BP_TrailPost_C" (Utilities|String|StringToName (Utilities|String|Append "post " (Utilities|String|ToString(Integer) (Variables|/Game/Blueprints/ThirdPersonBP/Blueprints/PlayerCharacter.PlayerCharacter_C|GetSignpost# (Variables|Default|GetPlayerRef)))))))
  (Transformation|SetActorLocation _playerref_2 (Transformation|GetWorldLocation (Variables|/Game/Blueprints/BP_TrailPost.BP_TrailPost_C|GetRespawnPoint (Utilities|Array|Get(acopy) _outactors))) false true)
  (Pawn|SetControlRotation (Game|GetPlayerController 0) (Transformation|GetWorldRotation (Variables|/Game/Blueprints/BP_TrailPost.BP_TrailPost_C|GetRespawnPoint (Utilities|Array|Get(acopy) _outactors))))
  (Default|GlitchBacktoTrail _playerref_2)
  (bind _returnvalue (Actor|GetActorOfClass "/Game/Blueprints/BP_LightingManager.BP_LightingManager_C"))
  (Default|SwitchtoNight _returnvalue)
  (Variables|/Game/Blueprints/ThirdPersonBP/Blueprints/PlayerCharacter.PlayerCharacter_C|SetInDeathMinigame _playerref false)
  (Default|ForceLighton _playerref)
  (Default|UpdateTimeUntilNextSpawn (Variables|/Game/Blueprints/ThirdPersonBP/Blueprints/PlayerCharacter.PlayerCharacter_C|GetMonsterRef _playerref)))

(event Custom|Fade%20Out%20Then%20end%20minigame
  (CallFunction|FadeOutScreen)
  (Utilities|FlowControl|Delay 3.0)
  (CallFunction|EndDeathMinigame)
  (Input|EnableInput (Variables|Default|GetPlayerRef) (Game|GetPlayerController 0))
  (Widget|SetRenderOpacity (Variables|/Game/Blueprints/ThirdPersonBP/Blueprints/PlayerCharacter.PlayerCharacter_C|GetHUDref (Variables|Default|GetPlayerRef)) 1.0))

(event EventBeginPlay
  (bind _asplayer_character (Utilities|Casting|CastToPlayerCharacter (Game|GetPlayerCharacter 0)))
  (Variables|Default|SetPlayerRef _asplayer_character)
  (bind _asmain_game_instance (Utilities|Casting|CastToMainGameInstance (Game|GetGameInstance)))
  (Variables|Default|SetGameInstanceRef _asmain_game_instance))

(fn ConstructionScript)

(fn AddInventoryItem
  (params (Item%20Name :type String))
  (Utilities|Array|Add (Variables|Default|GetInventory) Item%20Name))

(event Custom|Attempt%20To%20Leave%20Room
  (bind _inventory (Variables|Default|GetInventory))
  ;[1 1 1] Attempt to Leave Room
  (if (and (Utilities|Array|ContainsItem _inventory "Keys") (Utilities|Array|ContainsItem _inventory "Camera"))
    (CallFunction|FadeOutThenEndMinigame)
    (Utilities|FlowControl|Delay 1.0)
    (Audio|PlaySound2D "/Game/Audio/Door/wav_door_open.wav_door_open" 1.0 1.0 0.0 0 0)
    (else
      (Default|ShowThoughts (Variables|Default|GetGameInstanceRef) "I need my camcorder and my car keys." (Utilities|Struct|MakeSlateFontInfo "/Game/Fonts/naomis_hand-NewFathersFont/NaomisHand-Regular_Font.NaomisHand-Regular_Font" 0 (Utilities|Struct|MakeFontOutlineSettings 2 false false 0 "(R=0.500000,G=0.500000,B=0.500000,A=1.000000)")) (Utilities|Struct|MakeSlateColor "(R=0.000000,G=0.000000,B=0.000000,A=1.000000)") false 25.0 0.0 0.0 true false))))

(event Custom|SkipBackFromPhone
  (bind _playerref (Variables|Default|GetPlayerRef))
  (Rendering|Material|SetScalarParameterValue "/Game/ModelsMaterialsTextures/GlobalMaterialParams.GlobalMaterialParams" "GlitchStrength" 5.0 :!class /Script/Engine.KismetMaterialLibrary)
  (Transformation|SetActorLocation _playerref (+ (Transformation|GetActorLocation _playerref) "0,250.000000, 0") false true)
  (Utilities|FlowControl|Delay 0.1)
  (Rendering|Material|SetScalarParameterValue "/Game/ModelsMaterialsTextures/GlobalMaterialParams.GlobalMaterialParams" "GlitchStrength" (Variables|2ndMinigame|GetScreenGlitch/PanicAmount) :!class /Script/Engine.KismetMaterialLibrary))

(event Custom|Calm%20Down
  (bind _playerref (Variables|Default|GetPlayerRef))
  (if (not (Variables|/Game/MainGameInstance.MainGameInstance_C|GetShowingThoughts (Variables|Default|GetGameInstanceRef)))
    (bind _output_get (Variables|2ndMinigame|SetCalmDownClicks (Math|Integer|Clamp(Integer) (+ (Variables|2ndMinigame|GetCalmDownClicks) 1) 1 4)))
    (switch int _output_get
      (:1
        (Audio|Components|Audio|Play (Variables|Default|Getwav_EndingWalk_Breathing) 0.0)
        (Audio|Components|Audio|AdjustVolume (Variables|Default|Getwav_vinylCrackle) 0.0 0.001 "Linear" :!class /Script/Engine.AudioComponent)
        (Variables|2ndMinigame|SetScreenGlitch/PanicAmount 0.75)
        (Audio|Components|Audio|AdjustVolume (Variables|Default|Getwav_PhonePanicAttack_Main) 3.0 (Variables|2ndMinigame|GetScreenGlitch/PanicAmount) "Linear" :!class /Script/Engine.AudioComponent :!label _label)
        (Audio|Components|Audio|AdjustVolume (Variables|Default|Getwav_EndingWalk_Breathing) 3.0 (- 1.0 (Variables|2ndMinigame|GetScreenGlitch/PanicAmount)) "Linear" :!class /Script/Engine.AudioComponent)
        (bind _returnvalue (Rendering|Material|GetScalarParameterValue "/Game/ModelsMaterialsTextures/GlobalMaterialParams.GlobalMaterialParams" "GlitchStrength" :!class /Script/Engine.KismetMaterialLibrary :!label _label_2))
        (Rendering|Material|SetVectorParameterValue "/Game/ModelsMaterialsTextures/GlobalMaterialParams.GlobalMaterialParams" "RepressedOutlineColor" (Math|Color|Lerp(LinearColor) "(R=0.500000,G=0.500000,B=0.500000,A=1.000000)" "(R=0.500000,G=0.000000,B=0.000000,A=1.000000)" (Math|Interpolation|FInterptoConstant _returnvalue (Variables|2ndMinigame|GetScreenGlitch/PanicAmount) (Utilities|Time|GetWorldDeltaSeconds) 0.1)) :!class /Script/Engine.KismetMaterialLibrary)
        (Rendering|Material|SetScalarParameterValue "/Game/ModelsMaterialsTextures/GlobalMaterialParams.GlobalMaterialParams" "GlitchStrength" (Math|Interpolation|FInterptoConstant _returnvalue (Variables|2ndMinigame|GetScreenGlitch/PanicAmount) (Utilities|Time|GetWorldDeltaSeconds) 0.1) :!class /Script/Engine.KismetMaterialLibrary)
        (if (!= (Math|Interpolation|FInterptoConstant _returnvalue (Variables|2ndMinigame|GetScreenGlitch/PanicAmount) (Utilities|Time|GetWorldDeltaSeconds) 0.1) (Variables|2ndMinigame|GetScreenGlitch/PanicAmount))
          (Utilities|FlowControl|Delay 0.0)
          (goto _label_2)))
      (:2
        (Variables|2ndMinigame|SetScreenGlitch/PanicAmount 0.5)
        (goto _label))
      (:3
        (Variables|2ndMinigame|SetScreenGlitch/PanicAmount 0.0)
        (Utilities|FlowControl|Sequence
          (:then_0
            (goto _label))
          (:then_1
            (Utilities|FlowControl|Delay 3.0)
            (Audio|Components|Audio|AdjustVolume (Variables|Default|Getwav_EndingWalk_Breathing) 6.0 0.0 "Linear" :!class /Script/Engine.AudioComponent))
          (:then_2
            (Transformation|SetActorLocation _playerref (+ (Transformation|GetActorLocation _playerref) "1000.000000,0.000000, 0") false true)))))))