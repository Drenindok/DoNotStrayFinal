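; Actor that lays a trail of bloody footprint decals from an array of transforms offset from its location, optionally on BeginPlay.
; Generate loops on a short delay, spawning one fading-in, dark-red tinted decal per pass and playing a step sound at the incremented index's location.
; The construction script previews footprints as instanced meshes, or applies a one-shot offset to the stored locations.
; An all-at-once spawn loop is left unconnected.
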(event Custom|Generate
  (bind _returnvalue (Transformation|GetActorLocation))
  (bind _footprints (Variables|Default|GetFootprints))
  (bind _currentfootprintindex (Variables|Default|GetCurrentFootprintIndex))
  (bind _output (Utilities|Array|Get(acopy) _footprints _currentfootprintindex))
  (bind _returnvalue_2 (+ (.location _output) _returnvalue))
  (Utilities|FlowControl|Delay 0.525 :!label _label)
  (if (Utilities|Array|IsValidIndex _footprints _currentfootprintindex)
    (bind _returnvalue_3 (Rendering|Decal|SpawnDecalatLocation "/Game/ModelsMaterialsTextures/Materials/Footprints/Mat_BloodFootprint.Mat_BloodFootprint" (.scale _output) _returnvalue_2 (.rotation _output) 0.0))
    (Utilities|Array|Add (Variables|Default|GetSpawned%20Decals) _returnvalue_3)
    (Rendering|Components|Decal|SetFadeIn _returnvalue_3 0.0 1.0)
    (bind _returnvalue_4 (Rendering|Material|CreateDynamicMaterialInstance _returnvalue_3 :!class /Script/Engine.DecalComponent))
    (Rendering|Material|SetVectorParameterValue _returnvalue_4 "InitialColor" "(R=0.012500,G=0.000000,B=0.000000,A=1.000000)" :!class /Script/Engine.MaterialInstanceDynamic)
    (Math|Integer|IncrementInt (Variables|Default|GetCurrentFootprintIndex)
      (:%20%20
        (Audio|PlaySoundatLocation "/Game/Audio/Footsteps/Blood/Cue_Step_Blood.Cue_Step_Blood" _returnvalue_2 "0, 0, 0" 0.5 1.0 0.0 "/Game/Audio/Atten_MonsterNoises.Atten_MonsterNoises" 0 0)
        (goto _label)))))

(event EventBeginPlay
  (if (Variables|Default|GetGenerate%20On%20Begin%20Play)
    (CallFunction|Generate)))

(fn ConstructionScript
  (bind _footprints (Variables|Default|GetFootprints))
  (if (Variables|Default|GetVisualize)
    (for _array_element (Variables|Default|GetFootprints)
      (Class|InstancedStaticMeshComponent|AddInstanceWorldSpace (Variables|Default|GetInstancedStaticMesh) (Math|Transform|MakeTransform (+ (.location _array_element) (Transformation|GetActorLocation)) (.rotation _array_element) (* (.scale _array_element) 0.02))))
    (elif (Variables|Default|GetOffsetToNewLocation)
      (Variables|Default|SetOffsetToNewLocation false)
      (for (_array_element_2 _array_index) _footprints
        (Utilities|Array|SetArrayElem _footprints _array_index (Math|Transform|MakeTransform (- (.location _array_element_2) (Variables|Default|GetNewLocation)) (.rotation _array_element_2) (.scale _array_element_2))))
      (Variables|Default|SetNewLocation "0, 0, 0"))))