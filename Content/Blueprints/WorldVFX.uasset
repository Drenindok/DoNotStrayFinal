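; World VFX actor that controls exponential height fog and teleports itself to the player character's location every tick.
; Each tick it looks up BP_LoopingSubLevelLoader and, while the player is in the loop, slowly interpolates fog density toward a heavy maze fog.
; Otherwise it snaps back to the configured density and color, which the construction script also applies.
; Fog color stays constant, as the color interpolation is left unused.
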(event EventBeginPlay
  (bind _asplayer_character (Utilities|Casting|CastToPlayerCharacter (Game|GetPlayerCharacter 0)))
  (Variables|Default|SetPlayerRef _asplayer_character))

(event EventTick
  (params (DeltaSeconds :type Float%20%28single-precision%29))
  (Transformation|SetActorLocation (Transformation|GetActorLocation (Variables|Default|GetPlayerRef)) false true)
  (bind _returnvalue (Actor|GetActorOfClass "/Game/Blueprints/BP_LoopingSubLevelLoader.BP_LoopingSubLevelLoader_C"))
  (Utilities|IsValid _returnvalue
    (:Is%20Valid
      (if (Variables|/Game/Blueprints/BP_LoopingSubLevelLoader.BP_LoopingSubLevelLoader_C|GetPlayerInLoop _returnvalue)
        (CallFunction|SetMazeFog)
        (else
          (CallFunction|SetFogEffects :!label _label))))
    (:Is%20Not%20Valid
      (goto _label))))

(fn ConstructionScript
  (CallFunction|SetDefaultFog))

(fn SetFogEffects
  (Class|ExponentialHeightFogComponent|SetFogDensity (Variables|Default|GetExponentialHeightFog) (Variables|Default|GetFogDensity))
  (Class|ExponentialHeightFogComponent|SetFogInscatteringColor (Variables|Default|GetExponentialHeightFog) (Variables|Default|GetFogColor)))

(fn SetDefaultFog
  (bind _exponentialheightfog (Variables|Default|GetExponentialHeightFog))
  (Class|ExponentialHeightFogComponent|SetFogDensity _exponentialheightfog (Variables|Default|GetFogDensity))
  (Class|ExponentialHeightFogComponent|SetFogInscatteringColor _exponentialheightfog (Variables|Default|GetFogColor)))

(fn SetMazeFog
  (bind _exponentialheightfog (Variables|Default|GetExponentialHeightFog))
  (Class|ExponentialHeightFogComponent|SetFogDensity _exponentialheightfog (Math|Interpolation|FInterpTo (Variables|/Script/Engine.ExponentialHeightFogComponent|GetFogDensity _exponentialheightfog) 6.0 (Utilities|Time|GetWorldDeltaSeconds) 0.1))
  (Class|ExponentialHeightFogComponent|SetFogInscatteringColor (Variables|Default|GetExponentialHeightFog) (Variables|Default|GetFogColor)))