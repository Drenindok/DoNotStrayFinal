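; Spawnable sound actor that plays a preassigned sound, such as a monster's, or picks a random ambient one for the surface beneath it.
; A downward trace's physical surface selects a sound list, then a weighted random roll chooses the entry.
; The entry drives fade-in, volume and optional random start time.
; With a positive duration, the sound fades out after a random delay, and the actor polls each tick until playback stops, then destroys itself.
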(event EventBeginPlay
  (bind _selectedsound (Variables|Default|GetSelectedSound))
  (bind _selectedsound_2 (Variables|Default|GetSelectedSound))
  (bind _audio (Variables|Default|GetAudio))
  ;[1 1 1] If sound was already picked (meaning its a monster sound), just play that sound instead of picking a random environmental sound
  (if (!= (.sound _selectedsound_2) 0)
    (Audio|Components|Audio|SetSound _audio (.sound _selectedsound_2))
    (else
      (|Setenvironmentsound)))
  (Audio|Components|Audio|FadeIn _audio (.fadein _selectedsound) (.volume _selectedsound) (Math|Float|SelectFloat (Math|Random|RandomFloatinRange 0.0 (Variables|/Script/Engine.SoundBase|GetDuration (.sound _selectedsound))) 0.0 (.randomstarttime _selectedsound)) "Linear" :!class /Script/Engine.AudioComponent)
  (if (> (.minduration _selectedsound) 0.0)
    (Utilities|FlowControl|Delay (Math|Random|RandomFloatinRange (.minduration _selectedsound) (.maxduration _selectedsound)))
    (Audio|Components|Audio|FadeOut (Variables|Default|GetAudio) (.fadeout _selectedsound) 0.0 "Linear" :!class /Script/Engine.AudioComponent)
    (if (Audio|Components|Audio|IsPlaying (Variables|Default|GetAudio)) :!label _label
      (Utilities|FlowControl|Delay 0.0)
      (goto _label)
      (else
        (Actor|DestroyActor)))))

(fn ConstructionScript)

(fn WeightedRandom
  (params (Chances :type Array%20of%20Floats%20%28single-precision%29))
  (for _array_element Chances
    (LocalVariables|SetTotalWeight (+ (LocalVariables|GetTotalWeight) _array_element)))
  (LocalVariables|SetRandomWeight (Math|Random|RandomFloatinRange 0.0 (LocalVariables|GetTotalWeight)))
  (for (_array_element_2 _array_index) 0
    (bind _output_get (LocalVariables|SetCurrentWeight (+ (LocalVariables|GetCurrentWeight) _array_element_2)))
    (if (< (LocalVariables|GetRandomWeight) _output_get)
      (return _array_index))))