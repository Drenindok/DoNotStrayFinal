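; Basic controls tutorial actor that teaches looking, walking, sprinting and flashlight toggling through HUD messages.
; StartTutorials enables input checks immediately, then after a delay queues prompts from the current step onward, skipping any already completed.
; Tick polls mouse delta, horizontal speed and flashlight state to advance steps and clear prompts, destroying the actor after the last.
; A crouch prompt exists but is never run.
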(event Custom|Start%20Tutorials
  (Variables|Default|SetCheck%20For%20Player's%20Inputs true)
  (bind _asplayer_character (Utilities|Casting|CastToPlayerCharacter (Game|GetPlayerCharacter 0)))
  (Variables|Default|SetPlayerRef _asplayer_character)
  (Utilities|FlowControl|Delay 16.0)
  (switch int (Variables|Default|GetCurrentTutorialNumber)
    (:1
      (Default|QueTutorialMessage (Variables|/Game/Blueprints/ThirdPersonBP/Blueprints/PlayerCharacter.PlayerCharacter_C|GetHUDref (Variables|Default|GetPlayerRef)) (Utilities|Struct|MakeVar_TutorialPopup "Move the MOUSE to look around." -1.0))
      (Utilities|FlowControl|Delay 0.0)
      (Default|QueTutorialMessage (Variables|/Game/Blueprints/ThirdPersonBP/Blueprints/PlayerCharacter.PlayerCharacter_C|GetHUDref (Variables|Default|GetPlayerRef)) (Utilities|Struct|MakeVar_TutorialPopup "Press the WASD keys to move." -1.0) :!label _label)
      (Utilities|FlowControl|Delay 0.0)
      (Default|QueTutorialMessage (Variables|/Game/Blueprints/ThirdPersonBP/Blueprints/PlayerCharacter.PlayerCharacter_C|GetHUDref (Variables|Default|GetPlayerRef)) (Utilities|Struct|MakeVar_TutorialPopup "Hold SHIFT while moving FORWARD (W) to sprint." -1.0) :!label _label_2)
      (Utilities|FlowControl|Delay 0.0))
    (:2
      (goto _label))
    (:3
      (goto _label_2))
    (:4
      _))
  (Default|QueTutorialMessage (Variables|/Game/Blueprints/ThirdPersonBP/Blueprints/PlayerCharacter.PlayerCharacter_C|GetHUDref (Variables|Default|GetPlayerRef)) (Utilities|Struct|MakeVar_TutorialPopup "RIGHT CLICK to turn your light on and off." -1.0)))

(event Custom|CustomEvent_0)

(event EventTick
  (params (DeltaSeconds :type Float%20%28single-precision%29))
  (bind _returnvalue (Game|GetPlayerController 0))
  (bind (_deltax _deltay) (Class|PlayerController|GetInputMouseDelta _returnvalue))
  (if (Variables|Default|GetCheck%20For%20Player's%20Inputs)
    (switch int (Variables|Default|GetCurrentTutorialNumber)
      (:1
        (if (> (+ (Math|Float|Absolute(Float) _deltax) (Math|Float|Absolute(Float) _deltay)) 0.1)
          (Variables|Default|SetCurrentTutorialNumber 2)
          (Default|ClearandDisplayNextTutorialMessage (Variables|/Game/Blueprints/ThirdPersonBP/Blueprints/PlayerCharacter.PlayerCharacter_C|GetHUDref (Variables|Default|GetPlayerRef)) :!label _label)))
      (:2
        (if (> (Math|Vector|VectorLength (* (Transformation|GetVelocity (Variables|Default|GetPlayerRef)) "1.000000,1.000000, 0")) 5e+01)
          (Variables|Default|SetCurrentTutorialNumber 3)
          (goto _label)))
      (:3
        (if (> (Math|Vector|VectorLength (* (Transformation|GetVelocity (Variables|Default|GetPlayerRef)) "1.000000,1.000000, 0")) 5.5e+02)
          (Variables|Default|SetCurrentTutorialNumber 4)
          (goto _label)))
      (:4
        (if (Variables|/Game/Blueprints/ThirdPersonBP/Blueprints/PlayerCharacter.PlayerCharacter_C|GetFlashlightOn (Variables|Default|GetPlayerRef))
          (Utilities|FlowControl|Sequence
            (:then_0
              (Utilities|FlowControl|DoOnce true :!label _label_2
                (:Completed
                  (bind _output_get (Variables|Default|SetPlayer%20Has%20Turned%20Light%20On true))
                  (if (and _output_get (stale _output_get_2))
                    (Variables|Default|SetCurrentTutorialNumber 5)
                    (Utilities|FlowControl|Sequence
                      (:then_0
                        (goto _label))
                      (:then_1
                        (Utilities|FlowControl|Delay 1.0)
                        (Actor|DestroyActor)))))))
            (:then_1
              (goto _label_3 Reset)))
          (else
            (Utilities|FlowControl|Sequence
              (:then_0
                (Utilities|FlowControl|DoOnce true :!label _label_3
                  (:Completed
                    (bind _output_get_2 (Variables|Default|SetPlayer%20Has%20Turned%20Light%20Off true)))))
              (:then_1
                (goto _label_2 Reset)))))))))

(fn ConstructionScript)