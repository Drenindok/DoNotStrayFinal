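; Looping maze logic actor that updates bloody trails according to maze progress.
; UpdateBloodTrails loops over every BP_BloodyPathGenerator, clearing each one and, within the same loop, regenerating those whose tag matches MazeProgress.
; The first stage selects the "Path To Web" generators and the second selects "Path To Escape".
; BeginPlay caches the player character, which the trail update does not use.
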(event Custom|Update%20Blood%20Trails
  (bind _outactors (Actor|GetAllActorsOfClass "/Game/Blueprints/BP_BloodyPathGenerator.BP_BloodyPathGenerator_C"))
  (for _array_element _outactors
    (Default|ClearPath _array_element)
    (switch int (Variables|Default|GetMazeProgress)
      (:1
        (bind _outactors_2 (Actor|GetAllActorsOfClasswithTag "/Game/Blueprints/BP_BloodyPathGenerator.BP_BloodyPathGenerator_C" "Path To Web"))
        (for _array_element_2 _outactors_2
          (Default|Generate _array_element_2)))
      (:2
        (bind _outactors_3 (Actor|GetAllActorsOfClasswithTag "/Game/Blueprints/BP_BloodyPathGenerator.BP_BloodyPathGenerator_C" "Path To Escape"))
        (for _array_element_3 _outactors_3
          (Default|Generate _array_element_3))))))

(event EventBeginPlay
  (bind _asplayer_character (Utilities|Casting|CastToPlayerCharacter (Game|GetPlayerCharacter 0)))
  (Variables|Default|SetPlayerRef _asplayer_character))

(fn ConstructionScript)