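; Construction-script helper that holds a list of footprint transforms for a bloody path in the Repressed World.
; With Visualize on, it previews them as instanced static meshes offset by actor location, heavily scaled down, with X scale taken from Z.
; Otherwise, the one-shot OffsetToNewLocation toggle subtracts NewLocation from every stored footprint location, then resets both the toggle and the offset.
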(fn ConstructionScript
  (bind _footprints (Variables|Default|GetFootprints))
  (if (Variables|Default|GetVisualize)
    (for _array_element (Variables|Default|GetFootprints)
      (Class|InstancedStaticMeshComponent|AddInstanceWorldSpace (Variables|Default|GetInstancedStaticMesh) (Math|Transform|MakeTransform (+ (.location _array_element) (Transformation|GetActorLocation)) (.rotation _array_element) (Math|Vector|MakeVector (.z (* (.scale _array_element) 0.02)) (.y (* (.scale _array_element) 0.02)) (.z (* (.scale _array_element) 0.02))))))
    (elif (Variables|Default|GetOffsetToNewLocation)
      (Variables|Default|SetOffsetToNewLocation false)
      (for (_array_element_2 _array_index) _footprints
        (Utilities|Array|SetArrayElem _footprints _array_index (Math|Transform|MakeTransform (- (.location _array_element_2) (Variables|Default|GetNewLocation)) (.rotation _array_element_2) (.scale _array_element_2))))
      (Variables|Default|SetNewLocation "0, 0, 0"))))