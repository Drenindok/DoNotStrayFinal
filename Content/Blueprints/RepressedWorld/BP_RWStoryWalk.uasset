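; BP_RWStoryWalk is a collectible post in the Repressed World that the player can collect only once per save.
; On activation it adds itself to the player save's SpecificPostsCollected list, spawns a twilight squares explosion and destroys itself.
; Shortly after BeginPlay it destroys itself if the save already lists it.
; The ThoughtsTrigger sphere overlap runs into a DoOnce with nothing connected after it.
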(event OnComponentBeginOverlap(ThoughtsTrigger)
  (params (OverlappedComponent :type Primitive%20Component%20Object%20Reference) (OtherActor :type Actor%20Object%20Reference) (OtherComp :type Primitive%20Component%20Object%20Reference) (OtherBodyIndex :type Integer) (bFromSweep :type Boolean) (SweepResult :type Hit%20Result%20Structure%20%28by%20ref%29))
  ;[0 0.1521 1] Sphere trigger
  (Utilities|FlowControl|DoOnce false))

(event Custom|Activated
  (|Addposttopostsplayerhascollected))

(event EventBeginPlay
  (bind _asrepressed_world_character (Utilities|Casting|CastToRepressedWorldCharacter (Game|GetPlayerCharacter 0)))
  (Variables|Default|SetPlayer%20Ref _asrepressed_world_character)
  (Utilities|FlowControl|Delay 0.2)
  (if (Utilities|Array|ContainsItem (Variables|/Game/Save_SaveGame.Save_SaveGame_C|GetSpecificPostsCollected (Variables|/Game/Blueprints/ThirdPersonBP/Blueprints/RepressedWorldCharacter.RepressedWorldCharacter_C|GetSaveGame (Variables|Default|GetPlayer%20Ref))) self)
    (Actor|DestroyActor)))

(fn ConstructionScript)