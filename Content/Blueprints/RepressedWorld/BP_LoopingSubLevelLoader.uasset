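; Creates a seamlessly repeating world by tiling copies of a sublevel around the origin and wrapping the player within the central tile.
; When ShowSubLevels is set, the construction script loads level instances in a 3D grid sized by RepeatsPerAxis, skipping the hand-placed center.
; Tick teleports the player back one tile spacing upon passing half that distance, correcting one axis per frame.
; Loading logic in the event graph is disconnected.
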(event EventBeginPlay
  (bind _asrepressed_world_character (Utilities|Casting|CastToRepressedWorldCharacter (Game|GetPlayerCharacter 0)))
  ;[1 1 1] New method
  (Variables|Default|SetPlayerRef _asrepressed_world_character))

(event EventTick
  (params (DeltaSeconds :type Float%20%28single-precision%29))
  (bind _playerref (Variables|Default|GetPlayerRef))
  (bind _playerref_2 (Variables|Default|GetPlayerRef))
  (bind _distancebetweenworlds (Variables|Default|GetDistanceBetweenWorlds))
  (bind _playerref_3 (Variables|Default|GetPlayerRef))
  (bind _distancebetweenworlds_2 (Variables|Default|GetDistanceBetweenWorlds))
  (bind _playerref_4 (Variables|Default|GetPlayerRef))
  (bind _distancebetweenworlds_3 (Variables|Default|GetDistanceBetweenWorlds))
  (bind _playerref_5 (Variables|Default|GetPlayerRef))
  (bind _playerref_6 (Variables|Default|GetPlayerRef))
  (bind _distancebetweenworlds_4 (Variables|Default|GetDistanceBetweenWorlds))
  (bind _distancebetweenworlds_5 (Variables|Default|GetDistanceBetweenWorlds))
  (bind _distancebetweenworlds_6 (Variables|Default|GetDistanceBetweenWorlds))
  (bind _returnvalue (Transformation|GetActorLocation _playerref_5))
  (bind _returnvalue_2 (Transformation|GetActorLocation _playerref_6))
  (bind _returnvalue_3 (Transformation|GetActorLocation _playerref_2))
  (bind _returnvalue_4 (Transformation|GetActorLocation _playerref))
  (bind _returnvalue_5 (Transformation|GetActorLocation _playerref_4))
  (bind _returnvalue_6 (Transformation|GetActorLocation _playerref_3))
  ;[1 1 1] Too far on positive X
  (if (> (.x (Transformation|GetActorLocation (Variables|Default|GetPlayerRef))) (* (.x _distancebetweenworlds) 0.5))
    (Transformation|SetActorLocation _playerref (Math|Vector|MakeVector (- (.x _returnvalue_4) (.x _distancebetweenworlds)) (.y _returnvalue_4) (.z _returnvalue_4)) false true)
    (else
      ;[1 1 1] Too far on negative X
      (if (< (.x (Transformation|GetActorLocation (Variables|Default|GetPlayerRef))) (* (.x _distancebetweenworlds_3) -0.5))
        (Transformation|SetActorLocation _playerref_4 (Math|Vector|MakeVector (+ (.x _returnvalue_5) (.x _distancebetweenworlds_3)) (.y _returnvalue_5) (.z _returnvalue_5)) false true)
        (else
          ;[1 1 1] Too far on positive Y
          (if (> (.y (Transformation|GetActorLocation (Variables|Default|GetPlayerRef))) (* (.y _distancebetweenworlds_4) 0.5))
            (Transformation|SetActorLocation _playerref_5 (Math|Vector|MakeVector (.x _returnvalue) (- (.y _returnvalue) (.y _distancebetweenworlds_4)) (.z _returnvalue)) false true)
            (else
              ;[1 1 1] Too far on negative Y
              (if (< (.y (Transformation|GetActorLocation (Variables|Default|GetPlayerRef))) (* (.y _distancebetweenworlds_5) -0.5))
                (Transformation|SetActorLocation _playerref_6 (Math|Vector|MakeVector (.x _returnvalue_2) (+ (.y _returnvalue_2) (.y _distancebetweenworlds_5)) (.z _returnvalue_2)) false true)
                (else
                  ;[1 1 1] Too far on positive Z
                  (if (> (.z (Transformation|GetActorLocation (Variables|Default|GetPlayerRef))) (* (.z _distancebetweenworlds_2) 0.5))
                    (Transformation|SetActorLocation _playerref_2 (Math|Vector|MakeVector (.x _returnvalue_3) (.y _returnvalue_3) (- (.z _returnvalue_3) (.z _distancebetweenworlds_2))) false true)
                    (else
                      ;[1 1 1] Too far on negative Z
                      (if (< (.z (Transformation|GetActorLocation (Variables|Default|GetPlayerRef))) (* (.z _distancebetweenworlds_6) -0.5))
                        (Transformation|SetActorLocation _playerref_3 (Math|Vector|MakeVector (.x _returnvalue_6) (.y _returnvalue_6) (+ (.z _returnvalue_6) (.z _distancebetweenworlds_6))) false true)))))))))))))

(fn ConstructionScript
  (bind _repeatsperaxis (Variables|Default|GetRepeatsPerAxis))
  (Variables|Default|SetTotalTilesPerAxis (+ _repeatsperaxis (+ _repeatsperaxis "1.000000,1.000000,1.000000")))
  (Utilities|FlowControl|Sequence
    (:then_1
      (Variables|Default|SetInstanceNumber 0)
      ;[1 1 1] New method
      (if (Variables|Default|GetShowSubLevels)
        (for _index (range 0 (Math|Float|Truncate (- (.x (Variables|Default|GetTotalTilesPerAxis)) 1.0)))
          (for _index_2 (range 0 (Math|Float|Truncate (- (.y (Variables|Default|GetTotalTilesPerAxis)) 1.0)))
            (for _index_3 (range 0 (Math|Float|Truncate (- (.z (Variables|Default|GetTotalTilesPerAxis)) 1.0)))
              (if (not (Math|Vector|Equal(Vector) (- (* (Variables|Default|GetDistanceBetweenWorlds) (Math|Vector|MakeVector (Math|Conversions|ToFloat(Integer) _index) (Math|Conversions|ToFloat(Integer) _index_2) (Math|Conversions|ToFloat(Integer) _index_3))) (* (Variables|Default|GetDistanceBetweenWorlds) (Variables|Default|GetRepeatsPerAxis))) "0, 0, 0" 0.0001))
                (Class|LevelStreamingDynamic|LoadLevelInstancebySoftObjectPtr (Variables|Default|GetLevel) (- (* (Variables|Default|GetDistanceBetweenWorlds) (Math|Vector|MakeVector (Math|Conversions|ToFloat(Integer) _index) (Math|Conversions|ToFloat(Integer) _index_2) (Math|Conversions|ToFloat(Integer) _index_3))) (* (Variables|Default|GetDistanceBetweenWorlds) (Variables|Default|GetRepeatsPerAxis))) "0, 0, 0")))))))))