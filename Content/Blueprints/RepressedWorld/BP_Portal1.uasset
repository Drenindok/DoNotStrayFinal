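; Door that can link to another door as a see-through, walk-through portal, or work as a lockable ordinary door.
; While the player is near and the door renders, it positions the partner's scene capture to mirror the player camera.
; A collider teleports the player to the partner, rotating view and velocity by the yaw difference.
; Linked doors open and close in sync, and auto-close once the player leaves both radii.
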(event OnComponentBeginOverlap(TeleportCollider)
  (params (OverlappedComponent :type Primitive%20Component%20Object%20Reference) (OtherActor :type Actor%20Object%20Reference) (OtherComp :type Primitive%20Component%20Object%20Reference) (OtherBodyIndex :type Integer) (bFromSweep :type Boolean) (SweepResult :type Hit%20Result%20Structure%20%28by%20ref%29))
  (bind _returnvalue (Game|GetPlayerController 0))
  (bind _returnvalue_2 (Transformation|GetActorRotation))
  (bind _otherportal (Variables|Default|GetOtherPortal))
  (bind _playerref (Variables|Default|GetPlayerRef))
  (bind _output (Utilities|ResolveSoftReference _otherportal))
  (bind _cameraarm (Variables|/Game/Blueprints/ThirdPersonBP/Blueprints/RepressedWorldCharacter.RepressedWorldCharacter_C|GetCameraArm _playerref))
  (bind _charactermovement (Variables|/Script/Engine.Character|GetCharacterMovement _playerref))
  (bind _returnvalue_3 (Transformation|GetActorRotation _output))
  (bind _returnvalue_4 (- (.yaw _returnvalue_2) (.yaw _returnvalue_3)))
  (bind _returnvalue_5 (* _returnvalue_4 -1.0))
  (bind _returnvalue_6 (- _returnvalue_5 1.8e+02))
  (bind _returnvalue_7 (Math|Rotator|MakeRotator 0.0 0.0 _returnvalue_6))
  ;[1 1 1] Teleport the player when they overlap the teleport collider
  (if (Variables|Default|GetPortalLinked)
    (Variables|/Game/Blueprints/RepressedWorld/BP_Portal2.BP_Portal2_C|SetPlayerCloseToDoor (Utilities|ResolveSoftReference (Variables|Default|GetOtherPortal)) true)
    (Transformation|SetActorLocation (Variables|Default|GetPlayerRef) (Transformation|GetWorldLocation (Variables|/Game/Blueprints/RepressedWorld/BP_Portal2.BP_Portal2_C|GetSpawnArrow (Utilities|ResolveSoftReference (Variables|Default|GetOtherPortal)))) false true)
    (Variables|/Script/Engine.SpringArmComponent|SetbEnableCameraRotationLag _cameraarm false)
    (Pawn|SetControlRotation _returnvalue (Math|Rotator|CombineRotators (Pawn|GetControlRotation _returnvalue :!class /Script/Engine.Controller) _returnvalue_7))
    (Variables|/Script/Engine.MovementComponent|SetVelocity _charactermovement (Math|Vector|RotateVector (Variables|/Script/Engine.MovementComponent|GetVelocity _charactermovement) _returnvalue_7))
    (Utilities|FlowControl|Delay 0.0)
    (Variables|/Script/Engine.SpringArmComponent|SetbEnableCameraRotationLag _cameraarm true)))

(event OnComponentBeginOverlap(PortalPlane)
  (params (OverlappedComponent :type Primitive%20Component%20Object%20Reference) (OtherActor :type Actor%20Object%20Reference) (OtherComp :type Primitive%20Component%20Object%20Reference) (OtherBodyIndex :type Integer) (bFromSweep :type Boolean) (SweepResult :type Hit%20Result%20Structure%20%28by%20ref%29))
  ;[1 1 1] When you overlap the portal plane (meaning you are on the right side),
  ; disable the collider blocking the player from entering
  (if (Variables|Default|GetPortalLinked)
    (Collision|SetCollisionEnabled (Variables|Default|GetWrongWayBlocker) "NoCollision")))

(event OnComponentEndOverlap(PortalPlane)
  (params (OverlappedComponent :type Primitive%20Component%20Object%20Reference) (OtherActor :type Actor%20Object%20Reference) (OtherComp :type Primitive%20Component%20Object%20Reference) (OtherBodyIndex :type Integer))
  ;[1 1 1] When you overlap the portal plane (meaning you are on the right side),
  ; disable the collider blocking the player from entering
  (if (Variables|Default|GetPortalLinked)
    (Collision|SetCollisionEnabled (Variables|Default|GetWrongWayBlocker) "QueryAndPhysics")))

(event OnComponentBeginOverlap(TooFarRadius)
  (params (OverlappedComponent :type Primitive%20Component%20Object%20Reference) (OtherActor :type Actor%20Object%20Reference) (OtherComp :type Primitive%20Component%20Object%20Reference) (OtherBodyIndex :type Integer) (bFromSweep :type Boolean) (SweepResult :type Hit%20Result%20Structure%20%28by%20ref%29))
  (Variables|Default|SetPlayerCloseToDoor true))

(event OnComponentEndOverlap(TooFarRadius)
  (params (OverlappedComponent :type Primitive%20Component%20Object%20Reference) (OtherActor :type Actor%20Object%20Reference) (OtherComp :type Primitive%20Component%20Object%20Reference) (OtherBodyIndex :type Integer))
  (bind _doormesh (Variables|Default|GetDoorMesh))
  (bind _otherportal (Variables|Default|GetOtherPortal))
  (bind _doormesh_2 (Variables|Default|GetDoorMesh))
  (bind _output (Utilities|ResolveSoftReference _otherportal))
  (Variables|Default|SetPlayerCloseToDoor false)
  (Utilities|IsValid _output
    (:Is%20Valid
      (if (not (Variables|/Game/Blueprints/RepressedWorld/BP_Portal2.BP_Portal2_C|GetPlayerCloseToDoor _output))
        (if (Variables|Default|GetOpened) :!label _label
          ;[1 1 1] Opening/closing door
          ;;[1 1 1] If this is linked to another door, open/close that door as well
          (if (Variables|Default|GetPortalLinked)
            (Default|Open/CloseDoor (Utilities|ResolveSoftReference (Variables|Default|GetOtherPortal)) (not (Variables|Default|GetOpened))))
          (if (Variables|Default|GetOpened)
            (Transformation|SetRelativeLocationAndRotation _doormesh_2 "-5.000000,-45.000000, 0" "0,180.000000, 0" false true) ; reset door to starting position, to make sure the door syncs with\nother door
            (Components|MoveComponentTo _doormesh "-5.000000,-45.000000, 0" "0,90.000000, 0" true false 1.0 false) ; close
            (Audio|PlaySoundatLocation "/Game/Audio/Door/wav_door_close.wav_door_close" (Transformation|GetActorLocation) "0, 0, 0" 1.0 1.0 0.0 "/Game/Audio/Atten_MonsterNoises.Atten_MonsterNoises" 0 0)
            (Variables|Default|SetOpened false)
            (else
              (Transformation|SetRelativeLocationAndRotation _doormesh_2 "-5.000000,-45.000000, 0" "0,90.000000, 0" false true) ; reset door to starting position, to make sure the door syncs with\nother door
              (Audio|PlaySoundatLocation "/Game/Audio/Door/wav_door_open.wav_door_open" (Transformation|GetActorLocation) "0, 0, 0" 1.0 1.0 0.0 "/Game/Audio/Atten_MonsterNoises.Atten_MonsterNoises" 0 0)
              (Components|MoveComponentTo _doormesh "-5.000000,-45.000000, 0" "0,180.000000, 0" true false 1.0 false) ; open
              (Variables|Default|SetOpened true)))
          (Variables|Default|SetDoorMoving false))))
    (:Is%20Not%20Valid
      (goto _label))))

(event Custom|Activated
  (bind _doormesh (Variables|Default|GetDoorMesh))
  (bind _doormesh_2 (Variables|Default|GetDoorMesh))
  ;[1 1 1] Opening/closing door
  (if (Variables|Default|GetLocked)
    (Audio|PlaySoundatLocation "/Game/Audio/Door/wav_door_locked.wav_door_locked" (Transformation|GetActorLocation) "0, 0, 0" 1.0 1.0 0.0 "/Game/Audio/Atten_MonsterNoises.Atten_MonsterNoises" 0 0)
    (else
      ;;[1 1 1] If door is already moving due to player moving it, don't
      ;; let the player move it again
      (if (not (Variables|Default|GetDoorMoving))
        (Variables|Default|SetDoorMoving true)
        ;;[1 1 1] If this is linked to another door, open/close that door as well
        (if (Variables|Default|GetPortalLinked)
          (Default|Open/CloseDoor (Utilities|ResolveSoftReference (Variables|Default|GetOtherPortal)) (not (Variables|Default|GetOpened))))
        (if (Variables|Default|GetOpened)
          (Transformation|SetRelativeLocationAndRotation _doormesh_2 "-5.000000,-45.000000, 0" "0,180.000000, 0" false true) ; reset door to starting position, to make sure the door syncs with\nother door
          (Components|MoveComponentTo _doormesh "-5.000000,-45.000000, 0" "0,90.000000, 0" true false 1.0 false) ; close
          (Audio|PlaySoundatLocation "/Game/Audio/Door/wav_door_close.wav_door_close" (Transformation|GetActorLocation) "0, 0, 0" 1.0 1.0 0.0 "/Game/Audio/Atten_MonsterNoises.Atten_MonsterNoises" 0 0)
          (Variables|Default|SetOpened false)
          (else
            (Transformation|SetRelativeLocationAndRotation _doormesh_2 "-5.000000,-45.000000, 0" "0,90.000000, 0" false true) ; reset door to starting position, to make sure the door syncs with\nother door
            (Audio|PlaySoundatLocation "/Game/Audio/Door/wav_door_open.wav_door_open" (Transformation|GetActorLocation) "0, 0, 0" 1.0 1.0 0.0 "/Game/Audio/Atten_MonsterNoises.Atten_MonsterNoises" 0 0)
            (Components|MoveComponentTo _doormesh "-5.000000,-45.000000, 0" "0,180.000000, 0" true false 1.0 false) ; open
            (Variables|Default|SetOpened true)))
        (Variables|Default|SetDoorMoving false)))))

(event Custom|Open/CloseDoor
  (params (Open :type Boolean))
  (bind _doormesh (Variables|Default|GetDoorMesh))
  (bind _doormesh_2 (Variables|Default|GetDoorMesh))
  ;[1 1 1] Opening/closing door
  (Variables|Default|SetOpened (not Open)) ; set starting position of door to be the opposite of\nwhen end result should be (so if door is supposed\nto be opened, it has to start closed)
  (Variables|Default|SetDoorMoving true)
  (if (Variables|Default|GetOpened)
    (Transformation|SetRelativeLocationAndRotation _doormesh_2 "-5.000000,-45.000000, 0" "0,180.000000, 0" false true) ; reset door to starting position, to make sure the door syncs with\nother door
    (Components|MoveComponentTo _doormesh "-5.000000,-45.000000, 0" "0,90.000000, 0" true false 1.0 false) ; close
    (Audio|PlaySoundatLocation "/Game/Audio/Door/wav_door_close.wav_door_close" (Transformation|GetActorLocation) "0, 0, 0" 1.0 1.0 0.0 "/Game/Audio/Atten_MonsterNoises.Atten_MonsterNoises" 0 0)
    (Variables|Default|SetOpened false)
    (else
      (Transformation|SetRelativeLocationAndRotation _doormesh_2 "-5.000000,-45.000000, 0" "0,90.000000, 0" false true) ; reset door to starting position, to make sure the door syncs with\nother door
      (Audio|PlaySoundatLocation "/Game/Audio/Door/wav_door_open.wav_door_open" (Transformation|GetActorLocation) "0, 0, 0" 1.0 1.0 0.0 "/Game/Audio/Atten_MonsterNoises.Atten_MonsterNoises" 0 0)
      (Components|MoveComponentTo _doormesh "-5.000000,-45.000000, 0" "0,180.000000, 0" true false 1.0 false) ; open
      (Variables|Default|SetOpened true)))
  (Variables|Default|SetDoorMoving false))

(event EventBeginPlay
  ;[1 1 1] Set reference to player
  (bind _asrepressed_world_character (Utilities|Casting|CastToRepressedWorldCharacter (Game|GetPlayerCharacter 0)))
  (Variables|Default|SetPlayerRef _asrepressed_world_character))

(event EventTick
  (params (DeltaSeconds :type Float%20%28single-precision%29))
  (bind _returnvalue (Class|Actor|WasRecentlyRendered 0.2))
  (bind _portalplane (Variables|Default|GetPortalPlane))
  (bind _otherportal (Variables|Default|GetOtherPortal))
  (bind _output (Utilities|ResolveSoftReference _otherportal))
  (bind _portalview (Variables|/Game/Blueprints/RepressedWorld/BP_Portal2.BP_Portal2_C|GetPortalView _output))
  ;[1 1 1] Set other door's camera to record or not record
  (if (Variables|Default|GetPortalLinked)
    (if (Variables|Default|GetPlayerCloseToDoor)
      (Variables|/Script/Engine.SceneCaptureComponent|SetbCaptureEveryFrame _portalview _returnvalue)
      (Rendering|SetVisibility _portalplane true true)
      (if _returnvalue
        (CallFunction|Update2ndCameraPosition))
      (else
        (Variables|/Script/Engine.SceneCaptureComponent|SetbCaptureEveryFrame _portalview false)
        (Rendering|SetVisibility _portalplane false true)))))

(fn ConstructionScript
  (CallFunction|SetPortalLinked (Variables|Default|GetOtherPortal)))

(fn SetPortalLinked
  (params (OtherPortal :type BP%20Portal%202%20Soft%20Object%20Reference))
  (bind _output_get (Variables|Default|SetPortalLinked (Utilities|IsValidSoftObjectReference OtherPortal)))
  (if _output_get
    (Variables|Default|SetOtherPortal OtherPortal)
    (Collision|SetCollisionEnabled (Variables|Default|GetWrongWayBlocker) "QueryAndPhysics")
    (else
      (Rendering|SetVisibility (Variables|Default|GetPortalPlane) false true)
      (Collision|SetCollisionEnabled (Variables|Default|GetWrongWayBlocker) "NoCollision"))))

(event Custom|Update2ndCameraPosition
  (bind _returnvalue (Game|GetPlayerCameraManager 0))
  (bind _doorangle (|Inputs))
  (bind _transformcomponent (Variables|/Script/Engine.PlayerCameraManager|GetTransformComponent _returnvalue))
  (bind _returnvalue_2 (Transformation|GetWorldLocation _transformcomponent))
  (Transformation|SetWorldLocationAndRotation (Variables|/Game/Blueprints/RepressedWorld/BP_Portal2.BP_Portal2_C|GetPortalView (Utilities|ResolveSoftReference (Variables|Default|GetOtherPortal))) (+ _returnvalue_2 (- (Transformation|GetActorLocation (Utilities|ResolveSoftReference (Variables|Default|GetOtherPortal))) (+ _returnvalue_2 (Math|Vector|RotateVector (- (Transformation|GetActorLocation) _returnvalue_2) _doorangle)))) (Math|Rotator|CombineRotators (Transformation|GetWorldRotation _transformcomponent) _doorangle) false true))