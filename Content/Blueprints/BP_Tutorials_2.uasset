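; Tutorial Blueprint that queues contextual hints on the player's HUD for hiding underwater, climbing and avoiding the monster.
; Tick advances staged water and bridge hints from player state and a forward sphere trace, clearing or resetting them as conditions change.
; When the monster first wanders close, a one-time warning interrupts those hints and suspends them until it expires.
; Basic movement, light and crouch prompts are present but disconnected.
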(event EventBeginPlay
  (bind _asplayer_character (Utilities|Casting|CastToPlayerCharacter (Game|GetPlayerCharacter 0)))
  (Variables|Default|SetPlayerRef _asplayer_character))

(event EventTick
  (params (DeltaSeconds :type Float%20%28single-precision%29))
  (bind _returnvalue (Game|GetPlayerCharacter 0))
  (bind _playerref (Variables|Default|GetPlayerRef))
  (bind _playerref_2 (Variables|Default|GetPlayerRef))
  (bind _returnvalue_2 (Pawn|GetControlRotation _returnvalue :!class /Script/Engine.Pawn))
  (bind _returnvalue_3 (Transformation|GetActorLocation _playerref))
  (bind _inwater (Variables|/Game/Blueprints/ThirdPersonBP/Blueprints/PlayerCharacter.PlayerCharacter_C|GetInWater _playerref_2))
  (bind _returnvalue_4 (Math|Vector|GetForwardVector _returnvalue_2))
  (bind _returnvalue_5 (* (.y _returnvalue_4) 1e+02))
  (bind _returnvalue_6 (* (.x _returnvalue_4) 1e+02))
  (bind _returnvalue_7 (Math|Vector|MakeVector _returnvalue_6 _returnvalue_5 (.z _returnvalue_4)))
  (bind _returnvalue_8 (+ _returnvalue_3 _returnvalue_7))
  (Utilities|FlowControl|Sequence
    (:then_0
      (if (not (Variables|Default|GetMonsterTutorialDisplayed))
        ;[1 1 1] Hiding underwater tutorial
        (switch int (Variables|Default|GetWaterTutorialStage)
          (:1
            (if (not (== (Variables|Default|GetBridgeTutorialStage) 2))
              (if _inwater
                (Variables|Default|SetWaterTutorialStage 2)
                (Default|QueTutorialMessage (Variables|/Game/Blueprints/ThirdPersonBP/Blueprints/PlayerCharacter.PlayerCharacter_C|GetHUDref (Variables|Default|GetPlayerRef)) (Utilities|Struct|MakeVar_TutorialPopup "Hold CTRL to hide underwater. Be careful not to drown." -1.0)))))
          (:2
            (if _inwater
              (if (Variables|/Game/Blueprints/ThirdPersonBP/Blueprints/PlayerCharacter.PlayerCharacter_C|GetHeadUnderwater (Variables|Default|GetPlayerRef))
                (Variables|Default|SetWaterTutorialStage 3)
                (Default|ClearandDisplayNextTutorialMessage (Variables|/Game/Blueprints/ThirdPersonBP/Blueprints/PlayerCharacter.PlayerCharacter_C|GetHUDref (Variables|Default|GetPlayerRef))))
              (else
                (Variables|Default|SetWaterTutorialStage 1)
                (Default|ClearandDisplayNextTutorialMessage (Variables|/Game/Blueprints/ThirdPersonBP/Blueprints/PlayerCharacter.PlayerCharacter_C|GetHUDref (Variables|Default|GetPlayerRef)))))))))
    (:then_1
      (if (not (Variables|Default|GetMonsterTutorialDisplayed))
        ;[1 1 1] Bridge climbing tutorial
        (switch int (Variables|Default|GetBridgeTutorialStage)
          (:1
            (bind _returnvalue_9 (Collision|SphereTraceByChannel _returnvalue_3 _returnvalue_8 5.0 "TraceTypeQuery4" false 0 "None"))
            (if _returnvalue_9
              ;;[1 1 1] Clears water tutorial away, if it is currently displayed
              (if (== (Variables|Default|GetWaterTutorialStage) 2)
                (Variables|Default|SetWaterTutorialStage 1)
                (Default|ClearandDisplayNextTutorialMessage (Variables|/Game/Blueprints/ThirdPersonBP/Blueprints/PlayerCharacter.PlayerCharacter_C|GetHUDref (Variables|Default|GetPlayerRef))))
              (Variables|Default|SetBridgeTutorialStage 2)
              (Default|QueTutorialMessage (Variables|/Game/Blueprints/ThirdPersonBP/Blueprints/PlayerCharacter.PlayerCharacter_C|GetHUDref (Variables|Default|GetPlayerRef)) (Utilities|Struct|MakeVar_TutorialPopup "Press SPACEBAR to jump and climb up onto things." -1.0))))
          (:2
            (bind _returnvalue_10 (Collision|SphereTraceByChannel _returnvalue_3 _returnvalue_8 5.0 "TraceTypeQuery4" false 0 "None"))
            (if _returnvalue_10
              (if (Variables|/Game/Blueprints/ThirdPersonBP/Blueprints/PlayerCharacter.PlayerCharacter_C|GetClimbingLedge (Variables|Default|GetPlayerRef))
                (Variables|Default|SetBridgeTutorialStage 3)
                (Default|ClearandDisplayNextTutorialMessage (Variables|/Game/Blueprints/ThirdPersonBP/Blueprints/PlayerCharacter.PlayerCharacter_C|GetHUDref (Variables|Default|GetPlayerRef)) :!label _label))
              (else
                (Variables|Default|SetBridgeTutorialStage 1)
                (goto _label)))))))
    (:then_2
      ;[1 1 1] Avoiding Monster Tutorial
      (if (Utilities|Enum|Equal(Enum) (Variables|/Game/Blueprints/Monster/MonsterCharacter.MonsterCharacter_C|GetBehaviourState (Variables|/Game/Blueprints/ThirdPersonBP/Blueprints/PlayerCharacter.PlayerCharacter_C|GetMonsterRef (Variables|Default|GetPlayerRef))) "WanderingClose")
        (Utilities|FlowControl|DoOnce false
          (:Completed
            (Variables|Default|SetMonsterTutorialDisplayed true)
            ;;[1 1 1] If in the middle of either tutorial, remove them for now.
            (Variables|Default|SetWaterTutorialStage (Math|Integer|SelectInt 1 (Variables|Default|GetWaterTutorialStage) (== (Variables|Default|GetWaterTutorialStage) 2)))
            (Variables|Default|SetBridgeTutorialStage (Math|Integer|SelectInt 1 (Variables|Default|GetBridgeTutorialStage) (== (Variables|Default|GetBridgeTutorialStage) 2)))
            (Default|ClearandDisplayNextTutorialMessage (Variables|/Game/Blueprints/ThirdPersonBP/Blueprints/PlayerCharacter.PlayerCharacter_C|GetHUDref (Variables|Default|GetPlayerRef)))
            (Default|QueTutorialMessage (Variables|/Game/Blueprints/ThirdPersonBP/Blueprints/PlayerCharacter.PlayerCharacter_C|GetHUDref (Variables|Default|GetPlayerRef)) (Utilities|Struct|MakeVar_TutorialPopup "Something approaches. Be quiet. Listen.  
It will hear you more easily when it stops moving.  
Only move when it moves." 16.0))
            (Utilities|FlowControl|Delay 16.0)
            (Variables|Default|SetMonsterTutorialDisplayed false)))))))

(fn ConstructionScript)