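; Activatable appears to be a component that handles activation of its owning actor, showing thoughts and triggering scripted events.
; Activated forwards to the owner's Activated function through a short named timer, then optionally passes styled, interruptible thought text to MainGameInstance.
; A TriggerEvent switch starts the car-entry cutscene or changes BP_LightingManager's lighting for visual testing.
; Disconnected leftover nodes hold an older in-place thought parser and display.
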(event Custom|Activated
  (Utilities|Time|SetTimerbyFunctionName (Components|GetOwner) "Activated" 0.01)
  (Utilities|FlowControl|Sequence
    (:then_0
      (if (Variables|Default|GetShowThought?)
        (Default|ShowThoughts (Variables|Default|GetGameInstanceRef) (Variables|Default|GetThoughts) (Variables|Default|GetFont) (Variables|Default|GetFont%20Color) false 25.0 0.0 0.0 true)))
    (:then_1
      ;[1 1 1] Trigger Events/Special code
      (switch string (Variables|Default|GetTriggerEvent)
        (:EnterCar%28NoEvidence%29
          (bind _outactors (Actor|GetAllActorsOfClass "/Game/Blueprints/CutscenesCinematics/BP_EnterCar_Cutscene.BP_EnterCar_Cutscene_C"))
          (Default|EnterCar (Utilities|Array|Get(acopy) _outactors)))
        (:DayLighting
          ;[1 1 1] Switch time of day (this is just for testing visuals in visual tests level
          (bind _outactors_2 (Actor|GetAllActorsOfClass "/Game/Blueprints/BP_LightingManager.BP_LightingManager_C"))
          (Default|SwitchtoSunny (Utilities|Array|Get(acopy) _outactors_2)))
        (:NightLighting
          (bind _outactors_3 (Actor|GetAllActorsOfClass "/Game/Blueprints/BP_LightingManager.BP_LightingManager_C"))
          (Default|SwitchtoNight (Utilities|Array|Get(acopy) _outactors_3)))
        (:RepressedLighting
          (bind _outactors_4 (Actor|GetAllActorsOfClass "/Game/Blueprints/BP_LightingManager.BP_LightingManager_C"))
          (Default|SwitchtoRepressed (Utilities|Array|Get(acopy) _outactors_4)))))))

(event EventBeginPlay
  (bind _asmain_game_instance (Utilities|Casting|CastToMainGameInstance (Game|GetGameInstance)))
  (Variables|Default|SetGameInstanceRef _asmain_game_instance))