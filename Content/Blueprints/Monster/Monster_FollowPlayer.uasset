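; Monster that follows the player, approaching with AI MoveTo whenever it is farther away than its acceptance radius.
; BeginPlay caches the player character, and Tick issues the move while rotating a fog particle to face the player's camera.
; Tick also flickers the spotlight with clamped random intensity steps and drives the eye material's brightness from a scaled, similarly randomized intensity.
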(event EventTick
  (params (DeltaSeconds :type Float%20%28single-precision%29))
  (bind _returnvalue (Math|Random|RandomFloatinRange -5e+02 5e+02))
  (bind _spotlight (Variables|Default|GetSpotLight))
  (bind _playerref (Variables|Default|GetPlayerRef))
  (bind _intensity (Variables|/Script/Engine.LightComponentBase|GetIntensity _spotlight))
  (bind _returnvalue_2 (+ _intensity _returnvalue))
  (bind _returnvalue_3 (Math|Float|Clamp(Float) _returnvalue_2 2.5e+03 5e+03))
  (Utilities|FlowControl|Sequence
    (:then_0
      (Transformation|SetWorldRotation (Variables|Default|GetFogParticle) (Math|Rotator|FindLookatRotation (Transformation|GetWorldLocation (Variables|Default|GetFogParticle)) (Transformation|GetWorldLocation (Variables|/Game/Blueprints/ThirdPersonBP/Blueprints/PlayerCharacter.PlayerCharacter_C|GetCamera (Variables|Default|GetPlayerRef)))) false false)
      (if (> (Math|Vector|VectorLength (- (Transformation|GetActorLocation (Variables|Default|GetPlayerRef)) (Transformation|GetActorLocation))) 3e+02)
        (AI|AIMoveTo self (Transformation|GetActorLocation _playerref) _playerref 3e+02 false)))
    (:then_1
      (Rendering|Components|Light|SetIntensity _spotlight _returnvalue_3)
      (Rendering|Material|SetScalarParameterValueonMaterials (Variables|Default|GetEye) "Brightness" (* _returnvalue_3 0.01)))))

(event EventBeginPlay
  (bind _asplayer_character (Utilities|Casting|CastToPlayerCharacter (Game|GetPlayerCharacter 0)))
  (Variables|Default|SetPlayerRef _asplayer_character))

(fn ConstructionScript)