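; Ambience controller that crossfades swamp and forest sounds based on the player's height.
; On BeginPlay it caches the player character, then every Tick maps that character's Z position through a clamped range.
; The result sets the swamp audio component's volume multiplier and its inverse sets the forest's, so swamp dominates low down and forest higher up.
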(event EventTick
  (params (DeltaSeconds :type Float%20%28single-precision%29))
  (bind _playerref (Variables|Default|GetPlayerRef))
  (bind _returnvalue (Transformation|GetActorLocation _playerref))
  (bind _returnvalue_2 (Math|Float|MapRangeClamped (.z _returnvalue) 4e+02 1.4e+03 1.0 0.0))
  (Audio|Components|Audio|SetVolumeMultiplier (Variables|/Script/Engine.AmbientSound|GetAudioComponent (Utilities|ResolveSoftReference (Variables|Default|GetSwampAmbience))) _returnvalue_2 :!class /Script/Engine.AudioComponent)
  (Audio|Components|Audio|SetVolumeMultiplier (Variables|/Script/Engine.AmbientSound|GetAudioComponent (Utilities|ResolveSoftReference (Variables|Default|GetForestAmbience))) (- 1.0 _returnvalue_2) :!class /Script/Engine.AudioComponent))

(event EventBeginPlay
  (bind _asplayer_character (Utilities|Casting|CastToPlayerCharacter (Game|GetPlayerCharacter 0)))
  (Variables|Default|SetPlayerRef _asplayer_character))

(fn ConstructionScript)