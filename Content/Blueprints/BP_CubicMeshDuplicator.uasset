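; Editor-placed actor that duplicates a chosen mesh into a 3D grid using a Hierarchical Instanced Static Mesh.
; The Construction Script applies mesh and material, then adds instances spaced along world axes, each inheriting the actor's rotation and scale.
; An optional reference actor donates its transform and is then destroyed.
; A Visualize flag controls visibility during construction, while BeginPlay always shows the instances.
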(event EventBeginPlay
  (Rendering|SetVisibility (Variables|Default|GetHierarchicalInstancedStaticMesh) true false))

(fn ConstructionScript
  (bind _duplicatesperdirection (Variables|Default|GetDuplicatesPerDirection))
  (Rendering|Material|SetMaterial (Variables|Default|GetHierarchicalInstancedStaticMesh) 0 "/Game/ModelsMaterialsTextures/Materials/RepressedWorld/Mat_DuplicatedObject.Mat_DuplicatedObject")
  (Utilities|IsValid (Utilities|ResolveSoftReference (Variables|Default|GetCopy%20transform%20of%20:%20))
    (:Is%20Valid
      (Transformation|SetActorTransform (Transformation|GetActorTransform (Utilities|ResolveSoftReference (Variables|Default|GetCopy%20transform%20of%20:%20))))
      (Actor|DestroyActor (Utilities|ResolveSoftReference (Variables|Default|GetCopy%20transform%20of%20:%20)))
      (Variables|Default|SetCopy%20transform%20of%20:%20 0))
    (:Is%20Not%20Valid
      _))
  (Components|StaticMesh|SetStaticMesh (Variables|Default|GetHierarchicalInstancedStaticMesh) (Variables|Default|GetMesh))
  (Rendering|SetVisibility (Variables|Default|GetHierarchicalInstancedStaticMesh) (Variables|Default|GetVisualize) false)
  (if (Variables|Default|GetUpdate)
    (Variables|Default|SetUpdate false))
  (for _index (range 0 (Math|Float|Truncate (- (.x _duplicatesperdirection) 1.0)))
    (for _index_2 (range 0 (Math|Float|Truncate (- (.y _duplicatesperdirection) 1.0)))
      (for _index_3 (range 0 (Math|Float|Truncate (- (.z _duplicatesperdirection) 1.0)))
        (Class|InstancedStaticMeshComponent|AddInstanceWorldSpace (Variables|Default|GetHierarchicalInstancedStaticMesh) (Math|Transform|MakeTransform (+ (Transformation|GetActorLocation) (* (Variables|Default|GetDistancePerInstance) (Math|Vector|MakeVector (Math|Conversions|ToFloat(Integer) _index) (Math|Conversions|ToFloat(Integer) _index_2) (Math|Conversions|ToFloat(Integer) _index_3)))) (Transformation|GetActorRotation) (Transformation|GetActorScale3D)))))))

(fn Tgrfjhtrfjtr)