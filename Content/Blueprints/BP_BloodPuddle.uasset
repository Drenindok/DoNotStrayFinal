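; Blood puddle actor that spawns a blood decal at its transform, sized by the actor's scale, with a randomly chosen frame.
; A timeline drives the dynamic material's color, darkening the red and animating alpha as the blood dries, then destroys the actor.
; The decal has its own ten-minute fade, and the collision plane is removed earlier, after a fixed delay.
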(event EventBeginPlay
  (bind _returnvalue (Rendering|Material|CreateDynamicMaterialInstance "/Game/ModelsMaterialsTextures/Materials/Blood/Mat_Decal_Blood.Mat_Decal_Blood" "None" "None" :!class /Script/Engine.KismetMaterialLibrary))
  (Variables|Default|SetBlood%20Mat _returnvalue)
  (Variables|Default|SetBloodDecalFrame (Math|Random|RandomInteger 5))
  (Rendering|Material|SetScalarParameterValue (Variables|Default|GetBlood%20Mat) "Frame" (Math|Conversions|ToFloat(Integer) (Variables|Default|GetBloodDecalFrame)) :!class /Script/Engine.MaterialInstanceDynamic)
  (bind _returnvalue_2 (Rendering|Decal|SpawnDecalatLocation (Variables|Default|GetBlood%20Mat) (Transformation|GetActorScale3D) (Transformation|GetActorLocation) (Transformation|GetActorRotation) 6e+02))
  (Rendering|Components|Decal|SetFadeOut _returnvalue_2 0.0 6e+02 true)
  (Utilities|FlowControl|Sequence
    (:then_0
      (bind (_direction _blood_color _blood_alpha) (Timeline|Blood%20drying/fading PlayFromStart)
        (:Update
          (bind _output_get (Variables|Default|SetBlood%20Color (Utilities|Struct|MakeLinearColor (.r (Math|Color|Lerp(LinearColor) "(R=0.050000,G=0.000000,B=0.000000,A=1.000000)" "(R=0.012500,G=0.000000,B=0.000000,A=1.000000)" _blood_color)) (.g (Math|Color|Lerp(LinearColor) "(R=0.050000,G=0.000000,B=0.000000,A=1.000000)" "(R=0.012500,G=0.000000,B=0.000000,A=1.000000)" _blood_color)) (.b (Math|Color|Lerp(LinearColor) "(R=0.050000,G=0.000000,B=0.000000,A=1.000000)" "(R=0.012500,G=0.000000,B=0.000000,A=1.000000)" _blood_color)) _blood_alpha)))
          (Rendering|Material|SetVectorParameterValue (Variables|Default|GetBlood%20Mat) "Color" _output_get :!class /Script/Engine.MaterialInstanceDynamic))
        (:Finished
          (Actor|DestroyActor))))
    (:then_1
      (Utilities|FlowControl|Delay 4.5e+02)
      (Components|DestroyComponent (Variables|Default|GetCollisionPlane)))))

(fn ConstructionScript)