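; BP_TrailPost is a numbered trail signpost and checkpoint that doubles as an invisible thoughts-only trigger when flagged.
; Its thoughts sphere saves respawns, sets screen static and fires one-shot thoughts, cutscenes, checkpoint unlocks, lighting changes and player effects.
; A separate cube trigger, also reached from the sphere and checkpoint loading, pushes the post's Difficulty to the monster.
; The construction script toggles the mesh and tags by mode.
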(event OnComponentBeginOverlap(ThoughtsTrigger)
  (params (OverlappedComponent :type Primitive%20Component%20Object%20Reference) (OtherActor :type Actor%20Object%20Reference) (OtherComp :type Primitive%20Component%20Object%20Reference) (OtherBodyIndex :type Integer) (bFromSweep :type Boolean) (SweepResult :type Hit%20Result%20Structure%20%28by%20ref%29))
  (bind _player_ref (Variables|Default|GetPlayer%20Ref))
  (bind _player_ref_2 (Variables|Default|GetPlayer%20Ref))
  (bind _player_ref_3 (Variables|Default|GetPlayer%20Ref))
  (bind _monsterref (Variables|/Game/Blueprints/ThirdPersonBP/Blueprints/PlayerCharacter.PlayerCharacter_C|GetMonsterRef _player_ref_3))
  ;[0 0.1521 1] Sphere trigger
  (if (not (Variables|Events|GetDisableForSunnyEnding))
    (if (Variables|Default|GetNotAPost%28JustThoughts%29)
      _
      (else
        ;[1 1 1] Update current sign post and set screen static
        (Variables|/Game/Blueprints/ThirdPersonBP/Blueprints/PlayerCharacter.PlayerCharacter_C|SetNearSignpost _player_ref true)
        (Variables|/Game/Blueprints/ThirdPersonBP/Blueprints/PlayerCharacter.PlayerCharacter_C|SetSignpost# _player_ref (Variables|Default|GetPost#))))
    (|SetScreenStatic)
    (Utilities|FlowControl|Sequence
      (:then_0
        (if (not (Variables|Default|GetNotAPost%28JustThoughts%29)) ; don't update respawn point if this isn't a checkpoint
          (Default|SaveRespawnPoint (Variables|Default|GetPlayer%20Ref))))
      (:then_1
        (Utilities|FlowControl|DoOnce false
          (:Completed
            (CallFunction|DisplayThoughts))))
      (:then_2
        ;[0.8434 1 0] Start cutscenes
        (Utilities|FlowControl|DoOnce false
          (:Completed
            (if (Variables|Events|GetPlaysStopAndListenCutscene)
              (|StopAndListenCutscene)
              (elif (Variables|Events|GetEndsGame)
                (bind _outactors (Actor|GetAllActorsOfClass "/Game/Blueprints/CutscenesCinematics/BP_Static_Cutscene.BP_Static_Cutscene_C"))
                (Default|EndGame (Utilities|Array|Get(acopy) _outactors) false false false false)
                (elif (Variables|Events|GetStartsEndingChase)
                  (|EndingChaseSequence)
                  (elif (Variables|Events|GetUnlocksParadoxCheckpoint)
                    (CallFunction|UnlockCheckpoint "TimeParadox")
                    (elif (Variables|Events|GetUnlocksBridgeMazeExit)
                      (bind _returnvalue (Actor|GetActorOfClass "/Game/Blueprints/BP_LoopingSubLevelLoader.BP_LoopingSubLevelLoader_C"))
                      (Variables|/Game/Blueprints/BP_LoopingSubLevelLoader.BP_LoopingSubLevelLoader_C|SetPlayer%20Allowed%20To%20Leave _returnvalue true)
                      (Variables|/Game/Blueprints/BP_LoopingSubLevelLoader.BP_LoopingSubLevelLoader_C|SetPlayerInLoop _returnvalue true)))))))))
      (:then_3
        (Utilities|FlowControl|DoOnce false
          (:Completed
            ;[1 0.7826 0] Update time of day
            (switch Utilities|FlowControl|Switch|SwitchonEnum_SetTimeOfDay (Variables|Events|GetSetTimeOfDay)
              (:NewEnumerator5
                (bind _outactors_2 (Actor|GetAllActorsOfClass "/Game/Blueprints/BP_LightingManager.BP_LightingManager_C"))
                (Utilities|IsValid (Utilities|Array|Get(acopy) _outactors_2)
                  (:Is%20Valid
                    (Default|SwitchtoSunny (Utilities|Array|Get(acopy) _outactors_2)))))
              (:NewEnumerator6
                (bind _outactors_3 (Actor|GetAllActorsOfClass "/Game/Blueprints/BP_LightingManager.BP_LightingManager_C"))
                (Utilities|IsValid (Utilities|Array|Get(acopy) _outactors_3)
                  (:Is%20Valid
                    (Default|SwitchtoNight (Utilities|Array|Get(acopy) _outactors_3)))))
              (:NewEnumerator7
                (bind _outactors_4 (Actor|GetAllActorsOfClass "/Game/Blueprints/BP_LightingManager.BP_LightingManager_C"))
                (Utilities|IsValid (Utilities|Array|Get(acopy) _outactors_4)
                  (:Is%20Valid
                    (Default|SwitchtoRepressed (Utilities|Array|Get(acopy) _outactors_4)))))))))
      (:then_4
        ;[0 0 0] Play distortion sound at start of thoughts (used for ending walk distortion)
        (Utilities|FlowControl|DoOnce false
          (:Completed
            (if (Utilities|Enum|Equal(Enum) (Variables|PlaySound|GetPlaySoundAtEnd) "NewEnumerator8")
              (bind _returnvalue_2 (Audio|CreateSound2D (Variables|PlaySound|GetSound) 1.0 1.0 0.0 0))
              (Audio|Components|Audio|FadeIn _returnvalue_2 1.0 1.0 0.0 "Linear" :!class /Script/Engine.AudioComponent)))))
      (:then_5
        ;[1 0 0.7374] SetPlayerEffects (for cutscenes)
        (Utilities|FlowControl|DoOnce false
          (:Completed
            (if (Variables|Events|GetDisableSprinting)
              (Variables|/Game/Blueprints/ThirdPersonBP/Blueprints/PlayerCharacter.PlayerCharacter_C|SetSprintingDisabled _player_ref_2 true)
              (else
                (Variables|/Game/Blueprints/ThirdPersonBP/Blueprints/PlayerCharacter.PlayerCharacter_C|SetSprintingDisabled _player_ref_2 false)))
            (Variables|/Game/Blueprints/ThirdPersonBP/Blueprints/PlayerCharacter.PlayerCharacter_C|SetDizzinessOverride _player_ref_2 (Variables|Default|GetOverrideDizziness))
            ;[0 0 0] Ending walk
            (if (Variables|Events|GetActivateEndingWalk)
              (bind _outactors_5 (Actor|GetAllActorsOfClass "/Game/Blueprints/CutscenesCinematics/BP_ProxyCarStatic.BP_ProxyCarStatic_C"))
              (Variables|/Game/Blueprints/CutscenesCinematics/BP_ProxyCarStatic.BP_ProxyCarStatic_C|SetActivated (Utilities|Array|Get(acopy) _outactors_5) true)
              (Utilities|FlowControl|DoOnce false
                (:Completed
                  (bind _outactors_6 (Actor|GetAllActorsOfClasswithTag "/Script/Engine.TargetPoint" "MonsterFollowSpawn"))
                  (Game|SpawnActorfromClass "/Game/Blueprints/Monster/Monster_FollowPlayer.Monster_FollowPlayer_C" (Math|Transform|MakeTransform (Transformation|GetActorLocation (Utilities|Array|Get(acopy) _outactors_6)) "0, 0, 0" "1,1,1") "Undefined" 0 0)))))))
      (:then_6
        ;[1 1 1] Update difficulty (Unscaled)
        (if (and (Variables|Default|GetUpdatesDifficulty) (not (Variables|/Game/Blueprints/Monster/MonsterCharacter.MonsterCharacter_C|GetPlayer%20went%20out%20of%20bounds (Variables|/Game/Blueprints/ThirdPersonBP/Blueprints/PlayerCharacter.PlayerCharacter_C|GetMonsterRef (Variables|Default|GetPlayer%20Ref)))))
          (bind _outactors_7 (Actor|GetAllActorsOfClass "/Game/Blueprints/Monster/MonsterCharacter.MonsterCharacter_C"))
          (Variables|/Game/Blueprints/Monster/MonsterCharacter.MonsterCharacter_C|SetDifficulty (Utilities|Array|Get(acopy) _outactors_7) (Variables|Default|GetDifficulty))
          (if (> (Variables|/Game/Blueprints/Monster/MonsterCharacter.MonsterCharacter_C|GetTime%20Until%20Next%20Spawn _monsterref) (* (+ (.DespawnedTimeMin (Utilities|Struct|BreakVar_GlitchingMovingIn (.GlitchesMovingIn (Utilities|Struct|Breakvar_Difficulty (Variables|Default|GetDifficulty))))) (.DespawnedTimeMax (Utilities|Struct|BreakVar_GlitchingMovingIn (.GlitchesMovingIn (Utilities|Struct|Breakvar_Difficulty (Variables|Default|GetDifficulty)))))) 0.5))
            (Default|UpdateTimeUntilNextSpawn _monsterref)))))))

(event OnComponentEndOverlap(ThoughtsTrigger)
  (params (OverlappedComponent :type Primitive%20Component%20Object%20Reference) (OtherActor :type Actor%20Object%20Reference) (OtherComp :type Primitive%20Component%20Object%20Reference) (OtherBodyIndex :type Integer)))

(event OnComponentBeginOverlap(DifficultyUpdateTrigger)
  (params (OverlappedComponent :type Primitive%20Component%20Object%20Reference) (OtherActor :type Actor%20Object%20Reference) (OtherComp :type Primitive%20Component%20Object%20Reference) (OtherBodyIndex :type Integer) (bFromSweep :type Boolean) (SweepResult :type Hit%20Result%20Structure%20%28by%20ref%29))
  (bind _player_ref (Variables|Default|GetPlayer%20Ref))
  (bind _monsterref (Variables|/Game/Blueprints/ThirdPersonBP/Blueprints/PlayerCharacter.PlayerCharacter_C|GetMonsterRef _player_ref))
  ;[0 1 0.008271] Cube trigger (all this does is update difficulty, nothing else)
  ;[1 1 1] Update difficulty (Unscaled)
  (if (and (Variables|Default|GetUpdatesDifficulty) (not (Variables|/Game/Blueprints/Monster/MonsterCharacter.MonsterCharacter_C|GetPlayer%20went%20out%20of%20bounds (Variables|/Game/Blueprints/ThirdPersonBP/Blueprints/PlayerCharacter.PlayerCharacter_C|GetMonsterRef (Variables|Default|GetPlayer%20Ref)))))
    (bind _outactors (Actor|GetAllActorsOfClass "/Game/Blueprints/Monster/MonsterCharacter.MonsterCharacter_C"))
    (Variables|/Game/Blueprints/Monster/MonsterCharacter.MonsterCharacter_C|SetDifficulty (Utilities|Array|Get(acopy) _outactors) (Variables|Default|GetDifficulty))
    (if (> (Variables|/Game/Blueprints/Monster/MonsterCharacter.MonsterCharacter_C|GetTime%20Until%20Next%20Spawn _monsterref) (* (+ (.DespawnedTimeMin (Utilities|Struct|BreakVar_GlitchingMovingIn (.GlitchesMovingIn (Utilities|Struct|Breakvar_Difficulty (Variables|Default|GetDifficulty))))) (.DespawnedTimeMax (Utilities|Struct|BreakVar_GlitchingMovingIn (.GlitchesMovingIn (Utilities|Struct|Breakvar_Difficulty (Variables|Default|GetDifficulty)))))) 0.5))
      (Default|UpdateTimeUntilNextSpawn _monsterref))))

(event OnComponentEndOverlap(DifficultyUpdateTrigger)
  (params (OverlappedComponent :type Primitive%20Component%20Object%20Reference) (OtherActor :type Actor%20Object%20Reference) (OtherComp :type Primitive%20Component%20Object%20Reference) (OtherBodyIndex :type Integer))
  (if (not (Variables|Events|GetDisableForSunnyEnding))
    ;[1 1 1] "Pass all sign posts" tutorial
    (Variables|/Game/Blueprints/ThirdPersonBP/Blueprints/PlayerCharacter.PlayerCharacter_C|SetNearSignpost (Variables|Default|GetPlayer%20Ref) false)
    (if (Variables|Events|GetShowPassingSignpostsTutorial) ; If this is the first sign post, \nshow the hint explaining sign\nposts.
      (Utilities|FlowControl|DoOnce false
        (:Completed
          (Utilities|FlowControl|Delay 3.0)
          (Default|QueTutorialMessage (Variables|/Game/Blueprints/ThirdPersonBP/Blueprints/PlayerCharacter.PlayerCharacter_C|GetHUDref (Variables|Default|GetPlayer%20Ref)) (Utilities|Struct|MakeVar_TutorialPopup "Pass all trail posts then return to your car to finish the trail." 1e+01))
          (Utilities|FlowControl|Delay 2e+01)
          (Default|QueTutorialMessage (Variables|/Game/Blueprints/ThirdPersonBP/Blueprints/PlayerCharacter.PlayerCharacter_C|GetHUDref (Variables|Default|GetPlayer%20Ref)) (Utilities|Struct|MakeVar_TutorialPopup "Right click to turn your light on and off. " 6.0)))))))

(event Custom|LoadPostDataForCheckpoint
  (bind _player_ref (Variables|Default|GetPlayer%20Ref))
  (bind _monsterref (Variables|/Game/Blueprints/ThirdPersonBP/Blueprints/PlayerCharacter.PlayerCharacter_C|GetMonsterRef _player_ref))
  (CallFunction|DisplayThoughts)
  (Default|SaveRespawnPoint (Variables|Default|GetPlayer%20Ref))
  ;[1 1 1] Update difficulty (Unscaled)
  (if (and (Variables|Default|GetUpdatesDifficulty) (not (Variables|/Game/Blueprints/Monster/MonsterCharacter.MonsterCharacter_C|GetPlayer%20went%20out%20of%20bounds (Variables|/Game/Blueprints/ThirdPersonBP/Blueprints/PlayerCharacter.PlayerCharacter_C|GetMonsterRef (Variables|Default|GetPlayer%20Ref)))))
    (bind _outactors (Actor|GetAllActorsOfClass "/Game/Blueprints/Monster/MonsterCharacter.MonsterCharacter_C"))
    (Variables|/Game/Blueprints/Monster/MonsterCharacter.MonsterCharacter_C|SetDifficulty (Utilities|Array|Get(acopy) _outactors) (Variables|Default|GetDifficulty))
    (if (> (Variables|/Game/Blueprints/Monster/MonsterCharacter.MonsterCharacter_C|GetTime%20Until%20Next%20Spawn _monsterref) (* (+ (.DespawnedTimeMin (Utilities|Struct|BreakVar_GlitchingMovingIn (.GlitchesMovingIn (Utilities|Struct|Breakvar_Difficulty (Variables|Default|GetDifficulty))))) (.DespawnedTimeMax (Utilities|Struct|BreakVar_GlitchingMovingIn (.GlitchesMovingIn (Utilities|Struct|Breakvar_Difficulty (Variables|Default|GetDifficulty)))))) 0.5))
      (Default|UpdateTimeUntilNextSpawn _monsterref))))

(event EventBeginPlay
  (bind _asplayer_character (Utilities|Casting|CastToPlayerCharacter (Game|GetPlayerCharacter 0))
    (:then
      (Variables|Default|SetPlayer%20Ref _asplayer_character))
    (:CastFailed
      (Variables|Events|SetDisableForSunnyEnding true))))

(fn ConstructionScript
  (bind _staticmesh (Variables|Default|GetStaticMesh))
  (bind _staticmesh_2 (Variables|Default|GetStaticMesh))
  (if (Variables|Default|GetNotAPost%28JustThoughts%29)
    (Collision|SetCollisionEnabled _staticmesh_2 "NoCollision")
    (Rendering|SetVisibility _staticmesh_2 false true)
    (Variables|Default|SetTags (Utilities|Array|MakeArray))
    (else
      (Collision|SetCollisionEnabled _staticmesh "QueryAndPhysics")
      (Rendering|SetVisibility _staticmesh true true)
      (if (Variables|PlaySound|GetRunSoundMult)
        (Variables|PlaySound|SetRunSoundMult false)
        (Variables|Default|SetDifficulty (Utilities|Struct|Makevar_Difficulty (.glitchesmovingin (Variables|Default|GetDifficulty)) (.wanderingfar (Variables|Default|GetDifficulty)) (.wanderingclose (Variables|Default|GetDifficulty)) (* (.randomsoundchance (Variables|Default|GetDifficulty)) (Variables|PlaySound|GetSoundMult)) (.randomsounds (Variables|Default|GetDifficulty)) (.despawngraceperiod (Variables|Default|GetDifficulty)) (.toofardespawn (Variables|Default|GetDifficulty)) (.tooclosedespawn (Variables|Default|GetDifficulty)) (.riseuptime (Variables|Default|GetDifficulty)) (.chasewhenclose (Variables|Default|GetDifficulty)) (.chasewhenneardistance (Variables|Default|GetDifficulty)) (.proximitystaticdistance (Variables|Default|GetDifficulty)) (.footsteps (Variables|Default|GetDifficulty)) (.singingbreathing (Variables|Default|GetDifficulty)) (.fogvisibleinfarwander (Variables|Default|GetDifficulty)) false))
        (Variables|PlaySound|SetSoundMult 1.0))
      (Rendering|Components|TextRender|SetText (Variables|Default|GetTextRender) (Utilities|Text|ToText(Integer) (Variables|Default|GetPost#)))
      (Variables|Default|SetTags (Utilities|Array|MakeArray (Utilities|String|StringToName (Utilities|String|Append "post " (Utilities|String|ToString(Integer) (Variables|Default|GetPost#)))) "TrailPost")))))

(fn FadeOutAllThoughts
  (for _array_element (Variables|Default|GetDisplayedTexts)
    (Variables|/Game/UI/UI_ThoughtText.UI_ThoughtText_C|SetFadeIn _array_element false))
  ;[1 1 1] Play distortion sound after thoughts fade away (used for ending walk distortion)
  (if (Utilities|Enum|Equal(Enum) (Variables|PlaySound|GetPlaySoundAtEnd) "NewEnumerator9")
    (bind _returnvalue (Audio|CreateSound2D (Variables|PlaySound|GetSound) 1.0 1.0 0.0 0))
    (Audio|Components|Audio|FadeIn _returnvalue 1.0 1.0 0.0 "Linear" :!class /Script/Engine.AudioComponent)))

(fn UnlockCheckpoint
  (params (CheckpointName :type String))
  (bind _returnvalue (SaveGame|LoadGamefromSlot "PlayerData"))
  (bind _asplayer_save_data (Utilities|Casting|CastToPlayerSaveData _returnvalue))
  (Utilities|Array|AddUnique (Variables|/Game/PlayerSaveData.PlayerSaveData_C|GetCheckpoints _asplayer_save_data) CheckpointName)
  (SaveGame|SaveGametoSlot _asplayer_save_data "PlayerData"))

(fn DisplayThoughts
  (bind _charglitchchance (Variables|Thoughts|GetCharGlitchChance))
  (bind _player_ref (Variables|Default|GetPlayer%20Ref))
  (bind _savedata (Variables|/Game/Blueprints/ThirdPersonBP/Blueprints/PlayerCharacter.PlayerCharacter_C|GetSaveData _player_ref))
  (bind _asmain_game_instance (Utilities|Casting|CastToMainGameInstance (Game|GetGameInstance)))
  (Default|ShowThoughts _asmain_game_instance (Variables|Thoughts|GetThoughts) (Variables|Thoughts|GetFont) (Variables|Thoughts|GetFont%20Color) false 25.0 (Math|Float|SelectFloat (Utilities|Select :Index (Variables|/Game/PlayerSaveData.PlayerSaveData_C|GetRun#ToLoad _savedata) :Option%200 0.0 :Option%201 0.0 :Option%202 (Utilities|Select :Index (Math|Integer|Clamp(Integer) (Variables|/Game/PlayerSaveData.PlayerSaveData_C|Get2ndRunDeaths _savedata) 0 5) :Option%200 0.0075 :Option%201 0.015 :Option%202 0.0225 :Option%203 0.03 :Option%204 0.04 :Option%205 0.05)) _charglitchchance (< _charglitchchance 0.0)) (Variables|Thoughts|GetCharShakeAmount) false false))