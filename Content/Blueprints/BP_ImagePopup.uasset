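; BP_ImagePopup is an actor that shows a tinted image popup on BeginPlay, disabling player input until a key press dismisses it and the actor destroys itself.
; With a nonzero FadeTime, it fades the camera out, then optionally fades the image in, reversing this on dismissal.
; One timeline, rate-scaled to that duration, drives image opacity, HUD opacity and the global outline material parameter's alpha.
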(event Custom|FadeScreenOut
  (params (Duration :type Float%20%28single-precision%29) (FadeScreenToo :type Boolean))
  ;[1 1 1] Fade screen In/Out
  (Variables|Default|SetFadeScreenToo FadeScreenToo)
  (Components|Timeline|SetPlayRate (Variables|Default|GetScreen%20Fade%20Timeline) (/ 1.0 Duration))
  (if FadeScreenToo
    (CameraFades|StartCameraFade :self (Game|GetPlayerCameraManager 0) :ToAlpha 1.0 :Duration Duration :bHoldWhenFinished true)
    (bind _fade (Timeline|Screen%20Fade%20Timeline PlayFromStart)
      (:Update
        (bind _returnvalue (Rendering|Material|GetVectorParameterValue "/Game/ModelsMaterialsTextures/GlobalMaterialParams.GlobalMaterialParams" "RepressedOutlineColor" :!class /Script/Engine.KismetMaterialLibrary))
        (Rendering|Material|SetVectorParameterValue "/Game/ModelsMaterialsTextures/GlobalMaterialParams.GlobalMaterialParams" "RepressedOutlineColor" (Utilities|Struct|MakeLinearColor (.r _returnvalue) (.g _returnvalue) (.b _returnvalue) (Math|Float|SelectFloat _fade 0.0 (Variables|Default|GetFadeScreenToo))) :!class /Script/Engine.KismetMaterialLibrary)
        (Widget|SetRenderOpacity (Variables|/Game/Blueprints/ThirdPersonBP/Blueprints/PlayerCharacter.PlayerCharacter_C|GetHUDref (Variables|Default|GetPlayerRef)) (Math|Float|SelectFloat _fade 0.0 (Variables|Default|GetFadeScreenToo)))
        (if (Variables|Default|GetImageVisible)
          (Widget|SetRenderOpacity (Variables|Default|GetWidget) _fade))))
    (else
      (Timeline|Screen%20Fade%20Timeline PlayFromStart))))

(event Custom|FadeScreenIn
  (params (Duration :type Float%20%28single-precision%29) (FadeScreenToo :type Boolean))
  ;[1 1 1] Fade screen In/Out
  (Variables|Default|SetFadeScreenToo FadeScreenToo)
  (Components|Timeline|SetPlayRate (Variables|Default|GetScreen%20Fade%20Timeline) (/ 1.0 Duration))
  (if FadeScreenToo
    (CameraFades|StartCameraFade :self (Game|GetPlayerCameraManager 0) :FromAlpha 1.0 :Duration Duration :bHoldWhenFinished true)
    (bind _fade (Timeline|Screen%20Fade%20Timeline ReverseFromEnd)
      (:Update
        (bind _returnvalue (Rendering|Material|GetVectorParameterValue "/Game/ModelsMaterialsTextures/GlobalMaterialParams.GlobalMaterialParams" "RepressedOutlineColor" :!class /Script/Engine.KismetMaterialLibrary))
        (Rendering|Material|SetVectorParameterValue "/Game/ModelsMaterialsTextures/GlobalMaterialParams.GlobalMaterialParams" "RepressedOutlineColor" (Utilities|Struct|MakeLinearColor (.r _returnvalue) (.g _returnvalue) (.b _returnvalue) (Math|Float|SelectFloat _fade 0.0 (Variables|Default|GetFadeScreenToo))) :!class /Script/Engine.KismetMaterialLibrary)
        (Widget|SetRenderOpacity (Variables|/Game/Blueprints/ThirdPersonBP/Blueprints/PlayerCharacter.PlayerCharacter_C|GetHUDref (Variables|Default|GetPlayerRef)) (Math|Float|SelectFloat _fade 0.0 (Variables|Default|GetFadeScreenToo)))
        (if (Variables|Default|GetImageVisible)
          (Widget|SetRenderOpacity (Variables|Default|GetWidget) _fade))))
    (else
      (Timeline|Screen%20Fade%20Timeline ReverseFromEnd))))

(event EventBeginPlay
  (bind _fade_time (Variables|Default|GetFade%20Time))
  (bind _asplayer_character (Utilities|Casting|CastToPlayerCharacter (Game|GetPlayerCharacter 0)))
  (Variables|Default|SetPlayerRef _asplayer_character)
  (bind _returnvalue (UserInterface|CreateWidget "/Game/UI/UI_ImagePopup.UI_ImagePopup_C" 0 (Variables|Default|GetImage) (Variables|Default|GetFade%20Time)))
  (bind _output_get (Variables|Default|SetWidget _returnvalue))
  (UserInterface|Viewport|AddtoViewport _output_get 0)
  (Appearance|SetColorandOpacity (Variables|/Game/UI/UI_ImagePopup.UI_ImagePopup_C|GetReflectionImage (Variables|Default|GetWidget)) (Variables|Default|GetImageColor) :!class /Script/UMG.Image)
  (Input|DisableInput (Variables|Default|GetPlayerRef) (Game|GetPlayerController 0))
  (if (== _fade_time 0.0)
    (Widget|SetRenderOpacity (Variables|Default|GetWidget) 1.0)
    (else
      (CallFunction|FadeScreenOut _fade_time true)
      (Utilities|FlowControl|Delay _fade_time)
      (if (Variables|Default|GetActuallyShowImage)
        (CallFunction|FadeScreenin (Variables|Default|GetFade%20Time) false))
      (Variables|Default|SetImageVisible true)))
  (Input|EnableInput (Game|GetPlayerController 0)))

(event Input|KeyboardEvents|AnyKey
  (params (Key :type Key%20Structure :default "None"))
  (bind _returnvalue (Game|GetPlayerController 0))
  (bind _fade_time (Variables|Default|GetFade%20Time))
  (:Pressed
    (Utilities|FlowControl|DoOnce false
      (:Completed
        (if (== (Variables|Default|GetFade%20Time) 0.0)
          (Widget|RemovefromParent (Variables|Default|GetWidget))
          (else
            (if (Variables|Default|GetActuallyShowImage)
              (CallFunction|FadeScreenOut _fade_time false)
              (Utilities|FlowControl|Delay _fade_time))
            (Variables|Default|SetImageVisible false)
            (CallFunction|FadeScreenin (Variables|Default|GetFade%20Time) true)
            (Widget|RemovefromParent (Variables|Default|GetWidget))))
        (Input|EnableInput (Variables|Default|GetPlayerRef) _returnvalue)
        (Input|DisableInput _returnvalue)
        (Utilities|FlowControl|Delay (Variables|Default|GetFade%20Time))
        (Actor|DestroyActor)))))

(fn ConstructionScript)