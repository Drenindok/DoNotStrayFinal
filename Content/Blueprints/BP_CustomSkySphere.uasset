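; Sky sphere Blueprint that drives a dynamic sky material with sun, sky colors, clouds and stars.
; The construction script creates the material instance and runs RefreshMaterial, taking sun direction and color from an assigned directional light, or deriving them from SunHeight.
; Colors come from sun-height curves or manual properties, and negative sun height blends in stars.
; UpdateSunDirection re-applies light-driven parameters using a simpler pitch-to-height mapping.
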(fn ConstructionScript
  (bind _returnvalue (Rendering|Material|CreateDynamicMaterialInstance (Variables|BP_Skydome|GetSkySphereMesh) 0 (Variables|Default|GetSkyMat) "None" :!class /Script/Engine.PrimitiveComponent))
  (Variables|Default|SetSky%20material%20Ref _returnvalue)
  (if (Variables|Default|GetRefresh%20material) ; Updating bool in details panel causes construction script to run again
    _
    (else
      _))
  (Variables|Default|SetRefresh%20material false)
  (CallFunction|RefreshMaterial))

(fn UpdateSunDirection
  (bind _sky_material_ref (Variables|Default|GetSky%20material%20Ref))
  (bind _sky_material_ref_2 (Variables|Default|GetSky%20material%20Ref))
  (Rendering|Material|SetVectorParameterValue _sky_material_ref "Light direction" (Math|Conversions|ToLinearColor(Vector) (Math|Rotator|GetRotationXVector (Transformation|GetActorRotation (Variables|Default|GetDirectional%20light%20actor)))) :!class /Script/Engine.MaterialInstanceDynamic)
  (Rendering|Material|SetVectorParameterValue _sky_material_ref "Sun color" (Math|Conversions|ToLinearColor(Color) (Variables|/Script/Engine.LightComponentBase|GetLightColor (Variables|/Script/Engine.Light|GetLightComponent (Variables|Default|GetDirectional%20light%20actor)))) :!class /Script/Engine.MaterialInstanceDynamic)
  (Variables|Overridesettings|SetSun%20height (Math|Float|MapRangeUnclamped (.Pitch (Math|Rotator|BreakRotator (Transformation|GetActorRotation (Variables|Default|GetDirectional%20light%20actor)))) 0.0 -9e+01 0.0 1.0))
  (Rendering|Material|SetVectorParameterValue _sky_material_ref_2 "Horizon color" (Class|CurveLinearColor|GetClampedLinearColorValue (Variables|Default|GetHorizon%20color%20curve) (Variables|Overridesettings|GetSun%20height)) :!class /Script/Engine.MaterialInstanceDynamic)
  (Rendering|Material|SetVectorParameterValue _sky_material_ref_2 "Zenith color" (Class|CurveLinearColor|GetClampedLinearColorValue (Variables|Default|GetZenith%20color%20curve) (Variables|Overridesettings|GetSun%20height)) :!class /Script/Engine.MaterialInstanceDynamic)
  (Rendering|Material|SetVectorParameterValue _sky_material_ref_2 "Cloud color" (Class|CurveLinearColor|GetClampedLinearColorValue (Variables|Default|GetCloud%20color%20curve) (Variables|Overridesettings|GetSun%20height)) :!class /Script/Engine.MaterialInstanceDynamic)
  (Rendering|Material|SetScalarParameterValue _sky_material_ref_2 "Horizon falloff" (Math|Float|Lerp 3.0 8.0 (Math|Float|Absolute(Float) (Variables|Overridesettings|GetSun%20height))) :!class /Script/Engine.MaterialInstanceDynamic)
  (Rendering|Material|SetScalarParameterValue _sky_material_ref_2 "Sun height" (Math|Float|SelectFloat (Math|Float|Absolute(Float) (Variables|Overridesettings|GetSun%20height)) 0.0 (< (Variables|Overridesettings|GetSun%20height) 0.0)) :!class /Script/Engine.MaterialInstanceDynamic))

(fn RefreshMaterial
  (bind _sky_material_ref (Variables|Default|GetSky%20material%20Ref))
  (bind _directional_light_actor (Variables|Default|GetDirectional%20light%20actor))
  (bind _sky_material_ref_2 (Variables|Default|GetSky%20material%20Ref))
  (bind _sky_material_ref_3 (Variables|Default|GetSky%20material%20Ref))
  (bind _sky_material_ref_4 (Variables|Default|GetSky%20material%20Ref))
  (bind _sky_material_ref_5 (Variables|Default|GetSky%20material%20Ref))
  (bind _returnvalue (Transformation|GetActorRotation _directional_light_actor))
  (bind _pitch (Math|Rotator|BreakRotator _returnvalue))
  (Utilities|IsValid (Variables|Default|GetDirectional%20light%20actor) ; Has a directional light been assigned?
    (:Is%20Valid
      (Rendering|Material|SetVectorParameterValue _sky_material_ref_3 "Light direction" (Math|Conversions|ToLinearColor(Vector) (Math|Rotator|GetRotationXVector (Transformation|GetActorRotation (Variables|Default|GetDirectional%20light%20actor)))) :!class /Script/Engine.MaterialInstanceDynamic)
      (Rendering|Material|SetVectorParameterValue _sky_material_ref_3 "Sun color" (Math|Conversions|ToLinearColor(Color) (Variables|/Script/Engine.LightComponentBase|GetLightColor (Variables|/Script/Engine.Light|GetLightComponent (Variables|Default|GetDirectional%20light%20actor)))) :!class /Script/Engine.MaterialInstanceDynamic)
      (Variables|Overridesettings|SetSun%20height (Math|Float|SelectFloat (Math|Float|MapRangeUnclamped _pitch 18.0 0.0 -1.0 0.0) (Math|Float|MapRangeUnclamped _pitch 0.0 -9e+01 0.0 1.0) (> _pitch 0.0))))
    (:Is%20Not%20Valid
      (Rendering|Material|SetVectorParameterValue _sky_material_ref_2 "Light direction" (Math|Conversions|ToLinearColor(Vector) (Math|Rotator|GetRotationXVector (Math|Rotator|MakeRotator 0.0 (Math|Float|MapRangeUnclamped (Variables|Overridesettings|GetSun%20height) -1.0 1.0 9e+01 -9e+01) (.Yaw (Math|Rotator|BreakRotator (Transformation|GetActorRotation)))))) :!class /Script/Engine.MaterialInstanceDynamic)
      (Rendering|Material|SetVectorParameterValue _sky_material_ref_2 "Sun color" (Math|Color|Lerp(LinearColor) "(R=1.000000,G=0.221000,B=0.040000,A=1.000000)" "(R=0.954000,G=0.901000,B=0.744120,A=1.000000)" (Math|Float|Clamp(Float) (+ (Variables|Overridesettings|GetSun%20height) 0.2))) :!class /Script/Engine.MaterialInstanceDynamic)))
  (if (Variables|Default|GetColors%20determined%20by%20sun%20position)
    (Rendering|Material|SetVectorParameterValue _sky_material_ref_4 "Horizon color" (Class|CurveLinearColor|GetClampedLinearColorValue (Variables|Default|GetHorizon%20color%20curve) (Variables|Overridesettings|GetSun%20height)) :!class /Script/Engine.MaterialInstanceDynamic)
    (Rendering|Material|SetVectorParameterValue _sky_material_ref_4 "Zenith color" (Class|CurveLinearColor|GetClampedLinearColorValue (Variables|Default|GetZenith%20color%20curve) (Variables|Overridesettings|GetSun%20height)) :!class /Script/Engine.MaterialInstanceDynamic)
    (Rendering|Material|SetVectorParameterValue _sky_material_ref_4 "Cloud color" (Class|CurveLinearColor|GetClampedLinearColorValue (Variables|Default|GetCloud%20color%20curve) (Variables|Overridesettings|GetSun%20height)) :!class /Script/Engine.MaterialInstanceDynamic)
    (Rendering|Material|SetScalarParameterValue _sky_material_ref_4 "Horizon falloff" (Math|Float|Lerp 3.0 7.0 (Math|Float|Absolute(Float) (Variables|Overridesettings|GetSun%20height))) :!class /Script/Engine.MaterialInstanceDynamic)
    (else
      (Rendering|Material|SetVectorParameterValue _sky_material_ref "Horizon color" (Variables|Overridesettings|GetHorizon%20color) :!class /Script/Engine.MaterialInstanceDynamic)
      (Rendering|Material|SetVectorParameterValue _sky_material_ref "Zenith color" (Variables|Overridesettings|GetZenith%20Color) :!class /Script/Engine.MaterialInstanceDynamic)
      (Rendering|Material|SetVectorParameterValue _sky_material_ref "Overall color" (Variables|Overridesettings|GetOverall%20Color) :!class /Script/Engine.MaterialInstanceDynamic)
      (Rendering|Material|SetVectorParameterValue _sky_material_ref "Cloud color" (Variables|Overridesettings|GetCloud%20color) :!class /Script/Engine.MaterialInstanceDynamic)
      (Rendering|Material|SetScalarParameterValue _sky_material_ref "Horizon falloff" (Variables|Overridesettings|GetHorizon%20Falloff) :!class /Script/Engine.MaterialInstanceDynamic)))
  (Rendering|Material|SetScalarParameterValue _sky_material_ref_5 "Cloud speed" (Variables|Default|GetCloud%20speed) :!class /Script/Engine.MaterialInstanceDynamic)
  (Rendering|Material|SetScalarParameterValue _sky_material_ref_5 "Sun brightness" (Variables|Default|GetSun%20brightness) :!class /Script/Engine.MaterialInstanceDynamic)
  (Rendering|Material|SetScalarParameterValue _sky_material_ref_5 "Sun height" (Math|Float|SelectFloat (Math|Float|Absolute(Float) (Variables|Overridesettings|GetSun%20height)) 0.0 (< (Variables|Overridesettings|GetSun%20height) 0.0)) :!class /Script/Engine.MaterialInstanceDynamic)
  (Rendering|Material|SetScalarParameterValue _sky_material_ref_5 "Cloud opacity" (Variables|Default|GetCloud%20opacity) :!class /Script/Engine.MaterialInstanceDynamic)
  (Rendering|Material|SetScalarParameterValue _sky_material_ref_5 "Stars brightness" (Variables|Default|GetStars%20brightness) :!class /Script/Engine.MaterialInstanceDynamic))