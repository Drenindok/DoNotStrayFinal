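; Procedural bridge generator that rebuilds instanced mesh pieces along BridgeSpline in the construction script when Update is set.
; Each step alternates long and short pieces, picking a random variant and random flip, centred between two spline samples and aimed along them.
; Accumulated yaw change, scaled by Uwghewiugh, shifts later samples along the spline to compensate for turns.
; Only the short-piece components are explicitly cleared before rebuilding.
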(event EventBeginPlay)

(event Collision|EventActorBeginOverlap
  (params (OtherActor :type Actor%20Object%20Reference)))

(event EventTick
  (params (DeltaSeconds :type Float%20%28single-precision%29)))

(fn ConstructionScript
  (bind _returnvalue (Math|Random|RandomIntegerinRange 0 2))
  (bind _bridgespline (Variables|Default|GetBridgeSpline))
  (if (Variables|Default|GetUpdate)
    (Utilities|Array|Clear (Variables|Default|GetPrevious%20Piece%20Angle%20Array))
    (Variables|Default|SetTurning%20Distance%20Compensation 0.0)
    (Components|InstancedStaticMesh|ClearInstances (Variables|Default|GetShortPiece1))
    (for _index (range 0 (Math|Float|Truncate (- (/ (Spline|GetSplineLength (Variables|Default|GetBridgeSpline)) (Variables|Default|GetDistanceBetweenPieces)) 1.0)))
      (Variables|Default|SetTurning%20Distance%20Compensation (+ (Variables|Default|GetTurning%20Distance%20Compensation) (Math|Float|Absolute(Float) (.Yaw (Math|Rotator|BreakRotator (Math|Rotator|CombineRotators (Math|Rotator|CombineRotators (Math|Rotator|FindLookatRotation (Spline|GetLocationatDistanceAlongSpline _bridgespline (+ (* _index (Variables|Default|GetDistanceBetweenPieces)) (* (Variables|Default|GetTurning%20Distance%20Compensation) (Variables|Default|Getuwghewiugh))) "Local") (Spline|GetLocationatDistanceAlongSpline _bridgespline (+ (+ (* _index (Variables|Default|GetDistanceBetweenPieces)) (* (Variables|Default|GetTurning%20Distance%20Compensation) (Variables|Default|Getuwghewiugh))) (Variables|Default|GetDistanceBetweenPieces)) "Local")) "0,90.000000, 0") (* (Variables|Default|GetPrevious%20Piece%20Angle) -1.0)))))))
      (Utilities|FlowControl|FlipFlop
        (:A
          (switch int _returnvalue
            (:0
              (Components|InstancedStaticMesh|AddInstance (Variables|Default|GetLongPiece1) (Math|Transform|MakeTransform (* (+ (Spline|GetLocationatDistanceAlongSpline _bridgespline (+ (* _index (Variables|Default|GetDistanceBetweenPieces)) (* (Variables|Default|GetTurning%20Distance%20Compensation) (Variables|Default|Getuwghewiugh))) "Local") (Spline|GetLocationatDistanceAlongSpline _bridgespline (+ (+ (* _index (Variables|Default|GetDistanceBetweenPieces)) (* (Variables|Default|GetTurning%20Distance%20Compensation) (Variables|Default|Getuwghewiugh))) (Variables|Default|GetDistanceBetweenPieces)) "Local")) 0.5) (Math|Rotator|CombineRotators (Math|Rotator|CombineRotators (Math|Rotator|FindLookatRotation (Spline|GetLocationatDistanceAlongSpline _bridgespline (+ (* _index (Variables|Default|GetDistanceBetweenPieces)) (* (Variables|Default|GetTurning%20Distance%20Compensation) (Variables|Default|Getuwghewiugh))) "Local") (Spline|GetLocationatDistanceAlongSpline _bridgespline (+ (+ (* _index (Variables|Default|GetDistanceBetweenPieces)) (* (Variables|Default|GetTurning%20Distance%20Compensation) (Variables|Default|Getuwghewiugh))) (Variables|Default|GetDistanceBetweenPieces)) "Local")) "0,90.000000, 0") (Math|Rotator|SelectRotator "0, 0, 0" "0,180.000000, 0" (Math|Random|RandomBool))) "0.666600,0.666600,0.666600")))
            (:1
              (Components|InstancedStaticMesh|AddInstance (Variables|Default|GetLongPiece2) (Math|Transform|MakeTransform (* (+ (Spline|GetLocationatDistanceAlongSpline _bridgespline (+ (* _index (Variables|Default|GetDistanceBetweenPieces)) (* (Variables|Default|GetTurning%20Distance%20Compensation) (Variables|Default|Getuwghewiugh))) "Local") (Spline|GetLocationatDistanceAlongSpline _bridgespline (+ (+ (* _index (Variables|Default|GetDistanceBetweenPieces)) (* (Variables|Default|GetTurning%20Distance%20Compensation) (Variables|Default|Getuwghewiugh))) (Variables|Default|GetDistanceBetweenPieces)) "Local")) 0.5) (Math|Rotator|CombineRotators (Math|Rotator|CombineRotators (Math|Rotator|FindLookatRotation (Spline|GetLocationatDistanceAlongSpline _bridgespline (+ (* _index (Variables|Default|GetDistanceBetweenPieces)) (* (Variables|Default|GetTurning%20Distance%20Compensation) (Variables|Default|Getuwghewiugh))) "Local") (Spline|GetLocationatDistanceAlongSpline _bridgespline (+ (+ (* _index (Variables|Default|GetDistanceBetweenPieces)) (* (Variables|Default|GetTurning%20Distance%20Compensation) (Variables|Default|Getuwghewiugh))) (Variables|Default|GetDistanceBetweenPieces)) "Local")) "0,90.000000, 0") (Math|Rotator|SelectRotator "0, 0, 0" "0,180.000000, 0" (Math|Random|RandomBool))) "0.666600,0.666600,0.666600")))
            (:2
              (Components|InstancedStaticMesh|AddInstance (Variables|Default|GetLongPiece3) (Math|Transform|MakeTransform (* (+ (Spline|GetLocationatDistanceAlongSpline _bridgespline (+ (* _index (Variables|Default|GetDistanceBetweenPieces)) (* (Variables|Default|GetTurning%20Distance%20Compensation) (Variables|Default|Getuwghewiugh))) "Local") (Spline|GetLocationatDistanceAlongSpline _bridgespline (+ (+ (* _index (Variables|Default|GetDistanceBetweenPieces)) (* (Variables|Default|GetTurning%20Distance%20Compensation) (Variables|Default|Getuwghewiugh))) (Variables|Default|GetDistanceBetweenPieces)) "Local")) 0.5) (Math|Rotator|CombineRotators (Math|Rotator|CombineRotators (Math|Rotator|FindLookatRotation (Spline|GetLocationatDistanceAlongSpline _bridgespline (+ (* _index (Variables|Default|GetDistanceBetweenPieces)) (* (Variables|Default|GetTurning%20Distance%20Compensation) (Variables|Default|Getuwghewiugh))) "Local") (Spline|GetLocationatDistanceAlongSpline _bridgespline (+ (+ (* _index (Variables|Default|GetDistanceBetweenPieces)) (* (Variables|Default|GetTurning%20Distance%20Compensation) (Variables|Default|Getuwghewiugh))) (Variables|Default|GetDistanceBetweenPieces)) "Local")) "0,90.000000, 0") (Math|Rotator|SelectRotator "0, 0, 0" "0,180.000000, 0" (Math|Random|RandomBool))) "0.666600,0.666600,0.666600")))))
        (:B
          (switch int _returnvalue
            (:0
              (Components|InstancedStaticMesh|AddInstance (Variables|Default|GetShortPiece1) (Math|Transform|MakeTransform (* (+ (Spline|GetLocationatDistanceAlongSpline _bridgespline (+ (* _index (Variables|Default|GetDistanceBetweenPieces)) (* (Variables|Default|GetTurning%20Distance%20Compensation) (Variables|Default|Getuwghewiugh))) "Local") (Spline|GetLocationatDistanceAlongSpline _bridgespline (+ (+ (* _index (Variables|Default|GetDistanceBetweenPieces)) (* (Variables|Default|GetTurning%20Distance%20Compensation) (Variables|Default|Getuwghewiugh))) (Variables|Default|GetDistanceBetweenPieces)) "Local")) 0.5) (Math|Rotator|CombineRotators (Math|Rotator|CombineRotators (Math|Rotator|FindLookatRotation (Spline|GetLocationatDistanceAlongSpline _bridgespline (+ (* _index (Variables|Default|GetDistanceBetweenPieces)) (* (Variables|Default|GetTurning%20Distance%20Compensation) (Variables|Default|Getuwghewiugh))) "Local") (Spline|GetLocationatDistanceAlongSpline _bridgespline (+ (+ (* _index (Variables|Default|GetDistanceBetweenPieces)) (* (Variables|Default|GetTurning%20Distance%20Compensation) (Variables|Default|Getuwghewiugh))) (Variables|Default|GetDistanceBetweenPieces)) "Local")) "0,90.000000, 0") (Math|Rotator|SelectRotator "0, 0, 0" "0,180.000000, 0" (Math|Random|RandomBool))) "0.666600,0.666600,0.666600")))
            (:1
              (Components|InstancedStaticMesh|AddInstance (Variables|Default|GetShortPiece2) (Math|Transform|MakeTransform (* (+ (Spline|GetLocationatDistanceAlongSpline _bridgespline (+ (* _index (Variables|Default|GetDistanceBetweenPieces)) (* (Variables|Default|GetTurning%20Distance%20Compensation) (Variables|Default|Getuwghewiugh))) "Local") (Spline|GetLocationatDistanceAlongSpline _bridgespline (+ (+ (* _index (Variables|Default|GetDistanceBetweenPieces)) (* (Variables|Default|GetTurning%20Distance%20Compensation) (Variables|Default|Getuwghewiugh))) (Variables|Default|GetDistanceBetweenPieces)) "Local")) 0.5) (Math|Rotator|CombineRotators (Math|Rotator|CombineRotators (Math|Rotator|FindLookatRotation (Spline|GetLocationatDistanceAlongSpline _bridgespline (+ (* _index (Variables|Default|GetDistanceBetweenPieces)) (* (Variables|Default|GetTurning%20Distance%20Compensation) (Variables|Default|Getuwghewiugh))) "Local") (Spline|GetLocationatDistanceAlongSpline _bridgespline (+ (+ (* _index (Variables|Default|GetDistanceBetweenPieces)) (* (Variables|Default|GetTurning%20Distance%20Compensation) (Variables|Default|Getuwghewiugh))) (Variables|Default|GetDistanceBetweenPieces)) "Local")) "0,90.000000, 0") (Math|Rotator|SelectRotator "0, 0, 0" "0,180.000000, 0" (Math|Random|RandomBool))) "0.666600,0.666600,0.666600")))
            (:2
              (Components|InstancedStaticMesh|AddInstance (Variables|Default|GetShortPiece3) (Math|Transform|MakeTransform (* (+ (Spline|GetLocationatDistanceAlongSpline _bridgespline (+ (* _index (Variables|Default|GetDistanceBetweenPieces)) (* (Variables|Default|GetTurning%20Distance%20Compensation) (Variables|Default|Getuwghewiugh))) "Local") (Spline|GetLocationatDistanceAlongSpline _bridgespline (+ (+ (* _index (Variables|Default|GetDistanceBetweenPieces)) (* (Variables|Default|GetTurning%20Distance%20Compensation) (Variables|Default|Getuwghewiugh))) (Variables|Default|GetDistanceBetweenPieces)) "Local")) 0.5) (Math|Rotator|CombineRotators (Math|Rotator|CombineRotators (Math|Rotator|FindLookatRotation (Spline|GetLocationatDistanceAlongSpline _bridgespline (+ (* _index (Variables|Default|GetDistanceBetweenPieces)) (* (Variables|Default|GetTurning%20Distance%20Compensation) (Variables|Default|Getuwghewiugh))) "Local") (Spline|GetLocationatDistanceAlongSpline _bridgespline (+ (+ (* _index (Variables|Default|GetDistanceBetweenPieces)) (* (Variables|Default|GetTurning%20Distance%20Compensation) (Variables|Default|Getuwghewiugh))) (Variables|Default|GetDistanceBetweenPieces)) "Local")) "0,90.000000, 0") (Math|Rotator|SelectRotator "0, 0, 0" "0,180.000000, 0" (Math|Random|RandomBool))) "0.666600,0.666600,0.666600"))))))
      (if (> _index 1)
        (Utilities|Array|Add (Variables|Default|GetPrevious%20Piece%20Angle%20Array) (Math|Rotator|CombineRotators (Math|Rotator|CombineRotators (Math|Rotator|FindLookatRotation (Spline|GetLocationatDistanceAlongSpline _bridgespline (+ (* _index (Variables|Default|GetDistanceBetweenPieces)) (* (Variables|Default|GetTurning%20Distance%20Compensation) (Variables|Default|Getuwghewiugh))) "Local") (Spline|GetLocationatDistanceAlongSpline _bridgespline (+ (+ (* _index (Variables|Default|GetDistanceBetweenPieces)) (* (Variables|Default|GetTurning%20Distance%20Compensation) (Variables|Default|Getuwghewiugh))) (Variables|Default|GetDistanceBetweenPieces)) "Local")) "0,90.000000, 0") (* (Variables|Default|GetPrevious%20Piece%20Angle) -1.0))))
      (Variables|Default|SetPrevious%20Piece%20Angle (Math|Rotator|CombineRotators (Math|Rotator|FindLookatRotation (Spline|GetLocationatDistanceAlongSpline _bridgespline (+ (* _index (Variables|Default|GetDistanceBetweenPieces)) (* (Variables|Default|GetTurning%20Distance%20Compensation) (Variables|Default|Getuwghewiugh))) "Local") (Spline|GetLocationatDistanceAlongSpline _bridgespline (+ (+ (* _index (Variables|Default|GetDistanceBetweenPieces)) (* (Variables|Default|GetTurning%20Distance%20Compensation) (Variables|Default|Getuwghewiugh))) (Variables|Default|GetDistanceBetweenPieces)) "Local")) "0,90.000000, 0")))))